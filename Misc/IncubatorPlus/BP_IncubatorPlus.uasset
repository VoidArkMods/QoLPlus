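; QoL+ Egg Incubator structure that adds automatic temperature control, optional auto-hatching, a snap toggle during placement and server-configured tribe limit and temperature bonus.
; Auto temperature targets the ideal of the most numerous egg species, recalculating on egg add/remove or when no egg matches.
; UpdateIncubation drains egg durability on the server, hatching or damaging eggs by power and settings, while clients infer progress for smooth display.
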(event EventBeginPlay
  (bind _returnvalue (Game|GetGameMode))
  (|CallParentFunction)
  (Utilities|FlowControl|Delay 0)
  (if (Variables|Default|GetbIsPreviewStructure)
    (bind _returnvalue_2 (Class|Actor|GetOwnerController))
    (Input|EnableInput _returnvalue_2)
    (CallFunction|SPClearGlobalBuffDisabledSnaps _returnvalue_2)
    (else
      (Variables|/Script/ShooterGame.PrimalInventoryComponent|SetInventoryNameOverride (Variables|Default|GetMyInventoryComponent) "QoL+ Egg Incubator")
      (Networking|SwitchHasAuthority
        (:Authority
          (Utilities|FlowControl|Sequence
            (:then_0
              (Variables|Default|SetbIsLocked (not (Variables|Default|GetIsUnlocked)) true))
            (:then_1
              (bind _value (CallFunction|SPGetConfig-Float _returnvalue "IncubatorPerfectTempBonus" 1.2 1.0 1e+02))
              (Variables|Default|SetPerfectTempBonusOverride _value true))
            (:then_2
              (bind _value_2 (CallFunction|SPGetConfig-Int _returnvalue "IncubatorTribeLimit" 0 0 999999))
              (Variables|Default|SetTribeLimit _value_2)
              (if (> _value_2 0)
                (Utilities|FlowControl|Delay 0 1.0)
                (CallFunction|SPAddtoCustomActorList self (Utilities|String|BuildString(Integer) "SPlusIncubator_" "" (Variables|Default|GetTargetingTeam)))))
            (:then_3
              (bind _value_3 (CallFunction|SPGetConfig-Bool _returnvalue "IncubatorDisableAutoHatch"))
              (Variables|Default|SetDisableAutoHatch _value_3 true))))))))

(event Input|ActionEvents|InputActionDrag
  (params (Key :type Key%20Structure :default "None"))
  (:Pressed
    (bind _returnvalue (Class|Actor|GetOwnerController))
    (bind _success (CallFunction|SPToggleGlobalBuffDisabledSnaps _returnvalue (Utilities|Array|MakeArray) (Utilities|Array|MakeArray 1) (not (Variables|Default|GetDisableSnaps))))
    (if _success
      (Variables|Default|SetDisableSnaps (not (Variables|Default|GetDisableSnaps))))))

(fn ConstructionScript
  (|CallParentFunction))

(fn BPIsAllowedtoBuildEx
  (params (OutPlacementData :type Placement%20Data%20Structure%20%28by%20ref%29) (CurrentAllowedReason :type Integer) (PC :type Player%20Controller%20Object%20Reference) (bFinalPlacement :type Boolean) (bChoosingRotation :type Boolean))
  (bind _buildreason (CallFunction|SPCheckTribeLimit self "Incubator" CurrentAllowedReason (Variables|Default|GetTribeLimit) (Utilities|String|BuildString(Integer) "SPlusIncubator_" "" (Variables|Default|GetTargetingTeam)) bFinalPlacement PC))
  (return _buildreason))

(fn ReceiveDestroyed
  (|CallParentFunction)
  (Networking|SwitchHasAuthority
    (:Authority
      (if (not (Variables|Default|GetbIsPreviewStructure))
        (CallFunction|SPRemovefromCustomActorList self (Utilities|String|BuildString(Integer) "SPlusIncubator_" "" (Variables|Default|GetTargetingTeam)))))))

(fn BPonStructurePickup
  (params (PlayerController :type Player%20Controller%20Object%20Reference) (ItemType :type Primal%20Item%20Class%20Reference) (NewlyPickedUpItem :type Primal%20Item%20Object%20Reference) (bIsQuickPickup :type Boolean))
  (Networking|SwitchHasAuthority
    (:Authority
      (CallFunction|SPRemovefromCustomActorList self (Utilities|String|BuildString(Integer) "SPlusIncubator_" "" (Variables|Default|GetTargetingTeam))))))

(fn BPSetPlayerConstructor
  (params (PC :type Player%20Controller%20Object%20Reference))
  (bind _asbuff_structures_plus_global_buff (Utilities|Casting|CastToBuff_StructuresPlus_GlobalBuff (CallFunction|SPGetGlobalBuff PC)))
  (Variables|Default|SetDisableSnaps (> (Utilities|Array|Length (Variables|/QoLPlus/_Buffs/Buff_StructuresPlus_GlobalBuff.Buff_StructuresPlus_GlobalBuff_C|GetDisabledSnapsFrom _asbuff_structures_plus_global_buff)) 0))
  (CallFunction|SPClearGlobalBuffDisabledSnaps PC))

(fn BPTryMultiUse
  (params (ForPC :type Player%20Controller%20Object%20Reference) (UseIndex :type Integer))
  (Utilities|FlowControl|Sequence
    (:then_0
      (if (== UseIndex 601)
        (Variables|Default|SetIsUnlocked (not (Variables|Default|GetbIsLocked)))
        (else
          (switch int UseIndex
            (:9000
              (Variables|Default|SetAutoTempAdjust (not (Variables|Default|GetAutoTempAdjust)) true)
              (if (Variables|Default|GetAutoTempAdjust)
                (CallFunction|CalcIncubationTemp)))
            (:9001
              (Variables|Default|SetAutoHatchAllEggs (not (Variables|Default|GetAutoHatchAllEggs)) true))))))
    (:then_1
      (bind _returnvalue (|CallParentFunction ForPC UseIndex))
      (return _returnvalue))))

(fn IsValidSnapPointfrom
  (params (ParentStructure :type Primal%20Structure%20Object%20Reference) (MySnapPointFromIndex :type Integer))
  (return (not (Variables|Default|GetDisableSnaps))))

(fn BPGetMultiUseEntries
  (params (ForPC :type Player%20Controller%20Object%20Reference) (MultiUseEntries :type Array%20of%20Multi%20Use%20Entry%20Structures))
  (bind _returnvalue (|CallParentFunction ForPC MultiUseEntries))
  (Utilities|FlowControl|Sequence
    (:then_0
      (bind _returnvalue_2 (Class|PrimalStructure|AllowStructureAccess ForPC))
      (if _returnvalue_2
        (Utilities|Array|Add _returnvalue (Utilities|Struct|MakeMultiUseEntry (Utilities|String|SelectString "Automatic Temp. Control" "Manual Temp. Control" (Variables|Default|GetAutoTempAdjust)) 9000 -1000 true))
        (if (not (Variables|Default|GetDisableAutoHatch))
          (Utilities|Array|Add _returnvalue (Utilities|Struct|MakeMultiUseEntry (Utilities|String|SelectString "Auto Hatching Eggs" "Not Auto Hatching Eggs" (Variables|Default|GetAutoHatchAllEggs)) 9001 -1100 true)))))
    (:then_1
      (return _returnvalue))))

(fn ServerAddFertilizedEgg
  (params (EggItem :type Primal%20Item%20Consumable%20Egg%20Object%20Reference))
  (|CallParentFunction EggItem)
  (if (Variables|Default|GetAutoTempAdjust)
    (CallFunction|CalcIncubationTemp)))

(fn ServerRemoveFertilizedEgg
  (params (EggItem :type Primal%20Item%20Consumable%20Egg%20Object%20Reference))
  (|CallParentFunction EggItem)
  (if (Variables|Default|GetAutoTempAdjust)
    (CallFunction|CalcIncubationTemp)))

(fn UpdateIncubation
  (bind _returnvalue (Utilities|Time|GetGameTimeinSeconds))
  (bind _eggsloteggitems (Variables|Default|GetEggSlotEggItems))
  (if (and (> (Variables|Default|GetLastUpdateIncubation) 0.0) (>= (Utilities|Time|GetGameTimeinSeconds) (+ (Variables|Default|GetLastUpdateIncubation) (Math|Float|SelectFloat (Variables|Default|GetDedicatedServerIncubationUpdateRateSeconds) (Math|Float|SelectFloat (Variables|Default|GetListeningServerIncubationUpdateRateSeconds) (Variables|Default|GetClientIncubationUpdateRateSeconds) (Networking|IsServer)) (Networking|IsDedicatedServer)))))
    (Utilities|FlowControl|Sequence
      (:then_0
        ;[1 1 1] GetDeltaTime
        (LocalVariables|SetDeltaSec_UI (Math|Conversions|ToFloat(Integer) (- _returnvalue (Variables|Default|GetLastUpdateIncubation))))
        (Variables|Default|SetLastUpdateIncubation _returnvalue))
      (:then_1
        (Networking|SwitchHasAuthority
          (:Authority
            (for _array_element (Variables|/Script/ShooterGame.PrimalInventoryComponent|GetInventoryItems (Variables|Default|GetMyInventoryComponent))
              (bind _asprimal_item_consumable_egg (Utilities|Casting|CastToPrimalItemConsumable_Egg _array_element))
              (if (CallFunction|CheckIsFertilizedEgg _asprimal_item_consumable_egg)
                (LocalVariables|SetCurEgg_UI _asprimal_item_consumable_egg)
                (Utilities|FlowControl|Sequence
                  (:then_0
                    (if (Variables|Default|GetAutoTempAdjust)
                      (if (Math|Float|NearlyEqual(Float) (Math|Conversions|ToFloat(Integer) (Math|Float|Round (/ (+ (Variables|/Script/ShooterGame.PrimalItem|GetEggMaxTemperature _asprimal_item_consumable_egg) (Variables|/Script/ShooterGame.PrimalItem|GetEggMinTemperature _asprimal_item_consumable_egg)) 2.0))) (Variables|Default|GetTempControlValue) 0.01)
                        (LocalVariables|SetAtLeastOnePerfectTempEgg_UI true))))
                  (:then_1
                    (Utilities|Casting|CastToPrimalItemConsumable_UnderwaterEgg (LocalVariables|GetCurEgg_UI)
                      (:then
                        (bind _returnvalue_2 (Class|BiomeZoneVolume|IsPointUnderwater (Class|Actor|GetWorld) (Transformation|GetActorLocation) true 0.0 false false)) ; Don't incubate underwater eggs if the incubator is somehow no longer underwater
                        (if _returnvalue_2
                          (CallFunction|SetIncubatorCustomDatasforEgg (LocalVariables|GetCurEgg_UI) :!label _label)
                          (bind _bcanincubate (CallFunction|CanEggIncubateinTemp (LocalVariables|GetCurEgg_UI)))
                          (if _bcanincubate
                            (Variables|/Script/ShooterGame.PrimalItem|SetItemDurability (LocalVariables|GetCurEgg_UI) (Math|Float|Clamp(Float) (Math|Float|Max(Float) (- (Variables|/Script/ShooterGame.PrimalItem|GetItemDurability (LocalVariables|GetCurEgg_UI)) (* (* (* (* (LocalVariables|GetDeltaSec_UI) (Variables|/Script/ShooterGame.PrimalItem|GetEggLoseDurabilityPerSecond (LocalVariables|GetCurEgg_UI))) (Variables|/Script/ShooterGame.PrimalItem|GetExtraEggLoseDurabilityPerSecondMultiplier (LocalVariables|GetCurEgg_UI))) (Variables|Default|GetCachedEggHatchSpeedMultiplier)) (CallFunction|GetTempControlBonus (Variables|/Script/ShooterGame.PrimalItem|GetEggMinTemperature (LocalVariables|GetCurEgg_UI)) (Variables|/Script/ShooterGame.PrimalItem|GetEggMaxTemperature (LocalVariables|GetCurEgg_UI))))) 0.0) (Variables|Default|GetIncubationFloorClamp) (Variables|/Script/ShooterGame.PrimalItem|GetItemDurability (LocalVariables|GetCurEgg_UI))))
                            (Networking|SwitchHasAuthority :!label _label_2
                              (:Authority
                                (if (or (Math|Boolean|ANDBoolean (not (Variables|Default|GetbIsPowered)) (Variables|Default|GetbAutoHatchEggsWhenUnpowered) (<= (Variables|/Script/ShooterGame.PrimalItem|GetItemDurability (LocalVariables|GetCurEgg_UI)) 0.0)) (Math|Boolean|ANDBoolean (<= (Variables|/Script/ShooterGame.PrimalItem|GetItemDurability (LocalVariables|GetCurEgg_UI)) 0.0) (Variables|Default|GetAutoHatchAllEggs) (not (Variables|Default|GetDisableAutoHatch))))
                                  (bind _eggwasspawned (CallFunction|TrySpawnEggtoWorld (LocalVariables|GetCurEgg_UI)))
                                  (if _eggwasspawned
                                    (CallFunction|MCDestroyEggVFX (.ItemID1 (Class|PrimalItem|BPGetItemID (LocalVariables|GetCurEgg_UI))) (.ItemID2 (Class|PrimalItem|BPGetItemID (LocalVariables|GetCurEgg_UI))))
                                    (Class|PrimalInventoryComponent|RemoveItem (Variables|Default|GetMyInventoryComponent) (Variables|/Script/ShooterGame.PrimalItem|GetItemID (LocalVariables|GetCurEgg_UI)) false false false false))
                                  (else
                                    (Class|PrimalItem|UpdatedItem (LocalVariables|GetCurEgg_UI) false)))))
                            (elif (and (not (Variables|Default|GetbIsPowered)) (Variables|Default|GetbDamageEggsWhenUnpoweredAndUnableToIncubate))
                              (Variables|/Script/ShooterGame.PrimalItem|SetItemRating (LocalVariables|GetCurEgg_UI) (Math|Float|Max(Float) (- (Variables|/Script/ShooterGame.PrimalItem|GetItemRating (LocalVariables|GetCurEgg_UI)) (* (Variables|/Script/ShooterGame.PrimalItem|GetEggDroppedInvalidTempLoseItemRatingSpeed (LocalVariables|GetCurEgg_UI)) (LocalVariables|GetDeltaSec_UI))) 0.0))
                              (if (and (Networking|IsServer) (<= (Variables|/Script/ShooterGame.PrimalItem|GetItemRating (LocalVariables|GetCurEgg_UI)) 0.0))
                                (Class|PrimalInventoryComponent|RemoveItem (Variables|Default|GetMyInventoryComponent) (Variables|/Script/ShooterGame.PrimalItem|GetItemID (LocalVariables|GetCurEgg_UI)) false false false false)
                                (else
                                  (goto _label_2)))
                              (else
                                (goto _label_2))))))
                      (:CastFailed
                        (goto _label)))))))
            (if (and (Variables|Default|GetAutoTempAdjust) (not (LocalVariables|GetAtLeastOnePerfectTempEgg_UI)))
              (CallFunction|CalcIncubationTemp)))
          (:Remote
            ;[1 1 1] Inferred Incubation progress on remote clients for smooth display between syncs from the server
            (for (_array_element_2 _array_index) (Variables|Default|GetEggSlotInUse)
              (if (Math|Boolean|ANDBoolean _array_element_2 (Utilities|Array|IsValidIndex _eggsloteggitems _array_index) (Utilities|IsValid (Utilities|Array|Get(acopy) _eggsloteggitems _array_index)))
                (LocalVariables|SetCurEgg_UI (Utilities|Array|Get(acopy) _eggsloteggitems _array_index))
                (Utilities|Casting|CastToPrimalItemConsumable_UnderwaterEgg (LocalVariables|GetCurEgg_UI)
                  (:then
                    (bind _returnvalue_3 (Class|BiomeZoneVolume|IsPointUnderwater (Class|Actor|GetWorld) (Transformation|GetActorLocation) true 0.0 false false)) ; Don't incubate underwater eggs if the incubator is somehow no longer underwater
                    (if _returnvalue_3
                      (CallFunction|SetIncubatorCustomDatasforEgg (LocalVariables|GetCurEgg_UI) :!label _label_3)
                      (bind _bcanincubate_2 (CallFunction|CanEggIncubateinTemp (LocalVariables|GetCurEgg_UI)))
                      (if _bcanincubate_2
                        (Variables|/Script/ShooterGame.PrimalItem|SetItemDurability (LocalVariables|GetCurEgg_UI) (Math|Float|Clamp(Float) (Math|Float|Max(Float) (- (Variables|/Script/ShooterGame.PrimalItem|GetItemDurability (LocalVariables|GetCurEgg_UI)) (* (* (* (* (LocalVariables|GetDeltaSec_UI) (Variables|/Script/ShooterGame.PrimalItem|GetEggLoseDurabilityPerSecond (LocalVariables|GetCurEgg_UI))) (Variables|/Script/ShooterGame.PrimalItem|GetExtraEggLoseDurabilityPerSecondMultiplier (LocalVariables|GetCurEgg_UI))) (Variables|Default|GetCachedEggHatchSpeedMultiplier)) (CallFunction|GetTempControlBonus (Variables|/Script/ShooterGame.PrimalItem|GetEggMinTemperature (LocalVariables|GetCurEgg_UI)) (Variables|/Script/ShooterGame.PrimalItem|GetEggMaxTemperature (LocalVariables|GetCurEgg_UI))))) 0.0) (Variables|Default|GetIncubationFloorClamp) (Variables|/Script/ShooterGame.PrimalItem|GetItemDurability (LocalVariables|GetCurEgg_UI))))
                        (Networking|SwitchHasAuthority :!label _label_4
                          (:Authority
                            (if (or (Math|Boolean|ANDBoolean (not (Variables|Default|GetbIsPowered)) (Variables|Default|GetbAutoHatchEggsWhenUnpowered) (<= (Variables|/Script/ShooterGame.PrimalItem|GetItemDurability (LocalVariables|GetCurEgg_UI)) 0.0)) (Math|Boolean|ANDBoolean (<= (Variables|/Script/ShooterGame.PrimalItem|GetItemDurability (LocalVariables|GetCurEgg_UI)) 0.0) (Variables|Default|GetAutoHatchAllEggs) (not (Variables|Default|GetDisableAutoHatch))))
                              (bind _eggwasspawned_2 (CallFunction|TrySpawnEggtoWorld (LocalVariables|GetCurEgg_UI)))
                              (if _eggwasspawned_2
                                (CallFunction|MCDestroyEggVFX (.ItemID1 (Class|PrimalItem|BPGetItemID (LocalVariables|GetCurEgg_UI))) (.ItemID2 (Class|PrimalItem|BPGetItemID (LocalVariables|GetCurEgg_UI))))
                                (Class|PrimalInventoryComponent|RemoveItem (Variables|Default|GetMyInventoryComponent) (Variables|/Script/ShooterGame.PrimalItem|GetItemID (LocalVariables|GetCurEgg_UI)) false false false false))
                              (else
                                (Class|PrimalItem|UpdatedItem (LocalVariables|GetCurEgg_UI) false)))))
                        (elif (and (not (Variables|Default|GetbIsPowered)) (Variables|Default|GetbDamageEggsWhenUnpoweredAndUnableToIncubate))
                          (Variables|/Script/ShooterGame.PrimalItem|SetItemRating (LocalVariables|GetCurEgg_UI) (Math|Float|Max(Float) (- (Variables|/Script/ShooterGame.PrimalItem|GetItemRating (LocalVariables|GetCurEgg_UI)) (* (Variables|/Script/ShooterGame.PrimalItem|GetEggDroppedInvalidTempLoseItemRatingSpeed (LocalVariables|GetCurEgg_UI)) (LocalVariables|GetDeltaSec_UI))) 0.0))
                          (if (and (Networking|IsServer) (<= (Variables|/Script/ShooterGame.PrimalItem|GetItemRating (LocalVariables|GetCurEgg_UI)) 0.0))
                            (Class|PrimalInventoryComponent|RemoveItem (Variables|Default|GetMyInventoryComponent) (Variables|/Script/ShooterGame.PrimalItem|GetItemID (LocalVariables|GetCurEgg_UI)) false false false false)
                            (else
                              (goto _label_4)))
                          (else
                            (goto _label_4))))))
                  (:CastFailed
                    (goto _label_3)))))))))))

(fn CalcIncubationTemp
  (bind _dinoclassqtys_cit (LocalVariables|GetDinoClassQtys_CIT))
  (bind _dinoclassqtys_cit_2 (LocalVariables|GetDinoClassQtys_CIT))
  (for _array_element (Variables|/Script/ShooterGame.PrimalInventoryComponent|GetInventoryItems (Variables|Default|GetMyInventoryComponent))
    (bind _asprimal_item_consumable_egg (Utilities|Casting|CastToPrimalItemConsumable_Egg _array_element))
    (if (and (CallFunction|CheckIsFertilizedEgg _asprimal_item_consumable_egg) (> (Variables|/Script/ShooterGame.PrimalItem|GetItemDurability _asprimal_item_consumable_egg) 0.0))
      (LocalVariables|SetFoundIndex_CIT (Utilities|Array|FindItem (LocalVariables|GetDinosToSpawn_CIT) (Utilities|ResolveSoftReference (Variables|/Script/ShooterGame.PrimalItem|GetEggDinoClassToSpawn _asprimal_item_consumable_egg))))
      (if (>= (LocalVariables|GetFoundIndex_CIT) 0)
        (Utilities|Array|SetArrayElem _dinoclassqtys_cit (LocalVariables|GetFoundIndex_CIT) (+ (Utilities|Array|Get(acopy) _dinoclassqtys_cit (LocalVariables|GetFoundIndex_CIT)) 1))
        (else
          (Utilities|Array|Add (LocalVariables|GetDinosToSpawn_CIT) (Utilities|ResolveSoftReference (Variables|/Script/ShooterGame.PrimalItem|GetEggDinoClassToSpawn _asprimal_item_consumable_egg)))
          (Utilities|Array|Add (LocalVariables|GetDinoClassQtys_CIT) (Class|KismetSystemLibrary|MakeLiteralInteger 1))
          (Utilities|Array|Add (LocalVariables|GetEggIdealTemps_CIT) (Math|Conversions|ToFloat(Integer) (Math|Float|Round (/ (+ (Variables|/Script/ShooterGame.PrimalItem|GetEggMaxTemperature _asprimal_item_consumable_egg) (Variables|/Script/ShooterGame.PrimalItem|GetEggMinTemperature _asprimal_item_consumable_egg)) 2.0))))))))
  (if (> (Utilities|Array|Length _dinoclassqtys_cit_2) 0)
    (LocalVariables|SetMaxIndex_CIT (.IndexOfMaxValue (Math|Integer|MaxOfIntArray _dinoclassqtys_cit_2)))
    (Variables|Default|SetTempControlValue (Utilities|Array|Get(acopy) (LocalVariables|GetEggIdealTemps_CIT) (LocalVariables|GetMaxIndex_CIT)) true)
    (CallFunction|MCUpdateWarmingLighhts)))

(fn OnRepPerfectTempBonusOverride
  (Variables|Default|SetTempControlBonusMultiplierRangeMax (Variables|Default|GetPerfectTempBonusOverride)))