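; Tek oil pump structure (S+) that can automatically send its oil to the team's dedicated storage.
; An inventory menu toggle sets PhoneHome, running a randomized looping timer that is restarted on server save load.
; Each tick finds team-tagged storages via custom actor lists, randomly picks one accepting oil, and moves what fits.
; It also reads slot count from game config, restores lock state, and overrides one build-placement failure code.
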(event EventBPPostLoadedfromSaveGame
  (Networking|SwitchHasAuthority
    (:Authority
      (if (Variables|Default|GetPhoneHome)
        (Utilities|FlowControl|Delay 0 1.0)
        (CallFunction|ToggleTimer true)))))

(fn ConstructionScript
  (|CallParentFunction))

(fn ReceiveBeginPlay
  (|CallParentFunction)
  (if (not (Variables|Default|GetbIsPreviewStructure))
    (Networking|SwitchHasAuthority
      (:Authority
        (Utilities|FlowControl|Sequence
          (:then_0
            (bind _value (CallFunction|SPGetConfigSetting-InventorySize (Game|GetGameMode) "OilPumpSlotCount" 100))
            (Variables|Default|SetInventorySlots _value true))
          (:then_1
            (Variables|Default|SetbIsLocked (not (Variables|Default|GetIsUnlocked)) true)))))))

(fn BPIsAllowedtoBuild
  (params (OutPlacementData :type Placement%20Data%20Structure%20%28by%20ref%29) (CurrentAllowedReason :type Integer))
  (return (Math|Integer|SelectInt 1 CurrentAllowedReason (== CurrentAllowedReason -9))))

(fn BPGetMultiUseEntries
  (params (ForPC :type Player%20Controller%20Object%20Reference) (MultiUseEntries :type Array%20of%20Multi%20Use%20Entry%20Structures))
  (bind _entriesout (CallFunction|SPUpdateMultiUseMenu ForPC MultiUseEntries self false false false false))
  (Utilities|FlowControl|Sequence
    (:then_0
      (bind _returnvalue (Class|PrimalStructure|AllowStructureAccess ForPC))
      (if _returnvalue
        (Utilities|Array|Add _entriesout (Utilities|Struct|MakeMultiUseEntry (Utilities|String|SelectString "Transferring to Dedicated Storage" "Holding Inventory" (Variables|Default|GetPhoneHome)) 9000 -1000 true true))))
    (:then_1
      (return _entriesout))))

(fn BPTryMultiUse
  (params (ForPC :type Player%20Controller%20Object%20Reference) (UseIndex :type Integer))
  (Utilities|FlowControl|Sequence
    (:then_0
      (if (== UseIndex 601)
        (Variables|Default|SetIsUnlocked (not (Variables|Default|GetbIsLocked)))))
    (:then_1
      (if (== UseIndex 9000)
        (Variables|Default|SetPhoneHome (not (Variables|Default|GetPhoneHome)) true)
        (CallFunction|ToggleTimer (Variables|Default|GetPhoneHome))))
    (:then_2
      (return true))))

(fn OnRepInventorySlots)

(fn GetDedicatedStorage
  (bind _matchingstorages (LocalVariables|GetMatchingStorages))
  (bind _returnvalue (Utilities|Array|Length _matchingstorages))
  (Utilities|FlowControl|Sequence
    (:then_0
      (bind _returnvalue_2 (Class|VictoryCore|GetCustomActorList (Class|Actor|GetWorld) (Utilities|String|StringToName (Utilities|String|BuildString(Integer) "SPlusDedicatedStorage_" "" (Variables|Default|GetTargetingTeam)))))
      (Utilities|IsValid _returnvalue_2
        (:Is%20Valid
          (for _array_element (Variables|/Script/ShooterGame.CustomActorList|GetActorList _returnvalue_2)
            (bind _asprimal_structure_item_container (Utilities|Casting|CastToPrimalStructureItemContainer _array_element))
            (if (Utilities|SPIsValidArrayIndex (Variables|/Script/ShooterGame.PrimalInventoryComponent|GetRemoteAddItemOnlyAllowItemClasses (Variables|/Script/ShooterGame.PrimalStructureItemContainer|GetMyInventoryComponent _asprimal_structure_item_container)))
              (if (and (CallFunction|SPDoesInventoryHaveEmptySlots (Variables|/Script/ShooterGame.PrimalStructureItemContainer|GetMyInventoryComponent _asprimal_structure_item_container)) (Utilities|ClassIsChildOf (Utilities|Array|Get(acopy) (Variables|/Script/ShooterGame.PrimalInventoryComponent|GetRemoteAddItemOnlyAllowItemClasses (Variables|/Script/ShooterGame.PrimalStructureItemContainer|GetMyInventoryComponent _asprimal_structure_item_container))) "/Game/PrimalEarth/CoreBlueprints/Resources/PrimalItemResource_Oil.PrimalItemResource_Oil_C"))
                (Utilities|Array|Add (LocalVariables|GetMatchingStorages) _asprimal_structure_item_container)))))))
    (:then_1
      (return (select (> _returnvalue 0) (Utilities|Array|Get(acopy) _matchingstorages (Math|Random|RandomIntegerinRange 0 (- _returnvalue 1))) 0)))))

(fn HandleTransfer
  (bind _myinventorycomponent (Variables|Default|GetMyInventoryComponent))
  (Class|PrimalInventoryComponent|BPInventoryRefresh _myinventorycomponent)
  (bind _storage (CallFunction|GetDedicatedStorage))
  (Utilities|IsValid _storage
    (:Is%20Valid
      (bind _outitem (CallFunction|SPGetRemappedItem "/Game/PrimalEarth/CoreBlueprints/Resources/PrimalItemResource_Oil.PrimalItemResource_Oil_C"))
      (bind _total (CallFunction|SPGetCapacityforItem _outitem _storage))
      (if (> _total 0)
        (bind _returnvalue (Class|PrimalInventoryComponent|GetItemTemplateQuantity _myinventorycomponent _outitem 0 true false false false))
        (if (> _returnvalue 0)
          (LocalVariables|SetTransferQty (Math|Integer|Min(Integer) _returnvalue _total))
          (Class|PrimalInventoryComponent|BPIncrementItemTemplateQuantity _myinventorycomponent _outitem (* (LocalVariables|GetTransferQty) -1) true false true false false false 0 false)
          (Class|PrimalInventoryComponent|BPIncrementItemTemplateQuantity (Variables|/Script/ShooterGame.PrimalStructureItemContainer|GetMyInventoryComponent _storage) _outitem (LocalVariables|GetTransferQty) true false true false false false 0 false))))))

(fn ToggleTimer
  (params (Start :type Boolean))
  (if Start
    (Utilities|Time|SetTimerbyFunctionName 0 "HandleTransfer" (Math|Random|RandomFloatinRange 275.0 3e+02) true)
    (else
      (Utilities|Time|ClearTimerbyFunctionName 0 "HandleTransfer"))))