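; Structures Plus turret ammo box structure with configurable slot count and range, toggleable placement snapping and a lock state.
; After a short BeginPlay delay, the server restores the lock from IsUnlocked and reads game-mode config.
; RepNotifies apply those values to the inventory, placement radius and range visual.
; In preview, the Drag input toggles snapping through the player's global buff, and IsValidSnapPointFrom honors it.
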(event EventBeginPlay
  (bind _returnvalue (Game|GetGameMode))
  (|CallParentFunction)
  (Utilities|FlowControl|Delay 0)
  (if (Variables|Default|GetbIsPreviewStructure)
    (bind _returnvalue_2 (Class|Actor|GetOwnerController))
    (Input|EnableInput _returnvalue_2)
    (CallFunction|SPClearGlobalBuffDisabledSnaps _returnvalue_2)
    (else
      (Networking|SwitchHasAuthority
        (:Authority
          (Variables|Default|SetbIsLocked (not (Variables|Default|GetIsUnlocked)) true)
          (Utilities|FlowControl|Sequence
            (:then_0
              (bind _value (CallFunction|SPGetConfigSetting-InventorySize _returnvalue "AmmoBoxSlotCount" 300))
              (Variables|Default|SetInventorySlots _value true))
            (:then_1
              (bind _ammoboxrange (CallFunction|SPGetConfigSetting-TurretAmmoBoxRange _returnvalue))
              (Variables|Default|SetNewTurretAmmoRange _ammoboxrange true))))))))

(event Input|ActionEvents|InputActionDrag
  (params (Key :type Key%20Structure :default "None"))
  (:Pressed
    (bind _returnvalue (Class|Actor|GetOwnerController))
    (bind _success (CallFunction|SPToggleGlobalBuffDisabledSnaps _returnvalue (Utilities|Array|MakeArray) (Utilities|Array|MakeArray 1) (not (Variables|Default|GetDisableSnaps))))
    (if _success
      (Variables|Default|SetDisableSnaps (not (Variables|Default|GetDisableSnaps))))))

(fn ConstructionScript
  (|CallParentFunction))

(fn BPSetPlayerConstructor
  (params (PC :type Player%20Controller%20Object%20Reference))
  (bind _asbuff_structures_plus_global_buff (Utilities|Casting|CastToBuff_StructuresPlus_GlobalBuff (CallFunction|SPGetGlobalBuff PC)))
  (Variables|Default|SetDisableSnaps (> (Utilities|Array|Length (Variables|/QoLPlus/_Buffs/Buff_StructuresPlus_GlobalBuff.Buff_StructuresPlus_GlobalBuff_C|GetDisabledSnapsFrom _asbuff_structures_plus_global_buff)) 0))
  (CallFunction|SPClearGlobalBuffDisabledSnaps PC))

(fn IsValidSnapPointfrom
  (params (ParentStructure :type Primal%20Structure%20Object%20Reference) (MySnapPointFromIndex :type Integer))
  (return (not (Variables|Default|GetDisableSnaps))))

(fn BPTryMultiUse
  (params (ForPC :type Player%20Controller%20Object%20Reference) (UseIndex :type Integer))
  (Utilities|FlowControl|Sequence
    (:then_0
      (if (== UseIndex 601)
        (Variables|Default|SetIsUnlocked (not (Variables|Default|GetbIsLocked)))))
    (:then_1
      (bind _returnvalue (|CallParentFunction ForPC UseIndex))
      (return _returnvalue))))

(fn OnRepInventorySlots
  (Variables|/Script/ShooterGame.PrimalInventoryComponent|SetAbsoluteMaxInventoryItems (Variables|Default|GetMyInventoryComponent) (Variables|Default|GetInventorySlots)))

(fn OnRepNewTurretAmmoRange
  (bind _newturretammorange (Variables|Default|GetNewTurretAmmoRange))
  (Variables|Default|SetAmmoContainerPlacementRadius _newturretammorange)
  (Transformation|SetWorldScale3D (Variables|Default|GetVisualRadius) (Math|Conversions|ToVector(Float) (/ _newturretammorange 1e+01)))
  (bind _asprimal_inventory_ammo_box_plus (Utilities|Casting|CastToPrimalInventory_AmmoBoxPlus (Variables|Default|GetMyInventoryComponent)))
  (Variables|/QoLPlus/Misc/AmmoBoxPlus/PrimalInventory_AmmoBoxPlus.PrimalInventory_AmmoBoxPlus_C|SetRadiusToCheckForStructures _asprimal_inventory_ammo_box_plus _newturretammorange))