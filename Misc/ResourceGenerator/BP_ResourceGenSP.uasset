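; SP resource generator structure that overrides engine hooks for placement, interaction and resource-count reporting.
; Its multi-use menu is built by the shared SPUpdateMultiUseMenu helper, and placement checks remap one specific failure reason.
; ResourceCount is exposed through the special-int and item-quantity queries, without any inventory lookup in this file.
; It counts as a valid water source only when the querying pipe reference is invalid.
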(fn ConstructionScript
  (|CallParentFunction))

(fn BPIsAllowedtoBuild
  (params (OutPlacementData :type Placement%20Data%20Structure%20%28by%20ref%29) (CurrentAllowedReason :type Integer))
  (return (Math|Integer|SelectInt 1 CurrentAllowedReason (== CurrentAllowedReason -9))))

(fn BPGetMultiUseEntries
  (params (ForPC :type Player%20Controller%20Object%20Reference) (MultiUseEntries :type Array%20of%20Multi%20Use%20Entry%20Structures))
  (bind _entriesout (CallFunction|SPUpdateMultiUseMenu ForPC MultiUseEntries self false false false false))
  (return _entriesout))

(fn BPGetExtraSpecialBlueprintInt
  (params (toCheck :type Integer))
  (return (Math|Integer|SelectInt 0 (Variables|Default|GetResourceCount) (== toCheck 0))))

(fn BPGetQuantityOfItemWithoutCheckingInventory
  (params (ItemToCheckFor :type Primal%20Item%20Class%20Reference) (bRequireExactClassMatch :type Boolean))
  (return (Math|Integer|SelectInt (Variables|Default|GetResourceCount) -1 (!= ItemToCheckFor 0))))

(fn BPIsValidWaterSourceforPipe
  (params (ForWaterPipe :type Primal%20Structure%20Water%20Pipe%20Object%20Reference))
  (return (not (Utilities|IsValid ForWaterPipe))))