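; Charge station structure that stores charge from nearby lantern pets and vivariums and uses it to recharge batteries in its inventory.
; While activated, a randomized server timer drains pets in range at a 5:1 ratio, pulls from same-team vivariums and tops up batteries.
; Multi-use entries toggle the range mesh or trigger a cooldown-limited manual vivarium pull.
; Slots, range and capacity come from server config; stasis is prevented while active and not full.
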(fn ConstructionScript)

(fn BlueprintDrawHUD
  (params (HUD :type Shooter%20HUD%20Object%20Reference) (CenterX :type Float%20%28single-precision%29) (CenterY :type Float%20%28single-precision%29))
  (bind _canvas (Variables|/Script/Engine.HUD|GetCanvas HUD))
  (Class|Canvas|SetDrawColor _canvas (Math|Conversions|ToColor(LinearColor) "(R=0.000000,G=0.825000,B=0.031290,A=1.000000)"))
  (Class|Canvas|BPDrawTextCentered _canvas (Variables|/Script/ShooterGame.ShooterHUD|GetNormalFont HUD) (Utilities|String|Append (Utilities|String|Append (Utilities|String|Append "Current Charge: " (Utilities|String|ToString(Integer) (Variables|Default|GetStoredCharge_Current))) " / ") (Utilities|String|ToString(Integer) (Variables|Default|GetStoredCharge_Max))) CenterX (+ CenterY -7e+01) 1.0 1.0 true true))

(fn BPNotifyInventoryItemChange
  (params (bIsItemAdd :type Boolean) (theItem :type Primal%20Item%20Object%20Reference) (bEquipItem :type Boolean))
  (if bIsItemAdd
    (CallFunction|ChargeBatteries)))

(fn BPGetMultiUseEntries
  (params (ForPC :type Player%20Controller%20Object%20Reference) (MultiUseEntries :type Array%20of%20Multi%20Use%20Entry%20Structures))
  (bind _entriesout (CallFunction|SPUpdateMultiUseMenu ForPC MultiUseEntries self false false false false))
  (Utilities|FlowControl|Sequence
    (:then_0
      (bind _returnvalue (Class|PrimalStructure|AllowStructureAccess ForPC))
      (if _returnvalue
        (Utilities|Array|Add _entriesout (Utilities|Struct|MakeMultiUseEntry (Utilities|String|SelectString "Show Range" "Hide Range" (Variables|Default|GetIsRangeMeshHidden)) 9000 -1000))
        (if (< (Variables|Default|GetStoredCharge_Current) (Variables|Default|GetStoredCharge_Max))
          (Utilities|Array|Add _entriesout (Utilities|Struct|MakeMultiUseEntry "Pull Charge from Nearby Vivariums" 9001 -2000 true)))))
    (:then_1
      (return _entriesout))))

(fn BPContainerActivated
  (Networking|SwitchHasAuthority
    (:Authority
      (Utilities|Time|SetTimerbyFunctionName 0 "HandleChargeStation" (CallFunction|GetInterval)))))

(fn BPContainerDeactivated
  (Networking|SwitchHasAuthority
    (:Authority
      (Utilities|Time|ClearTimerbyFunctionName 0 "HandleChargeStation"))))

(fn OnRepIsRangeMeshHidden
  (Rendering|SetVisibility (Variables|Default|GetRangeMesh) (not (Variables|Default|GetIsRangeMeshHidden)) false))

(fn BPTryMultiUse
  (params (ForPC :type Player%20Controller%20Object%20Reference) (UseIndex :type Integer))
  (Utilities|FlowControl|Sequence
    (:then_0
      (switch int UseIndex
        (:Default
          (if (== UseIndex 601)
            (Variables|Default|SetIsUnlocked (not (Variables|Default|GetbIsLocked)))))
        (:9000
          (Variables|Default|SetIsRangeMeshHidden (not (Variables|Default|GetIsRangeMeshHidden)) true))
        (:9001
          (CallFunction|HandleGetVivariumCharge ForPC))))
    (:then_1
      (return true))))

(fn ReceiveBeginPlay
  (bind _returnvalue (Game|GetGameMode))
  (|CallParentFunction)
  (if (not (Variables|Default|GetbIsPreviewStructure))
    (Networking|SwitchHasAuthority
      (:Authority
        (Utilities|FlowControl|Sequence
          (:then_0
            (bind _value (CallFunction|SPGetConfigSetting-InventorySize _returnvalue "ChargeStationSlotCount" 50))
            (Variables|Default|SetInventorySlots _value true))
          (:then_1
            (bind _value_2 (CallFunction|SPGetConfig-Int _returnvalue "ChargeStationRangeInFoundations" 5 1 100))
            (Variables|Default|SetPullRange (* _value_2 3e+02) true))
          (:then_2
            (bind _value_3 (CallFunction|SPGetConfig-Int _returnvalue "ChargeStationMaxChargeAmount" 5000 1 1000000))
            (Variables|Default|SetStoredCharge_Max _value_3 true))
          (:then_3
            (Variables|Default|SetbIsLocked (not (Variables|Default|GetIsUnlocked)) true))
          (:then_4
            (if (Variables|Default|GetbContainerActivated)
              (Utilities|Time|SetTimerbyFunctionName 0 "HandleChargeStation" (CallFunction|GetInterval)))))))))

(fn HandleChargeStation
  (if (Variables|Default|GetbContainerActivated)
    (Utilities|FlowControl|Sequence
      (:then_0
        (CallFunction|ChargeBatteries))
      (:then_1
        (bind _chargeleeched (CallFunction|LeechChargefromPets))
        (if (> _chargeleeched 0.0)
          (CallFunction|ChargeBatteries)))
      (:then_2
        (bind _chargepulled (CallFunction|GetChargefromVivariums))
        (if (> _chargepulled 0.0)
          (CallFunction|ChargeBatteries)))
      (:then_3
        (Utilities|Time|SetTimerbyFunctionName 0 "HandleChargeStation" (CallFunction|GetInterval))))))

(fn LeechChargefromPets
  (Utilities|FlowControl|Sequence
    (:then_0
      (if (< (Variables|Default|GetStoredCharge_Current) (Variables|Default|GetStoredCharge_Max))
        (bind _returnvalue (Class|VictoryCore|ServerOctreeOverlapActorsClass (Class|PrimalActor|GetWorld) (Transformation|GetActorLocation) (Variables|Default|GetPullRange) "DINOPAWNS" "/Game/Aberration/CoreBlueprints/LanternPet_Character_BP.LanternPet_Character_BP_C" true))
        (bind _array_element (Utilities|Array|ForEachLoopwithBreak _returnvalue :!label _label)
          (:LoopBody
            (bind _aslantern_pet_character_bp (Utilities|Casting|CastToLanternPet_Character_BP _array_element))
            (if (Variables|/Script/Engine.Actor|GetbStasised _aslantern_pet_character_bp)
              (Class|PrimalActor|Unstasis _aslantern_pet_character_bp))
            (if (> (Math|Float|Floor (/ (Variables|/Game/Aberration/CoreBlueprints/LanternPet_Character_BP.LanternPet_Character_BP_C|GetcurrentChargeAmount _aslantern_pet_character_bp) 5.0)) 0)
              (LocalVariables|SetChargeLeechAmt (Math|Conversions|ToFloat(Integer) (Math|Integer|Min(Integer) (Math|Float|Floor (/ (Variables|/Game/Aberration/CoreBlueprints/LanternPet_Character_BP.LanternPet_Character_BP_C|GetcurrentChargeAmount _aslantern_pet_character_bp) 5.0)) (- (Variables|Default|GetStoredCharge_Max) (Variables|Default|GetStoredCharge_Current)))))
              (LocalVariables|SetTotalChargeLeeched (+ (Math|Conversions|ToFloat(Integer) (Math|Integer|Min(Integer) (Math|Float|Floor (/ (Variables|/Game/Aberration/CoreBlueprints/LanternPet_Character_BP.LanternPet_Character_BP_C|GetcurrentChargeAmount _aslantern_pet_character_bp) 5.0)) (- (Variables|Default|GetStoredCharge_Max) (Variables|Default|GetStoredCharge_Current)))) (LocalVariables|GetTotalChargeLeeched)))
              (Variables|Default|SetStoredCharge_Current (+ (Variables|Default|GetStoredCharge_Current) (Math|Float|Floor (LocalVariables|GetChargeLeechAmt))) false)
              (Variables|/Game/Aberration/CoreBlueprints/LanternPet_Character_BP.LanternPet_Character_BP_C|SetcurrentChargeAmount _aslantern_pet_character_bp (- (Variables|/Game/Aberration/CoreBlueprints/LanternPet_Character_BP.LanternPet_Character_BP_C|GetcurrentChargeAmount _aslantern_pet_character_bp) (* (LocalVariables|GetChargeLeechAmt) 5.0)) false)
              (Variables|/Game/Aberration/CoreBlueprints/LanternPet_Character_BP.LanternPet_Character_BP_C|SetbAutoChargeActive _aslantern_pet_character_bp false false)
              (Class|PrimalActor|MulticastProperty _aslantern_pet_character_bp "currentChargeAmount" false)
              (Class|PrimalActor|MulticastProperty _aslantern_pet_character_bp "bAutoChargeActive" false)
              (if (>= (Variables|Default|GetStoredCharge_Current) (Variables|Default|GetStoredCharge_Max))
                (goto _label Break))))
          (:Completed
            (Class|PrimalActor|MulticastProperty "StoredCharge_Current" false)))))
    (:then_1
      (return (LocalVariables|GetTotalChargeLeeched)))))

(fn ChargeBatteries
  (if (> (Variables|Default|GetStoredCharge_Current) 0)
    (bind _array_element (Utilities|Array|ForEachLoopwithBreak (Variables|/Script/ShooterGame.PrimalInventoryComponent|GetInventoryItems (Variables|Default|GetMyInventoryComponent)) :!label _label)
      (:LoopBody
        (bind _asprimal_item_charge_battery (Utilities|Casting|CastToPrimalItem_ChargeBattery _array_element))
        (if (> (- (Variables|/Script/ShooterGame.PrimalItem|GetMaxDurabiltiyOverride _asprimal_item_charge_battery) (Variables|/Script/ShooterGame.PrimalItem|GetItemDurability _asprimal_item_charge_battery)) 0.0)
          (LocalVariables|SetChargeTransferAmt (Math|Float|Min(Float) (- (Variables|/Script/ShooterGame.PrimalItem|GetMaxDurabiltiyOverride _asprimal_item_charge_battery) (Variables|/Script/ShooterGame.PrimalItem|GetItemDurability _asprimal_item_charge_battery)) (Math|Conversions|ToFloat(Integer) (Variables|Default|GetStoredCharge_Current))))
          (Default|AddDurabilitySafe _asprimal_item_charge_battery (LocalVariables|GetChargeTransferAmt))
          (Variables|Default|SetStoredCharge_Current (- (Variables|Default|GetStoredCharge_Current) (Math|Float|Floor (LocalVariables|GetChargeTransferAmt))) false)
          (if (<= (Variables|Default|GetStoredCharge_Current) 0)
            (goto _label Break))))
      (:Completed
        (Class|PrimalActor|MulticastProperty "StoredCharge_Current" false)))))

(fn BPUnstasis
  (bind _returnvalue (Class|VictoryCore|IsLoadingSaveGame))
  (if (not _returnvalue)
    (Networking|SwitchHasAuthority
      (:Authority
        (if (Variables|Default|GetbContainerActivated)
          (Utilities|Time|SetTimerbyFunctionName 0 "HandleChargeStation" (CallFunction|GetInterval)))))))

(fn BPPreventStasis
  (bind _returnvalue (Class|VictoryCore|IsLoadingSaveGame))
  (return (Math|Boolean|ANDBoolean (not _returnvalue) (< (Variables|Default|GetStoredCharge_Current) (Variables|Default|GetStoredCharge_Max)) (Variables|Default|GetbContainerActivated))))

(fn OnRepInventorySlots
  (Variables|/Script/ShooterGame.PrimalInventoryComponent|SetMaxInventoryItems (Variables|Default|GetMyInventoryComponent) (Variables|Default|GetInventorySlots)))

(fn GetChargefromVivariums
  (bind _returnvalue (Class|VictoryCore|ServerOctreeOverlapActorsClass (Class|PrimalActor|GetWorld) (Transformation|GetActorLocation) (Variables|Default|GetPullRange) "STRUCTURES" "/QoLPlus/Misc/Vivarium/BP_VivariumV2.BP_VivariumV2_C" true))
  (for _array_element _returnvalue
    (if (== (Variables|/Script/Engine.Actor|GetTargetingTeam _array_element) (Variables|Default|GetTargetingTeam))
      (bind _asbp_vivarium_v2 (Utilities|Casting|CastToBP_VivariumV2 _array_element))
      (bind _grantedamt (Default|RequestCharge _asbp_vivarium_v2 (Math|Conversions|ToFloat(Integer) (- (Variables|Default|GetStoredCharge_Max) (Variables|Default|GetStoredCharge_Current)))))
      (LocalVariables|SetChargePulled_GCV (+ _grantedamt (LocalVariables|GetChargePulled_GCV)))
      (Variables|Default|SetStoredCharge_Current (Math|Float|Floor (+ _grantedamt (Math|Conversions|ToFloat(Integer) (Variables|Default|GetStoredCharge_Current)))) false)))
  (return (LocalVariables|GetChargePulled_GCV)))

(fn HandleGetVivariumCharge
  (params (PC :type Player%20Controller%20Object%20Reference))
  (bind _returnvalue (Utilities|Time|GetGameTimeinSeconds))
  (bind _cooldown (CallFunction|SPGetConfigSetting-Pull (Game|GetGameMode)))
  (if (> _returnvalue (+ (Variables|Default|GetLastPullTime) _cooldown))
    (Variables|Default|SetLastPullTime _returnvalue)
    (bind _chargepulled (CallFunction|GetChargefromVivariums))
    (if (> _chargepulled 0.0)
      (Class|PrimalActor|MulticastProperty "StoredCharge_Current" false)
      (CallFunction|SPMessageClient PC (Utilities|String|BuildString(Integer) "" "" (Math|Float|Floor _chargepulled) " charge pulled.")))
    (else
      (CallFunction|SPMessageClient PC "There is a delay between pull attempts."))))

(fn GetInterval
  (return (Math|Float|SelectFloat (Math|Random|RandomFloatinRange 45.0 6e+01) 5.0 (Class|VictoryCore|IsShipping))))

(fn OnRepPullRange
  (bind _pullrange (Variables|Default|GetPullRange))
  (Class|KismetSystemLibrary|CanRunCosmeticEvents
    (:Yes
      (Transformation|SetWorldScale3D (Variables|Default|GetRangeMesh) (Math|Vector|MakeVector _pullrange _pullrange _pullrange)))))