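; Seatable toilet structure, apparently for ARK, that captures a sitter's poop and flushes it into compost fertilizer when irrigated.
; Pooping stores the item in its inventory, applies an XP buff, plays animation and sounds, and spoils any raw meat inside.
; The stored poop drives HasPoop, which blocks seating, shows the poop mesh and offers the Flush option.
; Flushing plays effects and gives the player compost; container activation toggles the water plane.
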(event Custom|NetFlushedToilet
  (bind _returnvalue (VehicleSound|GetRootComponent))
  (Utilities|SwitchNetAuthority
    (:PlayerServer
      _)
    (:Client
      _))
  (Effects|SpawnEmitterAttached "/Game/PrimalEarth/Effects/Particles/Water/ToiletFlush.ToiletFlush" _returnvalue "None" "0, 0,46.000000")
  (Audio|SpawnSoundAttached "/Game/PrimalEarth/Sound/SFX/HumanMale/WaterSFX/ToiletFlush.ToiletFlush" _returnvalue "None" "0, 0, 0" "0, 0, 0" "KeepRelativeOffset" true 1.0 1.0 0.0 0 0))

(fn ConstructionScript
  (|CallParentFunction))

(fn BPContainerDeactivated
  (Utilities|SwitchNetAuthority
    (:PlayerServer
      _)
    (:Client
      _))
  (Rendering|SetVisibility (Variables|Default|GetWaterPlane) false false))

(fn BPContainerActivated
  (Utilities|SwitchNetAuthority
    (:PlayerServer
      _)
    (:Client
      _))
  (Rendering|SetVisibility (Variables|Default|GetWaterPlane) true false))

(fn BPNotifyInventoryItemChange
  (params (bIsItemAdd :type Boolean) (theItem :type Primal%20Item%20Object%20Reference) (bEquipItem :type Boolean))
  (Networking|SwitchHasAuthority
    (:Authority
      (Utilities|Casting|CastToPrimalItemConsumable_HumanPoop theItem)
      (bind _returnvalue (Class|PrimalInventoryComponent|GetItemTemplateQuantity (Variables|Default|GetMyInventoryComponent) "/Game/PrimalEarth/CoreBlueprints/Items/Consumables/PrimalItemConsumable_HumanPoop.PrimalItemConsumable_HumanPoop_C" 0 true false false false))
      (Variables|Default|SetbHasPoop (> _returnvalue 0) true))))

(fn OnRepBHasPoop
  (Utilities|SwitchNetAuthority
    (:PlayerServer
      _)
    (:Client
      _))
  (Rendering|SetVisibility (Variables|Default|GetPoopMesh) (Variables|Default|GetbHasPoop) false)
  (Rendering|SetVisibility (Variables|Default|GetWaterPlane) (Variables|Default|GetbContainerActivated) false))

(fn ReceiveBeginPlay
  (CallFunction|OnRepBHasPoop))

(fn BPUnstasis
  (CallFunction|OnRepBHasPoop))

(fn BPHandleSitterPoop
  (params (ForSitter :type Shooter%20Character%20Object%20Reference))
  (bind _myinventorycomponent (Variables|Default|GetMyInventoryComponent))
  (Utilities|FlowControl|Sequence
    (:then_0
      (if (not (Variables|Default|GetbHasPoop))
        (LocalVariables|SetbRetVal true)
        (Variables|/Script/ShooterGame.PrimalCharacter|SetbDontActuallyEmitPoop ForSitter true)
        (bind _returnvalue (Class|PrimalCharacter|GetCharacterStatusComponent ForSitter))
        (Variables|/Script/ShooterGame.PrimalCharacterStatusComponent|SetPoopItemFoodConsumptionCache _returnvalue 0.0)
        (Class|PrimalCharacterStatusComponent|ServerSyncReplicatedValues _returnvalue)
        (Class|PrimalInventoryComponent|BPIncrementItemTemplateQuantity _myinventorycomponent "/Game/PrimalEarth/CoreBlueprints/Items/Consumables/PrimalItemConsumable_HumanPoop.PrimalItemConsumable_HumanPoop_C" 1 true false false false false false 0 false)
        (Utilities|FlowControl|Sequence
          (:then_0
            (bind _returnvalue_2 (Class|PrimalBuff|StaticAddBuff "/QoLPlus/Misc/Toilet/Buff_ToiletXP.Buff_ToiletXP_C" ForSitter 0 0 false))
            (bind _asbuff_toilet_xp (Utilities|Casting|CastToBuff_ToiletXP _returnvalue_2))
            (Default|ResetPoopEmissionEvent _asbuff_toilet_xp))
          (:then_1
            (Class|PrimalCharacter|PlayAnimEx ForSitter (Variables|/Script/ShooterGame.PrimalCharacter|GetPoopAnimation ForSitter) 1.0 "None" true true false true false 0.0 0.0)
            (Class|Actor|ActorPlaySound ForSitter (select (Variables|/Script/ShooterGame.ShooterCharacter|GetbIsFemale ForSitter) 0 0) true "None" "0, 0, 0")
            (Class|Actor|ActorPlaySound "/Game/PrimalEarth/Sound/SFX/HumanMale/WaterSFX/ToiletSplash_Cue.ToiletSplash_Cue" true "None" "0, 0, 0"))
          (:then_2
            (bind _returnvalue_3 (Class|PrimalInventoryComponent|GetItemTemplateQuantity _myinventorycomponent "/Game/PrimalEarth/CoreBlueprints/Items/Consumables/PrimalItemConsumable_RawMeat.PrimalItemConsumable_RawMeat_C" 0 true false false false))
            (if (> _returnvalue_3 0)
              (Class|PrimalInventoryComponent|BPIncrementItemTemplateQuantity _myinventorycomponent "/Game/PrimalEarth/CoreBlueprints/Items/Consumables/PrimalItemConsumable_RawMeat.PrimalItemConsumable_RawMeat_C" (* _returnvalue_3 -1) true false false false false false 0 false)
              (bind _outitem (CallFunction|SPGetRemappedItem "/Game/PrimalEarth/CoreBlueprints/Items/Consumables/PrimalItemConsumable_SpoiledMeat.PrimalItemConsumable_SpoiledMeat_C"))
              (Class|PrimalInventoryComponent|BPIncrementItemTemplateQuantity _myinventorycomponent _outitem _returnvalue_3 true false false false false false 0 false))))))
    (:then_1
      (return (LocalVariables|GetbRetVal)))))

(fn BPGetMultiUseEntries
  (params (ForPC :type Player%20Controller%20Object%20Reference) (MultiUseEntries :type Array%20of%20Multi%20Use%20Entry%20Structures))
  (bind _bcontaineractivated (Variables|Default|GetbContainerActivated))
  (bind _entriesout (CallFunction|SPUpdateMultiUseMenu ForPC MultiUseEntries self false false false false))
  (Utilities|FlowControl|Sequence
    (:then_0
      (if (Variables|Default|GetbHasPoop)
        (Utilities|Array|Add _entriesout (Utilities|Struct|MakeMultiUseEntry (Utilities|String|SelectString "Flush" "Flush (Requires Irrigation)" _bcontaineractivated) 454214 999999 (not _bcontaineractivated) true))))
    (:then_1
      (return _entriesout))))

(fn BPTryMultiUse
  (params (ForPC :type Player%20Controller%20Object%20Reference) (UseIndex :type Integer))
  (Utilities|FlowControl|Sequence
    (:then_0
      (switch int UseIndex
        (:454214
          (if (Variables|Default|GetbContainerActivated)
            (bind _asshooter_player_controller (Utilities|Casting|CastToShooterPlayerController ForPC))
            (Utilities|IsValid (Class|ShooterPlayerController|GetPlayerCharacter _asshooter_player_controller)
              (:Is%20Valid
                (CallFunction|NetFlushedToilet)
                (Class|PrimalInventoryComponent|BPIncrementItemTemplateQuantity (Variables|Default|GetMyInventoryComponent) "/Game/PrimalEarth/CoreBlueprints/Items/Consumables/PrimalItemConsumable_HumanPoop.PrimalItemConsumable_HumanPoop_C" -1000 true false true false false false 0 false)
                (Class|PrimalInventoryComponent|BPIncrementItemTemplateQuantity (Variables|/Script/ShooterGame.PrimalCharacter|GetMyInventoryComponent (Class|ShooterPlayerController|GetPlayerCharacter _asshooter_player_controller)) "/Game/PrimalEarth/CoreBlueprints/Items/Consumables/PrimalItemConsumable_Fertilizer_Compost.PrimalItemConsumable_Fertilizer_Compost_C" 1 true false true false false false 0 false)))))))
    (:then_1
      (return true))))

(fn BPSeatedPlayer
  (params (SeatedChar :type Shooter%20Character%20Object%20Reference) (AtSeatNumber :type Integer))
  (if (not (Class|VictoryCore|IsShipping))
    (Networking|SwitchHasAuthority)))

(fn BPAllowSeating
  (params (ForPC :type Shooter%20Player%20Controller%20Object%20Reference))
  (return (not (Variables|Default|GetbHasPoop))))