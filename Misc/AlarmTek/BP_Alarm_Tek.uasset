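; S+ Tek alarm structure that extends its parent's area detection and activation, with a config-driven per-tribe build limit.
; Per-team custom actor lists track placed alarms for the limit, and a same-team menu entry toggles replicated mesh visibility unless config disables hiding.
; Detection stores an allied player's controller as LastPC.
; The activation override resolves a PIN and checks for Transfer Control Units, but its PIN-consume call is unwired, leaving activation to the parent.
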(event Custom|HandleBeginPlayEvent
  (Utilities|FlowControl|Delay 0 1.0)
  (CallFunction|SPAddtoCustomActorList self (Utilities|String|BuildString(Integer) (Variables|Default|GetActorListName) "" (Variables|Default|GetTargetingTeam))))

(fn ConstructionScript
  (|CallParentFunction))

(fn OnRepIsHidden
  (if (not (Networking|IsDedicatedServer))
    (Rendering|SetVisibility (Variables|Default|GetMyStaticMesh) (or (Variables|Default|GetDisableHide) (not (Variables|Default|GetIsHidden))) false)))

(fn ReceiveBeginPlay
  (bind _returnvalue (Game|GetGameMode))
  (|CallParentFunction)
  (if (not (Variables|Default|GetbIsPreviewStructure))
    (Networking|SwitchHasAuthority
      (:Authority
        (Utilities|FlowControl|Sequence
          (:then_0
            (bind _disablehide (CallFunction|SPGetConfigSetting-Hide _returnvalue))
            (Variables|Default|SetDisableHide _disablehide true))
          (:then_1
            (bind _value (CallFunction|SPGetConfig-Int _returnvalue (Variables|Default|GetLimitConfigName) 0 0 999999))
            (Variables|Default|SetTribeLimit _value)
            (if (> _value 0)
              (CallFunction|HandleBeginPlayEvent)))
          (:then_2
            (if (and (Variables|Default|GetIsHidden) (CallFunction|SPHasStructureDecayed self))
              (Variables|Default|SetIsHidden false true)))
          (:then_3
            (Utilities|SwitchNetAuthority
              (:PlayerServer
                (CallFunction|OnRepIsHidden)))))))))

(fn BPServerHandleNetExecCommand
  (params (FromPC :type Player%20Controller%20Object%20Reference) (CommandName :type Name :default "None") (ExecParams :type BP%20Net%20Exec%20Params%20Structure%20%28by%20ref%29))
  (Utilities|FlowControl|Sequence
    (:then_0
      (switch name CommandName
        (:SetHidden
          (Variables|Default|SetIsHidden (Math|Conversions|ToBoolean(Integer) (.IntParam1 (Utilities|Struct|BreakBPNetExecParams ExecParams))) true))))
    (:then_1
      (return true))))

(fn BPGetMultiUseEntries
  (params (ForPC :type Player%20Controller%20Object%20Reference) (MultiUseEntries :type Array%20of%20Multi%20Use%20Entry%20Structures))
  (bind _returnvalue (|CallParentFunction ForPC MultiUseEntries))
  (bind _entriesout (CallFunction|SPUpdateMultiUseMenu ForPC _returnvalue self false false false false))
  (Utilities|FlowControl|Sequence
    (:then_0
      (if (and (== (Variables|/Script/Engine.Actor|GetTargetingTeam ForPC) (Variables|Default|GetTargetingTeam)) (not (Variables|Default|GetDisableHide)))
        (Utilities|Array|Add _entriesout (Utilities|Struct|MakeMultiUseEntry (Utilities|String|SelectString "Show" "Hide" (Variables|Default|GetIsHidden)) 9001 -1001))))
    (:then_1
      (return _entriesout))))

(fn BPTryMultiUse
  (params (ForPC :type Player%20Controller%20Object%20Reference) (UseIndex :type Integer))
  (Utilities|FlowControl|Sequence
    (:then_0
      (switch int UseIndex
        (:Default
          (|CallParentFunction ForPC UseIndex))
        (:9001
          (Variables|Default|SetIsHidden (not (Variables|Default|GetIsHidden)) true))))
    (:then_1
      (return true))))

(fn BPIsAllowedtoBuildEx
  (params (OutPlacementData :type Placement%20Data%20Structure%20%28by%20ref%29) (CurrentAllowedReason :type Integer) (PC :type Player%20Controller%20Object%20Reference) (bFinalPlacement :type Boolean) (bChoosingRotation :type Boolean))
  (bind _buildreason (CallFunction|SPCheckTribeLimit self (Variables|Default|GetStructureName) CurrentAllowedReason (Variables|Default|GetTribeLimit) (Utilities|String|BuildString(Integer) (Variables|Default|GetActorListName) "" (Variables|Default|GetTargetingTeam)) bFinalPlacement PC))
  (return _buildreason))

(fn ReceiveDestroyed
  (|CallParentFunction)
  (Networking|SwitchHasAuthority
    (:Authority
      (if (not (Variables|Default|GetbIsPreviewStructure))
        (CallFunction|SPRemovefromCustomActorList self (Utilities|String|BuildString(Integer) (Variables|Default|GetActorListName) "" (Variables|Default|GetTargetingTeam)))))))

(fn BPonStructurePickup
  (params (PlayerController :type Player%20Controller%20Object%20Reference) (ItemType :type Primal%20Item%20Class%20Reference) (NewlyPickedUpItem :type Primal%20Item%20Object%20Reference) (bIsQuickPickup :type Boolean))
  (Networking|SwitchHasAuthority
    (:Authority
      (CallFunction|SPRemovefromCustomActorList self (Utilities|String|BuildString(Integer) (Variables|Default|GetActorListName) "" (Variables|Default|GetTargetingTeam))))))

(fn HasFilteredTargetintheArea
  (bind _targetlost (|CallParentFunction))
  (Utilities|FlowControl|Sequence
    (:then_0
      (if _targetlost
        (bind (_radius _location) (CallFunction|GetOctreeDataforTargetDetectArea))
        (bind _value (CallFunction|GetOctreeCheckType))
        (bind _returnvalue (Class|VictoryCore|ServerOctreeOverlapActors (Class|PrimalActor|GetWorld) _location _radius _value (not (CallFunction|IsTargetDetectBox))))
        (bind _array_element (Utilities|Array|ForEachLoopwithBreak _returnvalue :!label _label)
          (:LoopBody
            (bind _asprimal_character (Utilities|Casting|CastToPrimalCharacter _array_element))
            (if (Class|PrimalCharacter|IsAlive _asprimal_character)
              (if (CallFunction|IsTargetDetectBox)
                (bind _value_2 (CallFunction|IsActorinBoxArea _asprimal_character (Variables|Default|GetTargetDetectBox)))
                (if _value_2
                  (bind _asshooter_character (Utilities|Casting|CastToShooterCharacter _asprimal_character :!label _label_2))
                  (bind _returnvalue_2 (Class|PrimalCharacter|IsAlliedwithOtherTeam _asshooter_character (Variables|Default|GetTargetingTeam)))
                  (if _returnvalue_2
                    (bind _returnvalue_3 (Class|Actor|GetOwnerController _asshooter_character))
                    (Variables|Default|SetLastPC _returnvalue_3)
                    (goto _label Break)))
                (else
                  (goto _label_2))))))))
    (:then_1
      (return _targetlost))))

(fn SetActivateStatetoStructure
  (params (PrimalStructure :type Primal%20Structure%20Object%20Reference) (Toggle :type Boolean) (NewActivateState :type Boolean) (Force :type Boolean))
  (Utilities|FlowControl|Sequence
    (:then_0
      (if (Math|Boolean|ORBoolean (Variables|Default|GetShouldToggle) Force (CallFunction|HasPendingPINActivation))
        (LocalVariables|SetActivePin_SAS (.PINCode (Utilities|Struct|BreakTekAlarmPINData (CallFunction|GetPINDatabyType "NewEnumerator2"))))
        (Utilities|FlowControl|Sequence
          (:then_0
            (if (== (LocalVariables|GetActivePin_SAS) 0)
              (LocalVariables|SetActivePin_SAS (.PINCode (Utilities|Struct|BreakTekAlarmPINData (CallFunction|GetPINDatabyType "NewEnumerator0"))))))
          (:then_1
            (if (> (LocalVariables|GetActivePin_SAS) 0)
              (Utilities|IsValid (Variables|Default|GetLastPC)
                (:Is%20Valid
                  (bind _asprimal_structure_item_container (Utilities|Casting|CastToPrimalStructureItemContainer PrimalStructure))
                  (if (Actor|ActorHasTag _asprimal_structure_item_container "SPlus_TransferControlUnit")
                    _))))))))
    (:then_1
      (|CallParentFunction PrimalStructure Toggle NewActivateState Force))))