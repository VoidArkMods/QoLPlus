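; Structures Plus Element Catalyzer, a crafting structure that by default must be placed in liquid Element.
; Placement checks use a sphere overlap to find an element-pool pain volume enclosing the placement point, otherwise returning a custom can't-build reason.
; A global-actor setting lifts that requirement and permits saddle attachment; without it, server-side activation is blocked on saddles.
; Crafting speed comes from server config at BeginPlay.
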(fn ConstructionScript
  (|CallParentFunction)
  (bind _assplus_global_actor (Utilities|Casting|CastToSPlusGlobalActor (CallFunction|SPGetGlobalActor self)))
  (Variables|Default|SetAllowOutsideOfElement (Variables|/QoLPlus/SPlusGlobalActor.SPlusGlobalActor_C|GetAllowElementCatalyzerOutOfElement _assplus_global_actor))
  (if (Variables|/QoLPlus/SPlusGlobalActor.SPlusGlobalActor_C|GetAllowElementCatalyzerOutOfElement _assplus_global_actor)
    (Variables|Default|SetbAllowAttachToSaddle true)
    (Variables|Default|SetbPreventAttachToSaddle false)))

(fn BPGetMultiUseEntries
  (params (ForPC :type Player%20Controller%20Object%20Reference) (MultiUseEntries :type Array%20of%20Multi%20Use%20Entry%20Structures))
  (bind _entriesout (CallFunction|SPUpdateMultiUseMenu ForPC MultiUseEntries self false false false false))
  (return _entriesout))

(fn ReceiveBeginPlay
  (|CallParentFunction)
  (if (not (Variables|Default|GetbIsPreviewStructure))
    (Networking|SwitchHasAuthority
      (:Authority
        (bind _value (CallFunction|SPGetConfigSetting-CraftingSpeed (Game|GetGameMode) "ElementCatalyzerCraftingSpeed"))
        (Variables|/Script/ShooterGame.PrimalInventoryComponent|SetCraftingItemSpeed (Variables|Default|GetMyInventoryComponent) _value)))))

(fn BPIsAllowedtoBuildEx
  (params (OutPlacementData :type Placement%20Data%20Structure%20%28by%20ref%29) (CurrentAllowedReason :type Integer) (PC :type Player%20Controller%20Object%20Reference) (bFinalPlacement :type Boolean) (bChoosingRotation :type Boolean))
  (LocalVariables|SetBuildReason CurrentAllowedReason)
  (Utilities|FlowControl|Sequence
    (:then_0
      (if (== (LocalVariables|GetBuildReason) 1)
        (LocalVariables|SetBuildReason (Math|Integer|SelectInt 1 -100 (or (Variables|Default|GetAllowOutsideOfElement) (CallFunction|IsinElement (.AdjustedLocation (Utilities|Struct|BreakPlacementData OutPlacementData))))))))
    (:then_1
      (return (LocalVariables|GetBuildReason)))))

(fn BPOverrideCantBuildReasonString
  (params (CantBuildReason :type Integer))
  (return (Utilities|String|SelectString "Must be placed in liquid Element" "" (== CantBuildReason -100))))

(fn IsinElement
  (params (Location :type Vector))
  (Utilities|FlowControl|Sequence
    (:then_0
      (bind (_outactors _returnvalue) (Class|KismetSystemLibrary|SphereOverlapActorsSimple 0 Location 115.0 "ObjectTypeQuery14" "/Script/Engine.PainCausingVolume" (Utilities|Array|MakeArray)))
      (if _returnvalue
        (bind _array_element (Utilities|Array|ForEachLoopwithBreak _outactors :!label _label)
          (:LoopBody
            (bind _aspain_causing_volume (Utilities|Casting|CastToPainCausingVolume _array_element))
            (if (and (.ReturnValue (Class|Volume|BPEncompassesPoint _aspain_causing_volume Location 1.0)) (== (Variables|/Script/Engine.PainCausingVolume|GetDamageType _aspain_causing_volume) "/Game/PrimalEarth/CoreBlueprints/DamageTypes/DmgType_ElementPool.DmgType_ElementPool_C"))
              (LocalVariables|SetretVal true)
              (goto _label Break))))))
    (:then_1
      (return (LocalVariables|GetretVal)))))

(fn BPCanbeActivated
  (LocalVariables|SetAllowActivation_CBA true)
  (Utilities|FlowControl|Sequence
    (:then_0
      (Networking|SwitchHasAuthority
        (:Authority
          (bind _assplus_global_actor (Utilities|Casting|CastToSPlusGlobalActor (CallFunction|SPGetGlobalActor self)))
          (if (not (Variables|/QoLPlus/SPlusGlobalActor.SPlusGlobalActor_C|GetAllowElementCatalyzerOutOfElement _assplus_global_actor))
            (LocalVariables|SetAllowActivation_CBA (not (Utilities|IsValid (Variables|Default|GetSaddleDino))))))))
    (:then_1
      (return (LocalVariables|GetAllowActivation_CBA)))))