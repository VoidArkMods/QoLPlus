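; S+ Hatchery structure that collects ground eggs, incubates them and gives an Oviraptor egg boost, with server-configured slots, range and multiplier.
; While activated, a looping DoScan timer incubates each tick and staggers collection and boost through a cycling index.
; Multi-use entries toggle collection and edit ignore/destroy lists via an aggregator buff UI and net exec commands.
; Replicated egg state drives Dodo animation and randomly sampled egg materials; chibi skins replace the Dodo mesh.
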(event Custom|DelayedEggMeshUpdateEvent
  (if (Variables|Default|GetAreEggsVisible)
    (bind _returnvalue (Class|PrimalInventoryComponent|FindAllItemsOfType (Variables|Default|GetMyInventoryComponent) "/Game/PrimalEarth/CoreBlueprints/Items/Consumables/PrimalItemConsumable_Egg.PrimalItemConsumable_Egg_C" false true false false false false false))
    (for _index (range 0 3)
      (Utilities|Array|SetArrayElem (Variables|Default|GetEggMaterials) _index (Variables|/Script/ShooterGame.PrimalItem|GetDroppedMeshMaterialOverride (Utilities|Array|Get(acopy) _returnvalue (Math|Random|RandomIntegerinRange 0 (Utilities|Array|LastIndex _returnvalue))))))
    (Class|PrimalActor|MulticastProperty "EggMaterials" false)))

(fn ConstructionScript
  (|CallParentFunction))

(fn OnRepAreEggsVisible
  (bind _areeggsvisible (Variables|Default|GetAreEggsVisible))
  (bind _dodo (Variables|Default|GetDodo))
  (Utilities|FlowControl|Sequence
    (:then_0
      (Networking|SwitchHasAuthority
        (:Authority
          (if (Variables|Default|GetAreEggsVisible)
            (Utilities|Time|SetTimerbyFunctionName 0 "DelayedEggMeshUpdateEvent" 2.0)))))
    (:then_1
      (Class|KismetSystemLibrary|CanRunCosmeticEvents
        (:Yes
          (Rendering|SetVisibility (Variables|Default|GetEggs) (Variables|Default|GetAreEggsVisible) true)
          (Components|Animation|PlayAnimation _dodo (select _areeggsvisible (Variables|Default|GetIncubatingAnimation) (Variables|Default|GetIdleAnimation)) true)
          (Variables|/Script/Engine.SkeletalMeshComponent|SetGlobalAnimRateScale _dodo (Math|Float|SelectFloat 0.25 1.0 _areeggsvisible))
          (Variables|/Script/Engine.SkeletalMeshComponent|SetbPauseAnims _dodo (not (Variables|Default|GetbContainerActivated))))))))

(fn BPServerHandleNetExecCommand
  (params (FromPC :type Player%20Controller%20Object%20Reference) (CommandName :type Name :default "None") (ExecParams :type BP%20Net%20Exec%20Params%20Structure%20%28by%20ref%29))
  (Utilities|FlowControl|Sequence
    (:then_0
      (Utilities|IsValid FromPC
        (:Is%20Valid
          (bind _assplus_misc_com_object (Utilities|Casting|CastToSPlus_Misc_ComObject (.ObjParam1 (Utilities|Struct|BreakBPNetExecParams ExecParams))))
          (switch name CommandName
            (:HatcherySetBlackList
              (Variables|Default|SetCollectionBlacklist (Variables|/QoLPlus/_ComObjects/SPlus_Misc_ComObject.SPlus_Misc_ComObject_C|GetObjectClasses _assplus_misc_com_object)))
            (:HatcherySetDestroyList
              (Variables|Default|SetCollectionDestroylist (Variables|/QoLPlus/_ComObjects/SPlus_Misc_ComObject.SPlus_Misc_ComObject_C|GetObjectClasses _assplus_misc_com_object)))))))
    (:then_1
      (return true))))

(fn ReceiveBeginPlay
  (bind _returnvalue (Game|GetGameMode))
  (|CallParentFunction)
  (if (not (Variables|Default|GetbIsPreviewStructure))
    (Utilities|FlowControl|Sequence
      (:then_0
        (Class|KismetSystemLibrary|CanRunCosmeticEvents
          (:Yes
            (bind _returnvalue_2 (Class|PrimalInventoryComponent|GetEquippedItemOfClass (Variables|Default|GetMyInventoryComponent) "/Game/PrimalEarth/CoreBlueprints/Items/Armor/Skin/ChibiDinos/PrimalItemSkin_ChibiDino_Base.PrimalItemSkin_ChibiDino_Base_C"))
            (CallFunction|UpdateDefaultMesh (not (Utilities|IsValid _returnvalue_2)))
            (Utilities|SwitchNetAuthority
              (:PlayerServer
                (CallFunction|OnRepAreEggsVisible))))))
      (:then_1
        (Networking|SwitchHasAuthority
          (:Authority
            (Utilities|FlowControl|Sequence
              (:then_0
                (bind _value (CallFunction|SPGetConfigSetting-InventorySize _returnvalue "HatcherySlotCount" 50))
                (Variables|Default|SetInvSlotOverride _value true))
              (:then_1
                (bind _value_2 (CallFunction|SPGetConfig-Int _returnvalue "HatcheryRangeInFoundations" 25 1 100))
                (Variables|Default|SetScanRadius (* _value_2 3e+02) true))
              (:then_2
                (bind _value_3 (CallFunction|SPGetConfig-Float _returnvalue "HatcheryIncubationMultiplier" 1.0 0.01 999999.0))
                (Variables|Default|SetIncubationMultiplier _value_3))
              (:then_3
                (bind _value_4 (CallFunction|SPGetConfig-Bool _returnvalue "DisableHatcheryOviBonus"))
                (Variables|Default|SetDisableOviEggBoost _value_4))
              (:then_4
                (Utilities|Struct|SetmembersinSP_ItemCollectorCollectData (Variables|Default|GetCollectData_Ground) true)))))))))

(fn BPGetMultiUseEntries
  (params (ForPC :type Player%20Controller%20Object%20Reference) (MultiUseEntries :type Array%20of%20Multi%20Use%20Entry%20Structures))
  (bind _color (CallFunction|SPGetMultiUseSpecialColor))
  (bind _returnvalue (Math|Conversions|ToColor(LinearColor) _color))
  (bind _returnvalue_2 (|CallParentFunction ForPC MultiUseEntries))
  (Utilities|FlowControl|Sequence
    (:then_0
      (if (== (Variables|/Script/Engine.Actor|GetTargetingTeam ForPC) (Variables|Default|GetTargetingTeam))
        (Utilities|Array|Add _returnvalue_2 (Utilities|Struct|MakeMultiUseEntry (Utilities|String|SelectString "Start Collecting Eggs" "Stop Collecting Eggs" (Variables|Default|GetDisableEggCollection)) 9003 -1006))
        (Utilities|Array|Add _returnvalue_2 (Utilities|Struct|MakeMultiUseEntry "[View Ignore List]" 9004 -450 true true false 0 _returnvalue))
        (Utilities|Array|Add _returnvalue_2 (Utilities|Struct|MakeMultiUseEntry "[View Destroy List]" 9005 -500 true true false 0 _returnvalue))))
    (:then_1
      (return _returnvalue_2))))

(fn BPTryMultiUse
  (params (ForPC :type Player%20Controller%20Object%20Reference) (UseIndex :type Integer))
  (|CallParentFunction ForPC UseIndex)
  (Utilities|FlowControl|Sequence
    (:then_0
      (switch int UseIndex
        (:9003
          (Variables|Default|SetDisableEggCollection (not (Variables|Default|GetDisableEggCollection)) true))
        (:9004
          (bind _asshooter_player_controller (Utilities|Casting|CastToShooterPlayerController ForPC))
          (bind _returnvalue (Class|PrimalBuff|StaticAddBuff "/QoLPlus/_Buffs/Buff_StructuresPlus_ItemAggregator.Buff_StructuresPlus_ItemAggregator_C" (Class|ShooterPlayerController|GetPlayerCharacter _asshooter_player_controller) 0 0 false))
          (bind _asbuff_structures_plus_item_aggregator (Utilities|Casting|CastToBuff_StructuresPlus_ItemAggregator _returnvalue))
          (Default|InitializeUI-SelectList _asbuff_structures_plus_item_aggregator "Eggs to Ignore" "HatcherySetBlackList" self (Variables|Default|GetCollectionBlacklist)))
        (:9005
          (bind _asshooter_player_controller_2 (Utilities|Casting|CastToShooterPlayerController ForPC))
          (bind _returnvalue_2 (Class|PrimalBuff|StaticAddBuff "/QoLPlus/_Buffs/Buff_StructuresPlus_ItemAggregator.Buff_StructuresPlus_ItemAggregator_C" (Class|ShooterPlayerController|GetPlayerCharacter _asshooter_player_controller_2) 0 0 false))
          (bind _asbuff_structures_plus_item_aggregator_2 (Utilities|Casting|CastToBuff_StructuresPlus_ItemAggregator _returnvalue_2))
          (Default|InitializeUI-SelectList _asbuff_structures_plus_item_aggregator_2 "Eggs to Destroy" "HatcherySetDestroyList" self (Variables|Default|GetCollectionDestroylist)))))
    (:then_1
      (return true))))

(fn DoScan
  (if (Variables|Default|GetbContainerActivated)
    (Utilities|FlowControl|Sequence
      (:then_0
        (if (not (Variables|Default|GetDisableIncubation))
          (CallFunction|IncubateEggs)))
      (:then_1
        (switch int (Variables|Default|GetSecondaryScanIndex)
          (:0
            (if (not (Variables|Default|GetDisableEggCollection))
              (CallFunction|Collect-Ground)))
          (:1
            (if (not (Variables|Default|GetDisableOviEggBoost)) :!label _label
              (CallFunction|GiveOviEggBoost)))
          (:3
            (goto _label))))
      (:then_2
        (Variables|Default|SetSecondaryScanIndex (Math|Integer|SelectInt 0 (+ (Variables|Default|GetSecondaryScanIndex) 1) (> (+ (Variables|Default|GetSecondaryScanIndex) 1) 3))))
      (:then_3
        (Utilities|Time|SetTimerbyFunctionName 0 "DoScan" (CallFunction|GetScanInterval))))))

(fn BPNotifyInventoryItemChange
  (params (bIsItemAdd :type Boolean) (theItem :type Primal%20Item%20Object%20Reference) (bEquipItem :type Boolean))
  (Utilities|FlowControl|Sequence
    (:then_0
      (Networking|SwitchHasAuthority
        (:Authority
          (Utilities|Casting|CastToPrimalItemConsumable_Egg theItem)
          (if (Math|Boolean|NotEqual(Boolean) bIsItemAdd (Variables|Default|GetAreEggsVisible))
            (bind _qty (CallFunction|GetItemQty (Variables|Default|GetMyInventoryComponent) "/Game/PrimalEarth/CoreBlueprints/Items/Consumables/PrimalItemConsumable_Egg.PrimalItemConsumable_Egg_C" false))
            (Variables|Default|SetAreEggsVisible (> _qty 0) true)))))
    (:then_1
      (if (or bIsItemAdd bEquipItem)
        (Utilities|Casting|CastToPrimalItemSkin_ChibiDino_Base theItem)
        (Class|KismetSystemLibrary|CanRunCosmeticEvents
          (:Yes
            (Utilities|FlowControl|Sequence
              (:then_0
                (bind _returnvalue (Class|PrimalInventoryComponent|GetEquippedItemOfClass (Variables|Default|GetMyInventoryComponent) "/Game/PrimalEarth/CoreBlueprints/Items/Armor/Skin/ChibiDinos/PrimalItemSkin_ChibiDino_Base.PrimalItemSkin_ChibiDino_Base_C"))
                (CallFunction|UpdateDefaultMesh (not (Utilities|IsValid _returnvalue))))
              (:then_1
                (if bEquipItem
                  (Class|KismetSystemLibrary|SetTimerforNextTick 0 "UpdateChibi" false))))))))))

(fn UpdateChibi
  (bind _returnvalue (Transformation|GetActorRotation))
  (Utilities|IsValid (Actor|GetComponentbyClass "/Game/PrimalEarth/CoreBlueprints/Items/Armor/Skin/ChibiDinos/SKComponent_SkinAttachment_ChibiDino.SKComponent_SkinAttachment_ChibiDino_C")
    (:Is%20Valid
      (for _array_element (Actor|GetComponentsByClass "/Game/PrimalEarth/CoreBlueprints/Items/Armor/Skin/ChibiDinos/SKComponent_SkinAttachment_ChibiDino.SKComponent_SkinAttachment_ChibiDino_C")
        (bind _asskcomponent_skin_attachment_chibi_dino (Utilities|Casting|CastToSKComponent_SkinAttachment_ChibiDino _array_element))
        (Utilities|FlowControl|Sequence
          (:then_0
            (if (not (Variables|/Game/PrimalEarth/CoreBlueprints/Items/Armor/Skin/ChibiDinos/SKComponent_SkinAttachment_ChibiDino.SKComponent_SkinAttachment_ChibiDino_C|GetSubMeshesAdded _asskcomponent_skin_attachment_chibi_dino))
              (Default|AttachSubMeshes _asskcomponent_skin_attachment_chibi_dino)))
          (:then_1
            (Variables|/Script/Engine.SkeletalMeshComponent|SetbPauseAnims _asskcomponent_skin_attachment_chibi_dino (not (Variables|Default|GetbContainerActivated)))
            (bind (_scale _locoffset _rotoffset) (CallFunction|GetChibiTransform _asskcomponent_skin_attachment_chibi_dino))
            (Transformation|SetWorldTransform _asskcomponent_skin_attachment_chibi_dino (Math|Transform|MakeTransform (+ (Math|Vector|RotateVector _locoffset _returnvalue) (Math|Vector|RotateVector (Variables|/Game/PrimalEarth/CoreBlueprints/Items/Armor/Skin/ChibiDinos/SKComponent_SkinAttachment_ChibiDino.SKComponent_SkinAttachment_ChibiDino_C|GetGroundedPositionOffset _asskcomponent_skin_attachment_chibi_dino) _returnvalue) (Math|Vector|RotateVector "0, 0,40.000000" _returnvalue) (Transformation|GetActorLocation)) (Math|Rotator|CombineRotators (Math|Rotator|CombineRotators _rotoffset _returnvalue) "0,90.000000, 0") (* _scale 2.0)) false false)
            (Rendering|SetVisibility _asskcomponent_skin_attachment_chibi_dino true true)))))
    (:Is%20Not%20Valid
      (Class|KismetSystemLibrary|SetTimerforNextTick 0 "UpdateChibi" false))))

(fn UpdateDefaultMesh
  (params (Show :type Boolean))
  (Class|KismetSystemLibrary|CanRunCosmeticEvents
    (:Yes
      (Rendering|SetVisibility (Variables|Default|GetDefaultMeshScene) Show true)
      (Variables|/Script/Engine.SkeletalMeshComponent|SetbPauseAnims (Variables|Default|GetDodo) (or (not Show) (not (Variables|Default|GetbContainerActivated)))))))

(fn OnRepEggMaterials
  (bind _eggmaterials (Variables|Default|GetEggMaterials))
  (Class|KismetSystemLibrary|CanRunCosmeticEvents
    (:Yes
      (Rendering|Material|SetMaterial (Variables|Default|GetEgg1) 0 (Utilities|Array|Get(acopy) _eggmaterials))
      (Rendering|Material|SetMaterial (Variables|Default|GetEgg2) 0 (Utilities|Array|Get(acopy) _eggmaterials 1))
      (Rendering|Material|SetMaterial (Variables|Default|GetEgg3) 0 (Utilities|Array|Get(acopy) _eggmaterials 2))
      (Rendering|Material|SetMaterial (Variables|Default|GetEgg4) 0 (Utilities|Array|Get(acopy) _eggmaterials 3)))))