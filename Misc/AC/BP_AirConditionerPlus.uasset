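; Structures Plus air conditioner for ARK, with configurable wireless power range, optional noise muting and custom placement rules.
; On the server it reads the game mode config, sizes its wireless exchange ranges and, after a delay, clears structure links with other units.
; During preview, Drag toggles snapping through the player's global buff.
; Placement overrides one build failure code and flags window-wall parents, which disables snapping to the unit.
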(event Custom|HandleBeginPlayEvent
  (bind _linkedstructures (Variables|Default|GetLinkedStructures))
  (Utilities|FlowControl|Delay 0 1.0)
  (Utilities|FlowControl|Sequence
    (:then_0
      (for _array_element _linkedstructures
        (Utilities|Casting|CastToBP_AirConditionerPlus _array_element)
        (Utilities|Array|Clear (Variables|/Script/ShooterGame.PrimalStructure|GetLinkedStructures _array_element)))
      (Utilities|Array|Clear _linkedstructures))
    (:then_1
      (bind _value (CallFunction|SPGetConfig-Int (Game|GetGameMode) "MaxPowerRangeInFoundations" 100 5 100))
      (for _array_element_2 (Variables|/Script/ShooterGame.PrimalInventoryComponent|GetWirelessExchanges (Variables|Default|GetPrimalInventoryBP_AC_Base_C1))
        (Variables|/Script/ShooterGame.PrimalWirelessExchangeData|SetConsumeRange _array_element_2 (* _value 3e+02))))))

(event Input|ActionEvents|InputActionDrag
  (params (Key :type Key%20Structure))
  (:Pressed
    (bind _returnvalue (Class|Actor|GetOwnerController))
    (bind _success (CallFunction|SPToggleGlobalBuffDisabledSnaps _returnvalue (Utilities|Array|MakeArray) (Utilities|Array|MakeArray 1) (not (Variables|Default|GetSnapsDisabled))))
    (if _success
      (Variables|Default|SetSnapsDisabled (not (Variables|Default|GetSnapsDisabled))))))

(fn ConstructionScript
  (|CallParentFunction)
  (if (not (Variables|Default|GetbIsPreviewStructure))
    (Networking|SwitchHasAuthority
      (:Authority
        (Utilities|FlowControl|Sequence
          (:then_0
            (bind _disablesound (CallFunction|SPGetConfigSetting-Noise (Game|GetGameMode)))
            (Variables|Default|SetDisableSound _disablesound true))
          (:then_1
            (for _array_element (Variables|/Script/ShooterGame.PrimalInventoryComponent|GetWirelessExchanges (Variables|Default|GetPrimalInventoryBP_AC_Base_C1))
              (Variables|/Script/ShooterGame.PrimalWirelessExchangeData|SetConsumeRange _array_element 3e+04))))))))

(fn BPIsAllowedtoBuild
  (params (OutPlacementData :type Placement%20Data%20Structure%20%28by%20ref%29) (CurrentAllowedReason :type Integer))
  (Variables|Default|SetIsSnappedToWindowWall (Utilities|ClassIsChildOf (Utilities|GetClass (.ParentStructure (Utilities|Struct|BreakPlacementData OutPlacementData))) "/Game/PrimalEarth/Structures/BuildingBases/WindowWall_Base_SM.WindowWall_Base_SM_C") false)
  (return (Math|Integer|SelectInt 1 CurrentAllowedReason (== CurrentAllowedReason -9))))

(fn BPGetMultiUseEntries
  (params (ForPC :type Player%20Controller%20Object%20Reference) (MultiUseEntries :type Array%20of%20Multi%20Use%20Entry%20Structures))
  (bind _entriesout (CallFunction|SPUpdateMultiUseMenu ForPC MultiUseEntries self false false false false))
  (return _entriesout))

(fn IsValidSnapPointto
  (params (ChildStructure :type Primal%20Structure%20Object%20Reference) (MySnapPointToIndex :type Integer))
  (return (not (Variables|Default|GetIsSnappedToWindowWall))))

(fn ReceiveBeginPlay
  (|CallParentFunction)
  (if (Variables|Default|GetbIsPreviewStructure)
    (bind _returnvalue (Class|Actor|GetOwnerController))
    (Input|EnableInput _returnvalue)
    (CallFunction|SPClearGlobalBuffDisabledSnaps _returnvalue)
    (else
      (Networking|SwitchHasAuthority
        (:Authority
          (CallFunction|HandleBeginPlayEvent))))))

(fn IsValidSnapPointfrom
  (params (ParentStructure :type Primal%20Structure%20Object%20Reference) (MySnapPointFromIndex :type Integer))
  (return (not (Variables|Default|GetSnapsDisabled))))

(fn BPSetPlayerConstructor
  (params (PC :type Player%20Controller%20Object%20Reference))
  (bind _asbuff_structures_plus_global_buff (Utilities|Casting|CastToBuff_StructuresPlus_GlobalBuff (CallFunction|SPGetGlobalBuff PC)))
  (Variables|Default|SetSnapsDisabled (> (Utilities|Array|Length (Variables|/QoLPlus/_Buffs/Buff_StructuresPlus_GlobalBuff.Buff_StructuresPlus_GlobalBuff_C|GetDisabledSnapsFrom _asbuff_structures_plus_global_buff)) 0))
  (CallFunction|SPClearGlobalBuffDisabledSnaps PC))

(fn OnRepDisableSound
  (if (not (Networking|IsDedicatedServer))
    (if (Variables|Default|GetDisableSound)
      (bind _asprimal_emitter_spawnable (Utilities|Casting|CastToPrimalEmitterSpawnable (Variables|/Script/Engine.ChildActorComponent|GetChildActor (Variables|Default|GetActivatedEmitter))))
      (Audio|Components|Audio|SetVolumeMultiplier (Variables|/Script/ShooterGame.PrimalEmitterSpawnable|GetSoundToPlay _asprimal_emitter_spawnable) 0.0 :!class /Script/Engine.AudioComponent))))