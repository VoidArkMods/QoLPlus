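; Structures Plus bunk bed that adds a toggleable snap-disable during placement and routes its multi-use menu through shared S+ helpers.
; The preview's Drag input flips DisableSnaps through the player's global buff, which the placed bed reads on construction before clearing it.
; The global actor can lift the floor requirement, and placement reason -9 is overridden to allowed.
; On the server, use cooldown comes from config.
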(event Input|ActionEvents|InputActionDrag
  (params (Key :type Key%20Structure :default "None"))
  (:Pressed
    (bind _returnvalue (Class|Actor|GetOwnerController))
    (bind _success (CallFunction|SPToggleGlobalBuffDisabledSnaps _returnvalue (Utilities|Array|MakeArray) (Utilities|Array|MakeArray 1) (not (Variables|Default|GetDisableSnaps))))
    (if _success
      (Variables|Default|SetDisableSnaps (not (Variables|Default|GetDisableSnaps))))))

(fn ConstructionScript
  (|CallParentFunction)
  (if (Variables|Default|GetbIsPreviewStructure)
    _
    (else
      (Networking|SwitchHasAuthority
        (:Authority
          _))))
  (bind _assplus_global_actor (Utilities|Casting|CastToSPlusGlobalActor (CallFunction|SPGetGlobalActor self)))
  (if (Variables|/QoLPlus/SPlusGlobalActor.SPlusGlobalActor_C|GetRemoveFloorRequirement _assplus_global_actor)
    (Variables|Default|SetbRequiresPlacementOnStructureFloors false)))

(fn BPGetMultiUseEntries
  (params (ForPC :type Player%20Controller%20Object%20Reference) (MultiUseEntries :type Array%20of%20Multi%20Use%20Entry%20Structures))
  (bind _entriesout (CallFunction|SPUpdateMultiUseMenu ForPC MultiUseEntries self false false false false))
  (return _entriesout))

(fn BPIsAllowedtoBuild
  (params (OutPlacementData :type Placement%20Data%20Structure%20%28by%20ref%29) (CurrentAllowedReason :type Integer))
  (return (Math|Integer|SelectInt 1 CurrentAllowedReason (== CurrentAllowedReason -9))))

(fn ReceiveBeginPlay
  (|CallParentFunction)
  (if (Variables|Default|GetbIsPreviewStructure)
    (bind _returnvalue (Class|Actor|GetOwnerController))
    (Input|EnableInput _returnvalue)
    (CallFunction|SPClearGlobalBuffDisabledSnaps _returnvalue)
    (else
      (Networking|SwitchHasAuthority
        (:Authority
          (bind _value (CallFunction|SPGetConfig-Float (Game|GetGameMode) "BunkBedCooldownTimeInSeconds" 1.2e+02 1.0 999999.0))
          (Variables|Default|SetUseCooldownTime _value))))))

(fn IsValidSnapPointfrom
  (params (ParentStructure :type Primal%20Structure%20Object%20Reference) (MySnapPointFromIndex :type Integer))
  (return (not (Variables|Default|GetDisableSnaps))))

(fn BPSetPlayerConstructor
  (params (PC :type Player%20Controller%20Object%20Reference))
  (bind _asbuff_structures_plus_global_buff (Utilities|Casting|CastToBuff_StructuresPlus_GlobalBuff (CallFunction|SPGetGlobalBuff PC)))
  (Variables|Default|SetDisableSnaps (> (Utilities|Array|Length (Variables|/QoLPlus/_Buffs/Buff_StructuresPlus_GlobalBuff.Buff_StructuresPlus_GlobalBuff_C|GetDisabledSnapsFrom _asbuff_structures_plus_global_buff)) 0))
  (CallFunction|SPClearGlobalBuffDisabledSnaps PC))