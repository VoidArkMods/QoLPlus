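; A Structures Plus standing torch structure that can light itself at night and never burns fuel.
; When auto mode is on, the server runs a looping timer that toggles the torch using day/night checks with dawn and dusk offsets; manual toggles override it until the next phase change.
; Flame particle and light colors follow structure paint and settings, which same-team players edit through a multi-tool buff.
; Zero consumption and automatic inventory top-ups keep it fueled.
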(event Custom|HandleBeginPlayEvent
  (Utilities|FlowControl|Delay 0 2.0)
  (if (.isauto (Variables|Default|GetTorchSettings))
    (Utilities|Time|SetTimerbyFunctionName 0 "CheckTime" 1e+01 true)))

(event Custom|SetLightSettingsEvent
  (params (Settings :type SP%20Light%20Settings%20Structure))
  (Variables|Default|SetTorchSettings Settings false)
  (CallFunction|UpdateTorchColor (Variables|Default|GetTorchColor))
  (Networking|SwitchHasAuthority
    (:Authority
      (Utilities|Time|ClearTimerbyFunctionName 0 "CheckTime")
      (if (.isauto (Variables|Default|GetTorchSettings))
        (Variables|Default|SetManualActivationState 0)
        (Utilities|Time|SetTimerbyFunctionName 0 "CheckTime" 1e+01 true)))))

(fn ConstructionScript)

(fn BPIsAllowedtoBuild
  (params (OutPlacementData :type Placement%20Data%20Structure%20%28by%20ref%29) (CurrentAllowedReason :type Integer))
  (return (Math|Integer|SelectInt 1 CurrentAllowedReason (== CurrentAllowedReason -9))))

(fn BPGetMultiUseEntries
  (params (ForPC :type Player%20Controller%20Object%20Reference) (MultiUseEntries :type Array%20of%20Multi%20Use%20Entry%20Structures))
  (bind _entriesout (CallFunction|SPUpdateMultiUseMenu ForPC MultiUseEntries self false false false false))
  (Utilities|FlowControl|Sequence
    (:then_0
      (if (== (Variables|/Script/Engine.Actor|GetTargetingTeam ForPC) (Variables|Default|GetTargetingTeam))
        (Utilities|Array|Add _entriesout (Utilities|Struct|MakeMultiUseEntry "[Change Settings]" 9001 -10 true false 0 (Math|Conversions|ToColor(LinearColor) (CallFunction|SPGetMultiUseSpecialColor))))))
    (:then_1
      (return _entriesout))))

(fn BPTryMultiUse
  (params (ForPC :type Player%20Controller%20Object%20Reference) (UseIndex :type Integer))
  (bind _bcontaineractivated (Variables|Default|GetbContainerActivated))
  (bind _torchsettings (Variables|Default|GetTorchSettings))
  (bind (_postdawnoffset _preduskoffset) (Utilities|Struct|BreakSPLightSettings _torchsettings))
  (Utilities|FlowControl|Sequence
    (:then_0
      (if (== UseIndex 9001)
        (CallFunction|SPApplyMultiToolBuff 3 ForPC self)))
    (:then_1
      (if (== UseIndex 600)
        (bind _isday (CallFunction|SPIsDayTime self _postdawnoffset _preduskoffset))
        (if (and _isday _bcontaineractivated)
          (Variables|Default|SetManualActivationState 1)
          (elif (and (not _isday) (not _bcontaineractivated))
            (Variables|Default|SetManualActivationState -1)
            (else
              (Variables|Default|SetManualActivationState 0))))))
    (:then_2
      (return true))))

(fn OnRepTorchColor
  (CallFunction|UpdateTorchColor (Variables|Default|GetTorchColor)))

(fn UpdateTorchColor
  (params (FlameColor :type Vector))
  (bind _returnvalue (* FlameColor 5e+01))
  (bind _returnvalue_2 (Math|Vector|MakeVector 5e+01 1e+01 2.0))
  (bind _busingstructurecolors (Variables|Default|GetbUsingStructureColors))
  (Class|KismetSystemLibrary|CanRunCosmeticEvents
    (:Yes
      (bind _asemitter_standing_torch_plus (Utilities|Casting|CastToEmitter_StandingTorchPlus (Variables|/Script/Engine.ChildActorComponent|GetChildActor (Variables|Default|GetActivatedEmitter))))
      (Effects|Components|ParticleSystem|SetVectorParameter (Variables|/Script/Engine.Emitter|GetParticleSystemComponent _asemitter_standing_torch_plus) "FlameColorA" (Math|Vector|SelectVector _returnvalue _returnvalue_2 _busingstructurecolors))
      (Effects|Components|ParticleSystem|SetVectorParameter (Variables|/Script/Engine.Emitter|GetParticleSystemComponent _asemitter_standing_torch_plus) "FlameColorB" (Math|Vector|SelectVector _returnvalue _returnvalue_2 _busingstructurecolors))
      (Effects|Components|ParticleSystem|SetVectorParameter (Variables|/Script/Engine.Emitter|GetParticleSystemComponent _asemitter_standing_torch_plus) "FlameLightColor" (* (Math|Vector|SelectVector (* FlameColor 1.3) (Math|Vector|MakeVector 1.3 0.5 0.0) _busingstructurecolors) (/ (.A (Utilities|Struct|BreakLinearColor (.PrimaryColor (Utilities|Struct|BreakSPLightSettings (Variables|Default|GetTorchSettings))))) 3.0))))))

(fn CheckTime
  (bind _isdaytime (Variables|Default|GetIsDayTime))
  (bind _torchsettings (Variables|Default|GetTorchSettings))
  (bind _bcontaineractivated (Variables|Default|GetbContainerActivated))
  (bind (_postdawnoffset _preduskoffset) (Utilities|Struct|BreakSPLightSettings _torchsettings))
  (bind _isday (CallFunction|SPIsDayTime self _postdawnoffset _preduskoffset))
  (Variables|Default|SetIsDaytime _isday)
  (Utilities|FlowControl|Sequence
    (:then_0
      (if (and (or (Math|Boolean|NotEqual(Boolean) _isday (Variables|Default|GetIsDaytime)) (Math|Boolean|Equal(Boolean) _isday (Variables|Default|GetbContainerActivated))) (== (Variables|Default|GetManualActivationState) 0))
        (if (Variables|Default|GetIsDayTime)
          (if _bcontaineractivated
            (Class|PrimalStructure|SetContainerActive false))
          (elif (not _bcontaineractivated)
            (Class|PrimalStructure|SetContainerActive true)))))
    (:then_1
      (if (!= (Variables|Default|GetManualActivationState) 0)
        (if (and (not _isdaytime) (== (Variables|Default|GetManualActivationState) 1))
          (Variables|Default|SetManualActivationState 0 :!label _label)
          (elif (and _isdaytime (== (Variables|Default|GetManualActivationState) -1))
            (goto _label)))))))

(fn ReceiveBeginPlay
  (|CallParentFunction)
  (if (not (Variables|Default|GetbIsPreviewStructure))
    (Utilities|FlowControl|Sequence
      (:then_0
        (Utilities|SwitchNetAuthority
          (:PlayerServer
            (CallFunction|OnRepTorchColor))))
      (:then_1
        (Networking|SwitchHasAuthority
          (:Authority
            (CallFunction|TopUpFuel)
            (CallFunction|HandleBeginPlayEvent)))))))

(fn BPGetFuelConsumptionMultiplier
  (return 0.0))

(fn BPContainerActivated
  (Networking|SwitchHasAuthority
    (:Authority
      (CallFunction|TopUpFuel))))

(fn TopUpFuel
  (bind _myinventorycomponent (Variables|Default|GetMyInventoryComponent))
  (bind _returnvalue (Class|PrimalInventoryComponent|GetItemTemplateQuantity _myinventorycomponent "/QoLPlus/_Resources/PrimalItemResource_SPlusFuel.PrimalItemResource_SPlusFuel_C" 0 true false true false))
  (if (> (- 100 _returnvalue) 90)
    (Class|PrimalInventoryComponent|BPIncrementItemTemplateQuantity _myinventorycomponent "/QoLPlus/_Resources/PrimalItemResource_SPlusFuel.PrimalItemResource_SPlusFuel_C" (- 100 _returnvalue) true false true false false false 0 false)))

(fn BPRefreshedStructureColors
  (Class|KismetSystemLibrary|CanRunCosmeticEvents
    (:Yes
      (if (Variables|Default|GetbUsingStructureColors)
        (bind _returnvalue (Class|PrimalStructure|GetStructureColor))
        (Variables|Default|SetTorchColor (Math|Vector|MakeVector (.R (Utilities|Struct|BreakLinearColor _returnvalue)) (.G (Utilities|Struct|BreakLinearColor _returnvalue)) (.B (Utilities|Struct|BreakLinearColor _returnvalue))) true)
        (else
          (Variables|Default|SetTorchColor "2.000000,0.400000,0.080000" true))))))