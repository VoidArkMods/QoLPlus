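; S+ Industrial Grinder structure that breaks items down into a configurable share of their crafting resources and instantly bulk-crafts blueprints.
; Menu entries offer single grind, grind all and auto-grind on activation; selected-item actions reach the server by net exec command.
; Grinding applies eligibility checks, a blacklist, per-grind caps and resource substitution.
; Authority loads server config at BeginPlay; RepNotifies apply slot count, scale and muting, removing particles when rescaled.
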(event Custom|RemoveParticlesEvent
  (bind _activatedemitter (Variables|Default|GetActivatedEmitter))
  (if (not (Networking|IsDedicatedServer))
    (if (not (Math|Float|NearlyEqual(Float) (Variables|Default|GetCustomScale) 1.0 0.01))
      (Utilities|IsValid _activatedemitter
        (:Is%20Valid
          (bind _asemitter (Utilities|Casting|CastToEmitter (Variables|/Script/Engine.ChildActorComponent|GetChildActor _activatedemitter)))
          (Components|DestroyComponent (Variables|/Script/Engine.Emitter|GetParticleSystemComponent _asemitter)))))))

(fn ConstructionScript
  (bind _bispreviewstructure (Variables|Default|GetbIsPreviewStructure))
  (|CallParentFunction)
  (if _bispreviewstructure
    _
    (else
      (Networking|SwitchHasAuthority
        (:Authority
          _))))
  (bind _assplus_global_actor (Utilities|Casting|CastToSPlusGlobalActor (CallFunction|SPGetGlobalActor self)))
  (Utilities|FlowControl|Sequence
    (:then_0
      (if (Variables|/QoLPlus/SPlusGlobalActor.SPlusGlobalActor_C|GetRemoveFloorRequirement _assplus_global_actor)
        (Variables|Default|SetbRequiresPlacementOnStructureFloors false)))
    (:then_1
      (if _bispreviewstructure
        (CallFunction|QOLPlusSetStructureScale (Variables|/QoLPlus/SPlusGlobalActor.SPlusGlobalActor_C|GetGrinderScaleMultiplier _assplus_global_actor) self)))))

(fn BPGetMultiUseEntries
  (params (ForPC :type Player%20Controller%20Object%20Reference) (MultiUseEntries :type Array%20of%20Multi%20Use%20Entry%20Structures))
  (bind _self self)
  (bind _entriesout (CallFunction|SPUpdateMultiUseMenu ForPC MultiUseEntries _self false false false false))
  (Utilities|FlowControl|Sequence
    (:then_0
      (bind _accesslevel (CallFunction|SPGetAccessLevel ForPC _self))
      (if (>= _accesslevel 2)
        (CallFunction|AddGrindButtontoMenu _entriesout ForPC)
        (Utilities|Array|Add _entriesout (Utilities|Struct|MakeMultiUseEntry (Utilities|String|SelectString "Disable Grind on Activation" "Enable Grind on Activation" (Variables|Default|GetAutoGrindOnActivation)) 9100 -777))))
    (:then_1
      (return _entriesout))))

(fn BPClientDoMultiUse
  (params (ForPC :type Player%20Controller%20Object%20Reference) (ClientUseIndex :type Integer))
  (switch int ClientUseIndex
    (:8878
      (bind _asshooter_player_controller (Utilities|Casting|CastToShooterPlayerController ForPC))
      (bind _returnvalue (Class|ShooterPlayerController|GetInventoryUISelectedItemRemote _asshooter_player_controller))
      (if (Utilities|IsValid _returnvalue)
        (Class|PrimalPlayerController|ClientSendNetExecCommandtoServer (Class|PrimalAutocastFunctions|PCtoPPC ForPC) self "Grind" (Utilities|Struct|MakeBPNetExecParams (.ItemID1 (Class|PrimalItem|BPGetItemID _returnvalue)) (.ItemID2 (Class|PrimalItem|BPGetItemID _returnvalue))) true)))))

(fn BPServerHandleNetExecCommand
  (params (FromPC :type Player%20Controller%20Object%20Reference) (CommandName :type Name :default "None") (ExecParams :type BP%20Net%20Exec%20Params%20Structure%20%28by%20ref%29))
  (bind (_intparam1 _intparam2) (Utilities|Struct|BreakBPNetExecParams ExecParams))
  (Utilities|FlowControl|Sequence
    (:then_0
      (bind _asshooter_player_controller (Utilities|Casting|CastToShooterPlayerController FromPC))
      (if (Utilities|Name|Equal(Name) CommandName "Grind")
        (bind _returnvalue (Class|PrimalInventoryComponent|BPFindItemwithID (Variables|Default|GetMyInventoryComponent) _intparam1 _intparam2))
        (if (Utilities|IsValid _returnvalue)
          (bind _returnvalue_2 (Class|PrimalItem|CanFullyCraft _returnvalue true))
          (if (Math|Boolean|ANDBoolean _returnvalue_2 (Variables|/Script/ShooterGame.PrimalItem|GetbIsBlueprint _returnvalue) (not (Variables|/Script/ShooterGame.PrimalItem|GetbAllowRemovalFromInventory _returnvalue)))
            (CallFunction|CraftAllInstant _returnvalue)
            (Class|ShooterPlayerController|ClientPlayLocalSound _asshooter_player_controller "/Game/PrimalEarth/Sound/SFX/Generic/BuzzSaw.BuzzSaw" false)
            (elif (Variables|/Script/ShooterGame.PrimalItem|GetbAllowRemovalFromInventory _returnvalue)
              (bind _isvalid (CallFunction|IsValidGrindingItem _returnvalue))
              (if _isvalid
                (CallFunction|GrindItem _returnvalue _asshooter_player_controller true)))))))
    (:then_1
      (return true))))

(fn GrindItem
  (params (ItemToGrind :type Primal%20Item%20Object%20Reference) (ForPC :type Shooter%20Player%20Controller%20Object%20Reference) (PlaySound :type Boolean))
  (bind _myinventorycomponent (Variables|Default|GetMyInventoryComponent))
  (bind _isvalid (CallFunction|IsValidGrindingItem ItemToGrind))
  (if _isvalid
    (Utilities|FlowControl|Sequence
      (:then_0
        (if PlaySound
          (Utilities|IsValid ForPC
            (:Is%20Valid
              (Class|ShooterPlayerController|ClientPlayLocalSound ForPC "/Game/PrimalEarth/Sound/SFX/Generic/BuzzSaw.BuzzSaw" false)))))
      (:then_1
        (bind _asprimal_item (Utilities|Casting|CastToPrimalItemClass (Utilities|GetClass ItemToGrind)))
        (bind _returnvalue (Class|VictoryCore|GetDefaultObject ItemToGrind))
        (bind _asprimal_item_2 (Utilities|Casting|CastToPrimalItem _returnvalue))
        (LocalVariables|SetQuantityToGrind (Math|Float|Floor (/ (Math|Conversions|ToFloat(Integer) (Variables|/Script/ShooterGame.PrimalItem|GetItemQuantity ItemToGrind)) (Math|Conversions|ToFloat(Integer) (Math|Integer|SelectInt (Variables|/Script/ShooterGame.PrimalItem|GetCraftingGiveItemCount _asprimal_item_2) (Variables|/Script/ShooterGame.PrimalItem|GetItemQuantity _asprimal_item_2) (> (Variables|/Script/ShooterGame.PrimalItem|GetCraftingGiveItemCount _asprimal_item_2) (Variables|/Script/ShooterGame.PrimalItem|GetItemQuantity _asprimal_item_2)))))))
        (Class|PrimalInventoryComponent|BPIncrementItemTemplateQuantity _myinventorycomponent _asprimal_item (* (* (Math|Float|Floor (/ (Math|Conversions|ToFloat(Integer) (Variables|/Script/ShooterGame.PrimalItem|GetItemQuantity ItemToGrind)) (Math|Conversions|ToFloat(Integer) (Math|Integer|SelectInt (Variables|/Script/ShooterGame.PrimalItem|GetCraftingGiveItemCount _asprimal_item_2) (Variables|/Script/ShooterGame.PrimalItem|GetItemQuantity _asprimal_item_2) (> (Variables|/Script/ShooterGame.PrimalItem|GetCraftingGiveItemCount _asprimal_item_2) (Variables|/Script/ShooterGame.PrimalItem|GetItemQuantity _asprimal_item_2)))))) (Math|Integer|SelectInt (Variables|/Script/ShooterGame.PrimalItem|GetCraftingGiveItemCount _asprimal_item_2) (Variables|/Script/ShooterGame.PrimalItem|GetItemQuantity _asprimal_item_2) (> (Variables|/Script/ShooterGame.PrimalItem|GetCraftingGiveItemCount _asprimal_item_2) (Variables|/Script/ShooterGame.PrimalItem|GetItemQuantity _asprimal_item_2)))) -1) true false true true false false ItemToGrind false)
        (for (_array_element _array_index) (Variables|/Script/ShooterGame.PrimalItem|GetBaseCraftingResourceRequirements ItemToGrind)
          (bind _returnvalue_2 (Class|PrimalItem|GetCraftingResourceRequirement ItemToGrind _array_index))
          (if (> _returnvalue_2 0)
            (bind _returnvalue_3 (Class|VictoryCore|GetClassDefaultObject (.ResourceItemType (Utilities|Struct|BreakCraftingResourceRequirement _array_element))))
            (bind _asprimal_item_3 (Utilities|Casting|CastToPrimalItem _returnvalue_3))
            (if (not (Variables|/Script/ShooterGame.PrimalItem|GetbIsAbstractItem _asprimal_item_3))
              (if (or (not (Variables|/Script/ShooterGame.PrimalItem|GetbResourcePreventGivingFromDemolition _asprimal_item_3)) (Variables|Default|GetReturnBlockedResources))
                (bind _outitemclass (CallFunction|GetReplacementItem (.ResourceItemType (Utilities|Struct|BreakCraftingResourceRequirement _array_element))))
                (Class|PrimalInventoryComponent|BPIncrementItemTemplateQuantity _myinventorycomponent _outitemclass (* (LocalVariables|GetQuantityToGrind) (Math|Integer|Min(Integer) (Math|Float|Ceil (* _returnvalue_2 (Variables|Default|GetGrindGiveItemsPercent))) (Variables|Default|GetMaxItemsToGivePerGrind))) true false false false false false 0 false)))))))))

(fn IsValidGrindingItem
  (params (ItemToCheck :type Primal%20Item%20Object%20Reference))
  (Utilities|FlowControl|Sequence
    (:then_0
      (bind _returnvalue (Class|VictoryCore|GetDefaultObject ItemToCheck))
      (bind _asprimal_item (Utilities|Casting|CastToPrimalItem _returnvalue))
      (if (Utilities|IsValid ItemToCheck)
        (LocalVariables|SetretVal (Math|Boolean|ANDBoolean (>= (Variables|/Script/ShooterGame.PrimalItem|GetItemQuantity ItemToCheck) (Math|Integer|SelectInt (Variables|/Script/ShooterGame.PrimalItem|GetCraftingGiveItemCount _asprimal_item) (Variables|/Script/ShooterGame.PrimalItem|GetItemQuantity _asprimal_item) (> (Variables|/Script/ShooterGame.PrimalItem|GetCraftingGiveItemCount _asprimal_item) (Variables|/Script/ShooterGame.PrimalItem|GetItemQuantity _asprimal_item)))) (> (Utilities|Array|Length (Variables|/Script/ShooterGame.PrimalItem|GetBaseCraftingResourceRequirements ItemToCheck)) 0) (not (Variables|/Script/ShooterGame.PrimalItem|GetbIsBlueprint ItemToCheck)) (or (Variables|/Script/ShooterGame.PrimalItem|GetbCanBeBlueprint ItemToCheck) (Variables|/Script/ShooterGame.PrimalItem|GetbForceAllowGrinding ItemToCheck)) (or (not (Variables|/Script/ShooterGame.PrimalItem|GetbForcePreventGrinding ItemToCheck)) (and (not (Variables|/Script/ShooterGame.PrimalItem|GetbForcePreventGrinding _asprimal_item)) (Variables|Default|GetAllowGrindingMissionItems))) (not (Variables|/Script/ShooterGame.PrimalItem|GetbIsCustomRecipe ItemToCheck)) (not (CallFunction|IsItemBlacklisted ItemToCheck))))))
    (:then_1
      (return (LocalVariables|GetretVal)))))

(fn GetReplacementItem
  (params (InItemClass :type Primal%20Item%20Class%20Reference))
  (bind _grindgiveitemfrom (Variables|Default|GetGrindGiveItemFrom))
  (bind _returnvalue (Utilities|Array|FindItem _grindgiveitemfrom InItemClass))
  (LocalVariables|SetOutItem InItemClass)
  (if (>= _returnvalue 0)
    (LocalVariables|SetOutItem (Utilities|Array|Get(acopy) (Variables|Default|GetGrindGiveItemTo) _returnvalue)))
  (return (LocalVariables|GetOutItem)))

(fn AddGrindButtontoMenu
  (params (Entries :type Array%20of%20Multi%20Use%20Entry%20Structures) (PC :type Player%20Controller%20Object%20Reference))
  (if (Variables|Default|GetbContainerActivated)
    (Utilities|FlowControl|Sequence
      (:then_0
        (bind _asshooter_player_controller (Utilities|Casting|CastToShooterPlayerController PC))
        (if (Pawn|IsLocalPlayerController _asshooter_player_controller)
          (bind _returnvalue (Class|ShooterPlayerController|GetInventoryUISelectedItemRemote _asshooter_player_controller))
          (bind _isvalid (CallFunction|IsValidGrindingItem _returnvalue))
          (if _isvalid
            (LocalVariables|SetDoGrindItem true)
            (Utilities|Array|Add Entries (Utilities|Struct|MakeMultiUseEntry (Utilities|String|SelectString "Grind Item" "Craft All Instant" (LocalVariables|GetDoGrindItem)) 8878 -1000 true true) :!label _label)
            (else
              (bind _returnvalue_2 (Class|PrimalItem|CanFullyCraft _returnvalue true))
              (if (Math|Boolean|ANDBoolean _returnvalue_2 (Variables|/Script/ShooterGame.PrimalItem|GetbIsBlueprint _returnvalue) (not (Variables|/Script/ShooterGame.PrimalItem|GetbAllowRemovalFromInventory _returnvalue)))
                (goto _label))))
          (else
            (goto _label))))
      (:then_1
        (Utilities|Array|Add Entries (Utilities|Struct|MakeMultiUseEntry "Grind All" 9002 -1001 true true))))))

(fn BPTryMultiUse
  (params (ForPC :type Player%20Controller%20Object%20Reference) (UseIndex :type Integer))
  (Utilities|FlowControl|Sequence
    (:then_0
      (if (== UseIndex 601)
        (Variables|Default|SetIsUnlocked (not (Variables|Default|GetbIsLocked)))))
    (:then_1
      (if (== UseIndex 9002)
        (bind _asshooter_player_controller (Utilities|Casting|CastToShooterPlayerController ForPC))
        (CallFunction|GrindAll _asshooter_player_controller)))
    (:then_2
      (if (== UseIndex 9100)
        (Variables|Default|SetAutoGrindOnActivation (not (Variables|Default|GetAutoGrindOnActivation)) true)))
    (:then_3
      (return true))))

(fn BPIsAllowedtoBuild
  (params (OutPlacementData :type Placement%20Data%20Structure%20%28by%20ref%29) (CurrentAllowedReason :type Integer))
  (return (Math|Integer|SelectInt 1 CurrentAllowedReason (== CurrentAllowedReason -9))))

(fn OnRepInventorySlots
  (Variables|/Script/ShooterGame.PrimalInventoryComponent|SetMaxInventoryItems (Variables|Default|GetMyInventoryComponent) (Variables|Default|GetInventorySlots)))

(fn GrindAll
  (params (PC :type Shooter%20Player%20Controller%20Object%20Reference))
  (for _array_element (Variables|/Script/ShooterGame.PrimalInventoryComponent|GetInventoryItems (Variables|Default|GetMyInventoryComponent))
    (bind _isvalid (CallFunction|IsValidGrindingItem _array_element))
    (if _isvalid
      (Utilities|Array|Add (LocalVariables|GetItemsToGrind) _array_element)))
  (if (> (Utilities|Array|Length (LocalVariables|GetItemsToGrind)) 0)
    (Utilities|FlowControl|Sequence
      (:then_0
        (Utilities|IsValid PC
          (:Is%20Valid
            (Class|ShooterPlayerController|ClientPlayLocalSound PC "/Game/PrimalEarth/Sound/SFX/Generic/BuzzSaw.BuzzSaw" false))))
      (:then_1
        (for _array_element_2 (LocalVariables|GetItemsToGrind)
          (CallFunction|GrindItem _array_element_2 PC false))))))

(fn CraftAllInstant
  (params (Item :type Primal%20Item%20Object%20Reference))
  (bind _basecraftingresourcerequirements (Variables|/Script/ShooterGame.PrimalItem|GetBaseCraftingResourceRequirements Item))
  (bind _myinventorycomponent (Variables|Default|GetMyInventoryComponent))
  (bind _craftinggivesitemquantityoverride (Variables|/Script/ShooterGame.PrimalItem|GetCraftingGivesItemQuantityOverride Item))
  (bind _asprimal_inventory_grinder_plus (Utilities|Casting|CastToPrimalInventory_GrinderPlus _myinventorycomponent))
  (bind _asprimal_item (Utilities|Casting|CastToPrimalItemClass (Utilities|GetClass Item)))
  (if (>= (Utilities|Array|FindItem (Variables|/QoLPlus/Misc/IndustrialGrinder/PrimalInventory_GrinderPlus.PrimalInventory_GrinderPlus_C|GetChildItems _asprimal_inventory_grinder_plus) _asprimal_item) 0)
    (LocalVariables|SetCraftQty 99999999)
    (for _array_element _basecraftingresourcerequirements
      (bind _returnvalue (Class|PrimalInventoryComponent|GetItemTemplateQuantity (Variables|Default|GetMyInventoryComponent) (.ResourceItemType (Utilities|Struct|BreakCraftingResourceRequirement _array_element)) 0 true false false false))
      (if (< (Math|Float|Floor (/ (Math|Conversions|ToFloat(Integer) _returnvalue) (.BaseResourceRequirement (Utilities|Struct|BreakCraftingResourceRequirement _array_element)))) (LocalVariables|GetCraftQty))
        (LocalVariables|SetCraftQty (Math|Float|Floor (/ (Math|Conversions|ToFloat(Integer) _returnvalue) (.BaseResourceRequirement (Utilities|Struct|BreakCraftingResourceRequirement _array_element)))))))
    (for _array_element_2 _basecraftingresourcerequirements
      (Class|PrimalInventoryComponent|BPIncrementItemTemplateQuantity (Variables|Default|GetMyInventoryComponent) (.ResourceItemType (Utilities|Struct|BreakCraftingResourceRequirement _array_element_2)) (Math|Float|Floor (* (* (LocalVariables|GetCraftQty) (.BaseResourceRequirement (Utilities|Struct|BreakCraftingResourceRequirement _array_element_2))) -1.0)) true false false true false false 0 false))
    (Class|PrimalInventoryComponent|BPIncrementItemTemplateQuantity _myinventorycomponent (Utilities|Array|Get(acopy) (Variables|/QoLPlus/Misc/IndustrialGrinder/PrimalInventory_GrinderPlus.PrimalInventory_GrinderPlus_C|GetParentItems _asprimal_inventory_grinder_plus) (Utilities|Array|FindItem (Variables|/QoLPlus/Misc/IndustrialGrinder/PrimalInventory_GrinderPlus.PrimalInventory_GrinderPlus_C|GetChildItems _asprimal_inventory_grinder_plus) _asprimal_item)) (* (LocalVariables|GetCraftQty) (Math|Integer|SelectInt (Variables|/Script/ShooterGame.PrimalItem|GetItemQuantity Item) _craftinggivesitemquantityoverride (<= _craftinggivesitemquantityoverride 0))) true false true false false false 0 false)))

(fn BPCanbeActivatedbyPlayer
  (params (PC :type Shooter%20Player%20Controller%20Object%20Reference))
  (return (or (== (Variables|/Script/Engine.Actor|GetTargetingTeam PC) (Variables|Default|GetTargetingTeam)) (not (Variables|Default|GetbIsLocked)))))

(fn ReceiveBeginPlay
  (bind _returnvalue (Game|GetGameMode))
  (|CallParentFunction)
  (if (not (Variables|Default|GetbIsPreviewStructure))
    (Networking|SwitchHasAuthority
      (:Authority
        (Utilities|FlowControl|Sequence
          (:then_0
            (bind _value (CallFunction|SPGetConfigSetting-InventorySize _returnvalue "GrinderSlotCount" 200))
            (Variables|Default|SetInventorySlots _value true))
          (:then_1
            (bind _value_2 (CallFunction|SPGetConfigSetting-CraftingSpeed _returnvalue "GrinderCraftingSpeed"))
            (Variables|/Script/ShooterGame.PrimalInventoryComponent|SetCraftingItemSpeed (Variables|Default|GetMyInventoryComponent) _value_2))
          (:then_2
            (bind _value_3 (CallFunction|SPGetConfig-Int _returnvalue "GrinderResourceReturnPercent" 30 1 100))
            (Variables|Default|SetGrindGiveItemsPercent (/ (Math|Conversions|ToFloat(Integer) _value_3) 1e+02)))
          (:then_3
            (bind _value_4 (CallFunction|SPGetConfig-Int _returnvalue "GrinderResourceReturnMax" 10000 1 999999))
            (Variables|Default|SetMaxItemsToGivePerGrind _value_4))
          (:then_4
            (bind _value_5 (CallFunction|SPGetConfig-Bool _returnvalue "GrinderReturnBlockedResources"))
            (Variables|Default|SetReturnBlockedResources _value_5))
          (:then_5
            (bind _asstring (CallFunction|SPGetConfig-Array _returnvalue "GrinderBlacklist"))
            (Variables|Default|SetGrinderBlacklist _asstring true))
          (:then_6
            (bind _value_6 (CallFunction|SPGetConfig-Float _returnvalue "GrinderScaleMultiplier" 1.0 0.1 2.0))
            (Variables|Default|SetCustomScale _value_6 true))
          (:then_7
            (bind _disablesound (CallFunction|SPGetConfigSetting-Noise _returnvalue))
            (Variables|Default|SetDisableSound _disablesound true))
          (:then_8
            (bind _value_7 (CallFunction|SPGetConfig-Bool _returnvalue "AllowGrindingMissionRewards"))
            (Variables|Default|SetAllowGrindingMissionItems _value_7 true))
          (:then_9
            (Variables|Default|SetbIsLocked (not (Variables|Default|GetIsUnlocked)) true)))))))

(fn IsItemBlacklisted
  (params (Item :type Primal%20Item%20Object%20Reference))
  (return (Utilities|Array|ContainsItem (Variables|Default|GetGrinderBlacklist) (Utilities|GetClassDisplayName (Utilities|GetClass Item)))))

(fn OnRepCustomScale
  (CallFunction|QOLPlusSetStructureScale (Variables|Default|GetCustomScale) self)
  (CallFunction|RemoveParticlesEvent))

(fn OnRepDisableSound
  (if (not (Networking|IsDedicatedServer))
    (if (Variables|Default|GetDisableSound)
      (bind _asprimal_emitter_spawnable (Utilities|Casting|CastToPrimalEmitterSpawnable (Variables|/Script/Engine.ChildActorComponent|GetChildActor (Variables|Default|GetActivatedEmitter))))
      (Audio|Components|Audio|SetVolumeMultiplier (Variables|/Script/ShooterGame.PrimalEmitterSpawnable|GetSoundToPlay _asprimal_emitter_spawnable) 0.0 :!class /Script/Engine.AudioComponent))))

(fn BPContainerActivated
  (Class|KismetSystemLibrary|IsRunningonServer
    (:Yes
      (if (Variables|Default|GetAutoGrindOnActivation)
        (CallFunction|GrindAll)))))