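; BP_VesselPlus is a placeable Vessel storage structure using Structures Plus (SP) helpers for its multi-use menu and configuration.
; On the authority, BeginPlay reads the configured slot count into InventorySlots, whose OnRep updates the inventory component's capacity.
; IsUnlocked mirrors the lock state after a menu action and restores IsLocked on BeginPlay.
; The build check overrides one specific placement failure code to allow placement.
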(fn ConstructionScript
  (|CallParentFunction))

(fn BPIsAllowedtoBuild
  (params (OutPlacementData :type Placement%20Data%20Structure%20%28by%20ref%29) (CurrentAllowedReason :type Integer))
  (return (Math|Integer|SelectInt 1 CurrentAllowedReason (== CurrentAllowedReason -9))))

(fn BPGetMultiUseEntries
  (params (ForPC :type Player%20Controller%20Object%20Reference) (MultiUseEntries :type Array%20of%20Multi%20Use%20Entry%20Structures))
  (bind _entriesout (CallFunction|SPUpdateMultiUseMenu ForPC MultiUseEntries self false false false false))
  (return _entriesout))

(fn BPTryMultiUse
  (params (ForPC :type Player%20Controller%20Object%20Reference) (UseIndex :type Integer))
  (if (== UseIndex 601)
    (Variables|Default|SetIsUnlocked (not (Variables|Default|GetbIsLocked))))
  (return true))

(fn OnRepInventorySlots
  (Variables|/Script/ShooterGame.PrimalInventoryComponent|SetMaxInventoryItems (Variables|Default|GetMyInventoryComponent) (Variables|Default|GetInventorySlots)))

(fn ReceiveBeginPlay
  (|CallParentFunction)
  (if (not (Variables|Default|GetbIsPreviewStructure))
    (Networking|SwitchHasAuthority
      (:Authority
        (Utilities|FlowControl|Sequence
          (:then_0
            (bind _value (CallFunction|SPGetConfigSetting-InventorySize (Game|GetGameMode) "VesselSlotCount" 20))
            (Variables|Default|SetInventorySlots _value true))
          (:then_1
            (Variables|Default|SetbIsLocked (not (Variables|Default|GetIsUnlocked)) true)))))))