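; Industrial cooker structure (Structures Plus style) that autocrafts from its inventory, with a team-restricted activation lock and a build-check override.
; On authority, BeginPlay reads game-mode config for slot count, crafting speed, electric-storm shutdown and sound muting.
; A multi-use entry cycles autocrafting between everything, all except dyes, and disabled.
; OnRep handlers apply slot count, emitter muting and autocraft mode, toggling dye blueprints individually.
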(fn ConstructionScript
  (|CallParentFunction))

(fn BPIsAllowedtoBuild
  (params (OutPlacementData :type Placement%20Data%20Structure%20%28by%20ref%29) (CurrentAllowedReason :type Integer))
  (return (Math|Integer|SelectInt 1 CurrentAllowedReason (== CurrentAllowedReason -9))))

(fn BPGetMultiUseEntries
  (params (ForPC :type Player%20Controller%20Object%20Reference) (MultiUseEntries :type Array%20of%20Multi%20Use%20Entry%20Structures))
  (bind _entriesout (CallFunction|SPUpdateMultiUseMenu ForPC MultiUseEntries self false false false false))
  (Utilities|FlowControl|Sequence
    (:then_0
      (bind _returnvalue (Class|PrimalStructure|AllowStructureAccess ForPC))
      (if _returnvalue
        (Utilities|Array|Add _entriesout (Utilities|Struct|MakeMultiUseEntry (Utilities|Select :Index (Variables|Default|GetAutoCraftMode) :Option%200 "Autocrafting Everything" :Option%201 "Autocrafting All Except Dyes" :Option%202 "Autocrafting Disabled") 9002 -1020 true true))))
    (:then_1
      (return _entriesout))))

(fn BPTryMultiUse
  (params (ForPC :type Player%20Controller%20Object%20Reference) (UseIndex :type Integer))
  (Utilities|FlowControl|Sequence
    (:then_0
      (if (== UseIndex 601)
        (Variables|Default|SetIsUnlocked (not (Variables|Default|GetbIsLocked)))
        (elif (== UseIndex 9002)
          (Variables|Default|SetAutoCraftMode (Math|Integer|SelectInt 0 (+ (Variables|Default|GetAutoCraftMode) 1) (> (+ (Variables|Default|GetAutoCraftMode) 1) 2)) true))))
    (:then_1
      (return true))))

(fn OnRepInventorySlots
  (Variables|/Script/ShooterGame.PrimalInventoryComponent|SetMaxInventoryItems (Variables|Default|GetMyInventoryComponent) (Variables|Default|GetInventorySlots)))

(fn BPCanbeActivatedbyPlayer
  (params (PC :type Shooter%20Player%20Controller%20Object%20Reference))
  (return (or (== (Variables|/Script/Engine.Actor|GetTargetingTeam PC) (Variables|Default|GetTargetingTeam)) (not (Variables|Default|GetbIsLocked)))))

(fn ReceiveBeginPlay
  (bind _returnvalue (Game|GetGameMode))
  (|CallParentFunction)
  (if (not (Variables|Default|GetbIsPreviewStructure))
    (Networking|SwitchHasAuthority
      (:Authority
        (Utilities|FlowControl|Sequence
          (:then_0
            (bind _value (CallFunction|SPGetConfigSetting-InventorySize _returnvalue "IndustrialCookerSlotCount" 100))
            (Variables|Default|SetInventorySlots _value true))
          (:then_1
            (bind _value_2 (CallFunction|SPGetConfigSetting-StormDisableElectronics _returnvalue))
            (Variables|Default|SetbDisableStructureOnElectricStorm _value_2))
          (:then_2
            (bind _value_3 (CallFunction|SPGetConfig-Float _returnvalue "IndustrialCookingPotCraftingSpeed" 12.0 1.0 1e+02))
            (Variables|/Script/ShooterGame.PrimalInventoryComponent|SetCraftingItemSpeed (Variables|Default|GetMyInventoryComponent) _value_3))
          (:then_3
            (bind _disablesound (CallFunction|SPGetConfigSetting-Noise _returnvalue))
            (Variables|Default|SetDisableSound _disablesound true))
          (:then_4
            (Variables|Default|SetbIsLocked (not (Variables|Default|GetIsUnlocked)) true))
          (:then_5
            (Utilities|SwitchNetAuthority
              (:PlayerServer
                (CallFunction|OnRepAutoCraftMode)))))))))

(fn OnRepDisableSound
  (if (not (Networking|IsDedicatedServer))
    (if (Variables|Default|GetDisableSound)
      (bind _asprimal_emitter_spawnable (Utilities|Casting|CastToPrimalEmitterSpawnable (Variables|/Script/Engine.ChildActorComponent|GetChildActor (Variables|Default|GetActivatedEmitter))))
      (Audio|Components|Audio|SetVolumeMultiplier (Variables|/Script/ShooterGame.PrimalEmitterSpawnable|GetSoundToPlay _asprimal_emitter_spawnable) 0.0 :!class /Script/Engine.AudioComponent))))

(fn OnRepAutoCraftMode
  (bind _myinventorycomponent (Variables|Default|GetMyInventoryComponent))
  (switch int (Variables|Default|GetAutoCraftMode)
    (:0
      (Variables|/Script/ShooterGame.PrimalInventoryComponent|SetbCheckForAutoCraftBlueprints _myinventorycomponent true)
      (CallFunction|ToggleDyeAutoCrafting true))
    (:1
      (CallFunction|ToggleDyeAutoCrafting false))
    (:2
      (Variables|/Script/ShooterGame.PrimalInventoryComponent|SetbCheckForAutoCraftBlueprints _myinventorycomponent false))))

(fn ToggleDyeAutoCrafting
  (params (Enable :type Boolean))
  (for _array_element (Variables|/Script/ShooterGame.PrimalInventoryComponent|GetInventoryItems (Variables|Default|GetMyInventoryComponent))
    (bind _asprimal_item_dye_generic (Utilities|Casting|CastToPrimalItemDyeGeneric _array_element))
    (if (and (Variables|/Script/ShooterGame.PrimalItem|GetbIsBlueprint _array_element) (not (Variables|/Script/ShooterGame.PrimalItem|GetbAllowRemovalFromInventory _array_element)))
      (Variables|/Script/ShooterGame.PrimalItem|SetbAutoCraftBlueprint _asprimal_item_dye_generic Enable))))