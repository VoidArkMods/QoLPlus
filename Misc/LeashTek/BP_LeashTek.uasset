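; Tek dino leash structure that movement-tethers same-team and baby dinos within a selectable radius.
; Multi-use wheel toggles activation, range, field visibility and manual leashing; nearby active leashes cap the range or block activation.
; An octree scan tethers dinos, while sphere overlap catches players' ridden or mounted dinos.
; A looping server timer sends wandering tethered dinos near the edge to uniformly random points in the inner half-radius.
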(event OnComponentBeginOverlap(PlayerDetectSphere)
  (params (OverlappedComponent :type Primitive%20Component%20Object%20Reference) (OtherActor :type Actor%20Object%20Reference) (OtherComp :type Primitive%20Component%20Object%20Reference) (OtherBodyIndex :type Integer) (bFromSweep :type Boolean) (SweepResult :type Hit%20Result%20Structure%20%28by%20ref%29))
  (if (CallFunction|GetIsActive)
    (bind _asshooter_character (Utilities|Casting|CastToShooterCharacter OtherActor))
    (if (== (Variables|/Script/Engine.Actor|GetTargetingTeam _asshooter_character) (Variables|Default|GetTargetingTeam))
      (Utilities|FlowControl|Sequence
        (:then_0
          (Utilities|IsValid (Variables|/Script/ShooterGame.ShooterCharacter|GetRidingDino _asshooter_character)
            (:Is%20Valid
              (Class|PrimalCharacter|SetMovementTether (Variables|/Script/ShooterGame.ShooterCharacter|GetRidingDino _asshooter_character) self (Variables|Default|GetEffectRadius) 0.0))))
        (:then_1
          (Utilities|IsValid (Variables|/Script/ShooterGame.PrimalCharacter|GetMountedDino _asshooter_character)
            (:Is%20Valid
              (Class|PrimalCharacter|SetMovementTether (Variables|/Script/ShooterGame.PrimalCharacter|GetMountedDino _asshooter_character) self (Variables|Default|GetEffectRadius) 0.0))))))))

(event Custom|HandleBeginPlayEvent
  (if (Variables|Default|GetActivated)
    (Utilities|FlowControl|Delay 0 1.0)
    (CallFunction|SetEffectRadius (Variables|Default|GetEffectRadius) true)))

(event Custom|MonitorDinoPositionsEvent
  (for _array_element (Variables|Default|GetTetheredDinos)
    (if (Variables|/Script/ShooterGame.PrimalDinoCharacter|GetbEnableTamedWandering _array_element)
      (if (>= (Transformation|GetDistanceTo _array_element) (* (Variables|Default|GetEffectRadius) 0.75))
        (bind _asaicontroller (Utilities|Casting|CastToAIController (Pawn|GetController _array_element)))
        (bind _destination (CallFunction|GetRandomDestination))
        (AI|Navigation|MovetoLocation _asaicontroller _destination -1.0 true true false true 0 true false)
        (if (not (Class|VictoryCore|IsShipping))
          (CallFunction|DrawDebugDestination _destination))))))

(event Custom|DrawDebugDestination
  (params (Location :type Vector))
  (if (not (Networking|IsDedicatedServer))
    (Rendering|Debug|DrawDebugBox 0 Location "50.000000,50.000000,5000.000000" "(R=0.042944,G=0.000000,B=1.000000,A=1.000000)" "0, 0, 0" 0.0 0.0 true)
    (Development|PrintString 0 (Utilities|String|ToString(Vector) Location))))

(event Custom|AddTetherToDino
  (params (Dino :type Primal%20Dino%20Character%20Object%20Reference))
  (EventDispatchers|BindEventtoOnMovementTetherSet Dino (delegate Custom|MovementTetherEvent__DelegateSignature_Event))
  (Class|PrimalDinoCharacter|SetMovementTether Dino self (Variables|Default|GetEffectRadius) 0.0))

(event Custom|MovementTetherEvent__DelegateSignature_Event
  (params (Pawn :type Pawn%20Object%20Reference) (TetherObject :type Actor%20Object%20Reference))
  (bind _asprimal_dino_character (Utilities|Casting|CastToPrimalDinoCharacter Pawn))
  (if (!= TetherObject self)
    (CallFunction|RemoveTetherfromDino _asprimal_dino_character)))

(event Custom|RemoveTetherFromDino
  (params (Dino :type Primal%20Dino%20Character%20Object%20Reference))
  (EventDispatchers|UnbindEventfromOnMovementTetherSet Dino (delegate Custom|MovementTetherEvent__DelegateSignature_Event))
  (Utilities|Array|RemoveItem (Variables|Default|GetTetheredDinos) Dino))

(fn ConstructionScript
  (|CallParentFunction)
  (if (not (Variables|Default|GetbIsPreviewStructure))
    (Collision|SetCollisionEnabled (Variables|Default|GetPlayerDetectSphere) "NoCollision")
    (if (not (Networking|IsDedicatedServer))
      (bind _returnvalue (Rendering|Material|CreateDynamicMaterialInstance 0 "/Game/Extinction/Effects/Gameplay/DinoLeash/MIC_DinoLeash_Area.MIC_DinoLeash_Area" "None" :!class /Script/Engine.KismetMaterialLibrary))
      (Variables|Default|SetRadialMaterialInstance _returnvalue)
      (Rendering|Material|SetMaterial (Variables|Default|GetEffectField) 0 _returnvalue))))

(fn BPGetMultiUseEntries
  (params (ForPC :type Player%20Controller%20Object%20Reference) (MultiUseEntries :type Array%20of%20Multi%20Use%20Entry%20Structures))
  (bind _returnvalue (Class|KismetSystemLibrary|MakeLiteralInteger 67101))
  (bind _activated (Variables|Default|GetActivated))
  (bind _returnvalue_2 (not _activated))
  (bind _entriesout (CallFunction|SPUpdateMultiUseMenu ForPC MultiUseEntries self false false false false))
  (Utilities|FlowControl|Sequence
    (:then_0
      (if (== (Variables|/Script/Engine.Actor|GetTargetingTeam ForPC) (Variables|Default|GetTargetingTeam))
        (bind _maxsetting (CallFunction|GetMaximumAllowedRadius))
        (LocalVariables|SetMaxSetting _maxsetting)
        (Utilities|Array|Add _entriesout (Utilities|Struct|MakeMultiUseEntry (Utilities|String|SelectString "Deactivate" (Utilities|String|SelectString "Can't Activate (Interference)" "Activate" (< (LocalVariables|GetMaxSetting) 0)) _activated) 67100 (Math|Integer|SelectInt 1000 -1 _returnvalue_2) (and _returnvalue_2 (< (LocalVariables|GetMaxSetting) 0)) false 0 false (Math|Conversions|ToColor(LinearColor) (Variables|Default|GetDisabledWheelColor)) 1.0 1.0))
        (bind _returnvalue_3 (Class|PrimalGameData|BPGetGameData))
        (Utilities|Array|Add _entriesout (Utilities|Struct|MakeMultiUseEntry "[Change Range]" _returnvalue -2 true true true false 0 false (Variables|/Script/ShooterGame.PrimalGameData|GetWheelFolderColor _returnvalue_3)))
        (for (_array_element _array_index) (Variables|Default|GetSettingNames)
          (Utilities|Array|Add _entriesout (Utilities|Struct|MakeMultiUseEntry _array_element (+ _array_index 67110) (+ _array_index 1) (and (< (LocalVariables|GetMaxSetting) _array_index) (Variables|Default|GetActivated)) (== _array_index (Variables|Default|GetRadiusSetting)) false 0 false _returnvalue (Math|Conversions|ToColor(LinearColor) (Variables|Default|GetDisabledWheelColor)) (Variables|/Script/ShooterGame.PrimalGameData|GetWheelFolderColor _returnvalue_3))))
        (Utilities|Array|Add _entriesout (Utilities|Struct|MakeMultiUseEntry "[Back]" 88810 999 true true true false 0 false _returnvalue (Variables|/Script/ShooterGame.PrimalGameData|GetWheelBackColor _returnvalue_3)))
        (if (Variables|Default|GetActivated)
          (Utilities|Array|Add _entriesout (Utilities|Struct|MakeMultiUseEntry (Utilities|String|SelectString "Show Radius" "Hide Radius" (Variables|Default|GetHideRadiusEffect)) 67099 5000))
          (Utilities|Array|Add _entriesout (Utilities|Struct|MakeMultiUseEntry "Leash Dinos" 67101 150)))))
    (:then_1
      (return _entriesout))))

(fn BPTryMultiUse
  (params (ForPC :type Player%20Controller%20Object%20Reference) (UseIndex :type Integer))
  (Utilities|FlowControl|Sequence
    (:then_0
      (if (== (Variables|/Script/Engine.Actor|GetTargetingTeam ForPC) (Variables|Default|GetTargetingTeam))
        (switch int UseIndex
          (:Default
            (switch int UseIndex
              (:67110
                (Variables|Default|SetRadiusSetting 0 true))
              (:67111
                (Variables|Default|SetRadiusSetting 1 true))
              (:67112
                (Variables|Default|SetRadiusSetting 2 true))
              (:67113
                (Variables|Default|SetRadiusSetting 3 true)))
            (CallFunction|SetEffectRadius (Utilities|Array|Get(acopy) (Variables|Default|GetRadiusOptions) (Variables|Default|GetRadiusSetting)) false))
          (:67099
            (Variables|Default|SetHideRadiusEffect (not (Variables|Default|GetHideRadiusEffect)) true))
          (:67100
            (CallFunction|Activate (not (Variables|Default|GetActivated))))
          (:67101
            (CallFunction|TetherDinosinRadius)))))
    (:then_1
      (return false))))

(fn OnRepActivated
  (Utilities|FlowControl|Sequence
    (:then_0
      (Networking|SwitchHasAuthority
        (:Authority
          (if (Variables|Default|GetActivated)
            (Utilities|Time|SetTimerbyFunctionName 0 "MonitorDinoPositionsEvent" 5.0 true)
            (else
              (Utilities|Time|ClearTimerbyFunctionName 0 "MonitorDinoPositionsEvent"))))))
    (:then_1
      (if (not (Networking|IsDedicatedServer))
        (Class|KismetSystemLibrary|CanRunCosmeticEvents
          (:Yes
            (CallFunction|UpdateVisibility)))))))

(fn Activate
  (params (Activated :type Boolean))
  (bind _tethereddinos (Variables|Default|GetTetheredDinos))
  (bind _playerdetectsphere (Variables|Default|GetPlayerDetectSphere))
  (bind _output (Utilities|Array|Get(acopy) _tethereddinos))
  (Class|KismetSystemLibrary|IsRunningonServer
    (:Yes
      (Variables|Default|SetActivated Activated true)
      (if (CallFunction|GetIsActive)
        (Collision|SetCollisionEnabled (Variables|Default|GetPlayerDetectSphere) "QueryAndPhysics")
        (bind _maxsetting (CallFunction|GetMaximumAllowedRadius))
        (Variables|Default|SetRadiusSetting (Math|Integer|Min(Integer) _maxsetting (Variables|Default|GetRadiusSetting)) true)
        (CallFunction|SetEffectRadius (Utilities|Array|Get(acopy) (Variables|Default|GetRadiusOptions) (Variables|Default|GetRadiusSetting)) true)
        (else
          (while (> (Utilities|Array|Length (Variables|Default|GetTetheredDinos)) 0)
            (if (and (Utilities|IsValid (Variables|/Script/ShooterGame.PrimalCharacter|GetTetherActor _output)) (Utilities|IsValid _output))
              (Class|PrimalDinoCharacter|ClearMovementTether _output)
              (else
                (Utilities|Array|RemoveIndex _tethereddinos))))
          (Collision|SetCollisionEnabled _playerdetectsphere "NoCollision")
          (Components|Sphere|SetSphereRadius _playerdetectsphere 1.0 false)))
      (return))))

(fn BPPlacedStructure
  (params (ForPC :type Player%20Controller%20Object%20Reference))
  (bind _maxsetting (CallFunction|GetMaximumAllowedRadius))
  (CallFunction|Activate (>= _maxsetting 0)))

(fn BPIsAllowedtoBuild
  (params (OutPlacementData :type Placement%20Data%20Structure%20%28by%20ref%29) (CurrentAllowedReason :type Integer))
  (return (Math|Integer|SelectInt 1 CurrentAllowedReason (== CurrentAllowedReason -9))))

(fn BPClientDoMultiUse
  (params (ForPC :type Player%20Controller%20Object%20Reference) (ClientUseIndex :type Integer))
  (bind _returnvalue (Class|KismetSystemLibrary|MakeLiteralInteger 67101))
  (Utilities|FlowControl|Sequence
    (:then_0
      (bind _asshooter_player_controller (Utilities|Casting|CastToShooterPlayerController ForPC))
      (if (== ClientUseIndex _returnvalue)
        (Class|ShooterPlayerController|SetMultiUseWheelCategory _asshooter_player_controller _returnvalue 0 0)))
    (:then_1
      (|CallParentFunction ForPC ClientUseIndex))))

(fn OnRepEffectRadius
  (if (Variables|Default|GetActivated)
    (Transformation|SetWorldScale3D (Variables|Default|GetEffectField) (Math|Conversions|ToVector(Float) (/ (Variables|Default|GetEffectRadius) (Variables|Default|GetEffectScalar))))
    (if (not (Networking|IsDedicatedServer))
      (Rendering|Material|SetScalarParameterValue (Variables|Default|GetRadialMaterialInstance) "NearDistanceFade" (+ (Variables|Default|GetEffectRadius) 3e+03) :!class /Script/Engine.MaterialInstanceDynamic))))

(fn SetEffectRadius
  (params (EffectRadius :type Float%20%28double-precision%29) (ForceSet :type Boolean))
  (Class|KismetSystemLibrary|IsRunningonServer
    (:Yes
      (if (or ForceSet (!= (Variables|Default|GetEffectRadius) EffectRadius))
        (Variables|Default|SetEffectRadius EffectRadius true)
        (if (CallFunction|GetIsActive)
          (for _array_element (Variables|Default|GetTetheredDinos)
            (Class|PrimalCharacter|SetMovementTether _array_element self (Variables|Default|GetEffectRadius) 0.0))
          (CallFunction|TetherDinosinRadius)
          (Components|Sphere|SetSphereRadius (Variables|Default|GetPlayerDetectSphere) (/ (Variables|Default|GetEffectRadius) (Variables|Default|GetScaleFactor)) true)
          (Transformation|SetWorldScale3D (Variables|Default|GetEffectField) (Math|Conversions|ToVector(Float) (/ (Variables|Default|GetEffectRadius) (Variables|Default|GetEffectScalar))))
          (return))))))

(fn TetherDinosinRadius
  (bind _returnvalue (Class|VictoryCore|ServerOctreeOverlapActorsClass (Class|PrimalActor|GetWorld) (Transformation|GetActorLocation) (Variables|Default|GetEffectRadius) "SPATIALNETWORKEDACTORS" "/Script/ShooterGame.PrimalDinoCharacter" false))
  (for _array_element _returnvalue
    (bind _asprimal_dino_character (Utilities|Casting|CastToPrimalDinoCharacter _array_element))
    (if (and (or (== (Variables|/Script/Engine.Actor|GetTargetingTeam _asprimal_dino_character) (Variables|Default|GetTargetingTeam)) (< (Variables|/Script/ShooterGame.PrimalDinoCharacter|GetBabyAge _asprimal_dino_character) 1.0)) (< (Utilities|Array|FindItem (Variables|Default|GetTetheredDinos) _asprimal_dino_character) 0))
      (CallFunction|AddTethertoDino _asprimal_dino_character)
      (Utilities|Array|Insert (Variables|Default|GetTetheredDinos) _asprimal_dino_character)))
  (return))

(fn GetMaximumAllowedRadius
  (bind _returnvalue (Transformation|GetActorLocation))
  (LocalVariables|SetIndex (- (Utilities|Array|Length (Variables|Default|GetRadiusOptions)) 1))
  (LocalVariables|SetMax (Utilities|Array|Get(acopy) (Variables|Default|GetRadiusOptions) (LocalVariables|GetIndex)))
  (Utilities|FlowControl|Sequence
    (:then_0
      (Class|KismetSystemLibrary|IsRunningonServer
        (:Yes
          ;[1 1 1] Check Server
          (bind _returnvalue_2 (Class|VictoryCore|ServerOctreeOverlapActorsClass (Class|PrimalActor|GetWorld) _returnvalue (+ (LocalVariables|GetMax) (Utilities|Array|Get(acopy) (Variables|Default|GetRadiusOptions))) "STRUCTURES" "/Game/Extinction/Structures/DinoLeash/Structure_DinoLeash.Structure_DinoLeash_C" true))
          (for _array_element _returnvalue_2
            (if (!= _array_element self)
              (bind (_isactive _effectradius) (CallFunction|GetNearbyLeashDetails _array_element))
              (if _isactive
                (LocalVariables|SetMax (Math|Float|Min(Float) (- (Utilities|Distance2D (Transformation|GetActorLocation) (Transformation|GetActorLocation _array_element)) _effectradius) (LocalVariables|GetMax)))))))
        (:No
          ;[1 1 1] Check Client
          (Utilities|Array|Add (LocalVariables|GetIgnore) self)
          (bind _outactors (Class|KismetSystemLibrary|SphereOverlapActorsSimple 0 _returnvalue (+ (LocalVariables|GetMax) (Utilities|Array|Get(acopy) (Variables|Default|GetRadiusOptions))) "ObjectTypeQuery9" (Utilities|GetClass self) (LocalVariables|GetIgnore)))
          (for _array_element_2 _outactors
            (if (!= _array_element_2 self)
              (bind (_isactive_2 _effectradius_2) (CallFunction|GetNearbyLeashDetails _array_element_2))
              (if _isactive_2
                (LocalVariables|SetMax (Math|Float|Min(Float) (- (Utilities|Distance2D (Transformation|GetActorLocation) (Transformation|GetActorLocation _array_element_2)) _effectradius_2) (LocalVariables|GetMax)))))))))
    (:then_1
      (while (and (>= (LocalVariables|GetIndex) 0) (> (Utilities|Array|Get(acopy) (Variables|Default|GetRadiusOptions) (LocalVariables|GetIndex)) (LocalVariables|GetMax)))
        (LocalVariables|SetIndex (- (LocalVariables|GetIndex) 1)))
      (return (LocalVariables|GetMax) (LocalVariables|GetIndex)))))

(fn BlueprintDrawPreviewHUD
  (params (HUD :type Shooter%20HUD%20Object%20Reference) (CenterX :type Float%20%28single-precision%29) (CenterY :type Float%20%28single-precision%29))
  (bind _canvas (Variables|/Script/Engine.HUD|GetCanvas HUD))
  (bind _maxsetting (CallFunction|GetMaximumAllowedRadius))
  (Class|Canvas|SetDrawColor _canvas (Math|Conversions|ToColor(LinearColor) (Math|Color|SelectColor "(R=0.000000,G=1.000000,B=0.000000,A=0.750000)" "(R=1.000000,G=0.000000,B=0.000000,A=0.750000)" (>= _maxsetting 0))))
  (Class|Canvas|BPDrawTextCentered _canvas (Variables|/Script/ShooterGame.ShooterHUD|GetNormalFont HUD) (Utilities|String|SelectString (Utilities|String|ToString(Text) (Utilities|Text|FormatText "Max Range: {0}" (Utilities|Text|ToText(String) (Utilities|Array|Get(acopy) (Variables|Default|GetSettingNames) _maxsetting)))) "Interference" (>= _maxsetting 0)) CenterX (+ CenterY 25.0) 1.0 1.0 true true))

(fn BPContainerActivated
  (bind _maxsetting (CallFunction|GetMaximumAllowedRadius))
  (CallFunction|Activate (and (Variables|Default|GetActivated) (>= _maxsetting 0))))

(fn BPContainerDeactivated
  (CallFunction|Activate (Variables|Default|GetActivated)))

(fn GetIsActive
  (return (Variables|Default|GetActivated)))

(fn ReceiveBeginPlay
  (|CallParentFunction)
  (if (not (Variables|Default|GetbIsPreviewStructure))
    (Networking|SwitchHasAuthority
      (:Authority
        (Utilities|FlowControl|Sequence
          (:then_0
            (Utilities|SwitchNetAuthority
              (:PlayerServer
                (CallFunction|OnRepActivated)
                (CallFunction|OnRepEffectRadius)
                (CallFunction|OnRepHideRadiusEffect))))
          (:then_1
            (CallFunction|HandleBeginPlayEvent)))))))

(fn UpdateVisibility
  (bind _effectfield (Variables|Default|GetEffectField))
  (Utilities|FlowControl|Sequence
    (:then_0
      (Transformation|SetWorldScale3D _effectfield (Math|Conversions|ToVector(Float) (/ (Variables|Default|GetEffectRadius) (Variables|Default|GetEffectScalar))))
      (if (Variables|Default|GetHideRadiusEffect)
        (Rendering|SetVisibility _effectfield false true)
        (else
          (Rendering|SetVisibility _effectfield (CallFunction|GetIsActive) true))))
    (:then_1
      (return))))

(fn BPAdjustDamage
  (params (IncomingDamage :type Float%20%28single-precision%29) (TheDamageEvent :type Damage%20Event%20Structure) (EventInstigator :type Controller%20Object%20Reference) (DamageCauser :type Actor%20Object%20Reference) (bIsPointDamage :type Boolean) (PointHitInfo :type Hit%20Result%20Structure))
  (LocalVariables|SetDamage IncomingDamage)
  (Utilities|FlowControl|Sequence
    (:then_0
      (bind _asprimal_dino_character (Utilities|Casting|CastToPrimalDinoCharacter DamageCauser))
      (if (== (Variables|/Script/Engine.Actor|GetTargetingTeam _asprimal_dino_character) (Variables|Default|GetTargetingTeam))
        (LocalVariables|SetDamage 0.0)))
    (:then_1
      (if (== (.HitComponent (Collision|BreakHitResult PointHitInfo)) (Variables|Default|GetPlayerDetectSphere))
        (LocalVariables|SetDamage 0.0)))
    (:then_2
      (return (LocalVariables|GetDamage)))))

(fn OnRepHideRadiusEffect
  (if (not (Networking|IsDedicatedServer))
    (Rendering|SetVisibility (Variables|Default|GetEffectField) (not (Variables|Default|GetHideRadiusEffect)) false)))

(fn GetNearbyLeashDetails
  (params (LeashRef :type Actor%20Object%20Reference))
  (Utilities|FlowControl|Sequence
    (:then_0
      (bind _asstructure_dino_leash (Utilities|Casting|CastToStructure_DinoLeash LeashRef)
        (:then
          (if (and (Variables|/Game/Extinction/Structures/DinoLeash/Structure_DinoLeash.Structure_DinoLeash_C|GetActivated _asstructure_dino_leash) (Variables|/Script/ShooterGame.PrimalStructureItemContainer|GetbIsPowered _asstructure_dino_leash))
            (LocalVariables|SetbIsOtherLeashActive true)
            (LocalVariables|SetOtherLeashRadius (Variables|/Game/Extinction/Structures/DinoLeash/Structure_DinoLeash.Structure_DinoLeash_C|GetEffectRadius _asstructure_dino_leash))))
        (:CastFailed
          (bind _asbp_leash_tek (Utilities|Casting|CastToBP_LeashTek LeashRef))
          (if (Variables|BP_LeashTek_C|GetActivated _asbp_leash_tek)
            (LocalVariables|SetbIsOtherLeashActive true)
            (LocalVariables|SetOtherLeashRadius (Variables|BP_LeashTek_C|GetEffectRadius _asbp_leash_tek))))))
    (:then_1
      (return (LocalVariables|GetbIsOtherLeashActive) (LocalVariables|GetOtherLeashRadius)))))

(fn GetRandomDestination
  (bind _returnvalue (Math|Random|RandomFloatinRange 0.0 1.0))
  (bind _returnvalue_2 (Transformation|GetActorLocation))
  (LocalVariables|SetRadius_GRD (* (* (Variables|Default|GetEffectRadius) 0.5) (Math|Float|Sqrt _returnvalue)))
  (LocalVariables|SetTheta_GRD (* _returnvalue (Math|Trig|GetPI) 2.0))
  (return (Math|Vector|MakeVector (+ (* (LocalVariables|GetRadius_GRD) (Math|Trig|Cos(Radians) (LocalVariables|GetTheta_GRD))) (.x _returnvalue_2)) (+ (* (LocalVariables|GetRadius_GRD) (Math|Trig|Sin(Radians) (LocalVariables|GetTheta_GRD))) (.y _returnvalue_2)) (.z _returnvalue_2))))