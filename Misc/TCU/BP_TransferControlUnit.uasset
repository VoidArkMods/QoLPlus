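; Structures Plus Transfer Control Unit: a placeable structure that runs preset bulk transfers within a configured range, subject to a cooldown.
; The multi-use wheel selects the active preset, and the OmniTool buff edits presets through net exec commands.
; Use or PIN entry triggers the transfer, while container activation lights the emissive material until the server resets it.
; Per-team custom actor lists enforce the configurable tribe build limit.
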(event Custom|HandleBeginPlayEvent
  (Utilities|FlowControl|Delay 0 1.0)
  (CallFunction|SPAddtoCustomActorList self (Utilities|String|BuildString(Integer) "SPlusTCUs_" "" (Variables|Default|GetTargetingTeam))))

(event EventBPContainerActivated
  (bind _activemat (Variables|Default|GetActiveMat))
  (Utilities|FlowControl|Sequence
    (:then_0
      (Utilities|IsValid _activemat
        (:Is%20Valid
          (Rendering|Material|SetVectorParameterValue _activemat "Emissive - Color and Intensity" "(R=0.000000,G=1.000000,B=0.165230,A=2.000000)" :!class /Script/Engine.MaterialInstanceDynamic))))
    (:then_1
      (Class|KismetSystemLibrary|IsRunningonServer
        (:Yes
          (Utilities|FlowControl|Delay 0 (Variables|Default|GetPullCooldown))
          (Class|PrimalStructure|SetContainerActive false))))))

(event EventBPContainerDeactivated
  (bind _activemat (Variables|Default|GetActiveMat))
  (Utilities|IsValid _activemat
    (:Is%20Valid
      (Rendering|Material|SetVectorParameterValue _activemat "Emissive - Color and Intensity" "(R=0.000000,G=0.000000,B=0.000000,A=1.000000)" :!class /Script/Engine.MaterialInstanceDynamic))))

(fn ConstructionScript
  (|CallParentFunction)
  (if (and (not (Variables|Default|GetbIsPreviewStructure)) (not (Networking|IsDedicatedServer)))
    (bind _returnvalue (Rendering|Material|CreateDynamicMaterialInstance 0 "/Game/Genesis/Dinos/HLNA/HLN_A_Colorized_MIC.HLN_A_Colorized_MIC" "None" :!class /Script/Engine.KismetMaterialLibrary))
    (Variables|Default|SetActiveMat _returnvalue)
    (Rendering|Material|SetMaterial (Variables|Default|GetStaticMesh1) 0 _returnvalue)
    (Rendering|Material|SetVectorParameterValue :self _returnvalue :ParameterName "Emissive - Color and Intensity" :!class /Script/Engine.MaterialInstanceDynamic)))

(fn BPGetMultiUseEntries
  (params (ForPC :type Player%20Controller%20Object%20Reference) (MultiUseEntries :type Array%20of%20Multi%20Use%20Entry%20Structures))
  (bind _color (CallFunction|SPGetMultiUseSpecialColor))
  (bind _self self)
  (bind _returnvalue (Math|Conversions|ToColor(LinearColor) _color))
  (bind _entriesout (CallFunction|SPUpdateMultiUseMenu ForPC MultiUseEntries _self false false false false))
  (Utilities|FlowControl|Sequence
    (:then_0
      (bind _accesslevel (CallFunction|SPGetAccessLevel ForPC _self))
      (if (>= _accesslevel 2)
        (Utilities|Array|Add _entriesout (Utilities|Struct|MakeMultiUseEntry "[Edit Transfers]" 9000 -1000 true false 0 _returnvalue))
        (Utilities|Array|Add _entriesout (Utilities|Struct|MakeMultiUseEntry "[Set Active Transfer]" 9001 -1000 true true true false 0 _returnvalue))
        (for (_array_element _array_index) (Variables|Default|GetPresetNames)
          (Utilities|Array|Add _entriesout (Utilities|Struct|MakeMultiUseEntry _array_element (+ _array_index 9002) _array_index (== _array_index (Variables|Default|GetActiveTransferIndex)) false 0 9001 _returnvalue)))))
    (:then_1
      (return _entriesout))))

(fn ReceiveBeginPlay
  (bind _returnvalue (Game|GetGameMode))
  (|CallParentFunction)
  (if (not (Variables|Default|GetbIsPreviewStructure))
    (Networking|SwitchHasAuthority
      (:Authority
        (Utilities|FlowControl|Sequence
          (:then_0
            (bind (_disablepulling _pullrange _cooldown) (CallFunction|SPGetConfigSetting-Pull _returnvalue))
            (Variables|Default|SetPullRange _pullrange)
            (Variables|Default|SetPullCooldown _cooldown false))
          (:then_1
            (bind _value (CallFunction|SPGetConfig-Int _returnvalue "TribeTCULimit" 0 0 999999))
            (Variables|Default|SetTribeLimit _value)
            (if (> _value 0)
              (CallFunction|HandleBeginPlayEvent))))))))

(fn BPTryMultiUse
  (params (ForPC :type Player%20Controller%20Object%20Reference) (UseIndex :type Integer))
  (Utilities|FlowControl|Sequence
    (:then_0
      (switch int UseIndex
        (:Default
          (if (== UseIndex 600)
            (CallFunction|PerformTransfer ForPC)))
        (:9000
          (bind _asshooter_player_controller (Utilities|Casting|CastToShooterPlayerController ForPC))
          (bind _returnvalue (Class|PrimalBuff|StaticAddBuff "/QoLPlus/_Buffs/Buff_StructuresPlus_OmniTool.Buff_StructuresPlus_OmniTool_C" (Class|ShooterPlayerController|GetPlayerCharacter _asshooter_player_controller) 0 0 false))
          (bind _asbuff_structures_plus_omni_tool (Utilities|Casting|CastToBuff_StructuresPlus_OmniTool _returnvalue))
          (Default|Transfer-InitializeUIfromStructure _asbuff_structures_plus_omni_tool self (Variables|Default|GetPresets) (Variables|Default|GetPresetNames)))
        (:9002
          (Variables|Default|SetActiveTransferIndex 0 true))
        (:9003
          (Variables|Default|SetActiveTransferIndex 1 true))
        (:9004
          (Variables|Default|SetActiveTransferIndex 2 true))
        (:9005
          (Variables|Default|SetActiveTransferIndex 3 true))
        (:9006
          (Variables|Default|SetActiveTransferIndex 4 true))))
    (:then_1
      (return true))))

(fn BPServerHandleNetExecCommand
  (params (FromPC :type Player%20Controller%20Object%20Reference) (CommandName :type Name :default "None") (ExecParams :type BP%20Net%20Exec%20Params%20Structure%20%28by%20ref%29))
  (bind (_intparam1 _intarrayparam1 _floatarrayparam1 _objparam1 _stringparam1) (Utilities|Struct|BreakBPNetExecParams ExecParams))
  (bind _presets (Variables|Default|GetPresets))
  (Utilities|FlowControl|Sequence
    (:then_0
      (switch name CommandName
        (:SetPreset
          (bind _assplus_omnitool_com_object (Utilities|Casting|CastToSPlus_Omnitool_ComObject _objparam1))
          (if (Utilities|Array|IsValidIndex (Variables|/QoLPlus/_ComObjects/SPlus_Omnitool_ComObject.SPlus_Omnitool_ComObject_C|GetTransferData _assplus_omnitool_com_object))
            (Utilities|Array|SetArrayElem (Variables|Default|GetPresets) _intparam1 (Utilities|Array|Get(acopy) (Variables|/QoLPlus/_ComObjects/SPlus_Omnitool_ComObject.SPlus_Omnitool_ComObject_C|GetTransferData _assplus_omnitool_com_object)))))
        (:SetPresetName
          (Utilities|Array|SetArrayElem (Variables|Default|GetPresetNames) _intparam1 _stringparam1)
          (Class|PrimalActor|MulticastProperty "PresetNames" false))
        (:ApplyPresets
          (bind _assplus_omnitool_com_object_2 (Utilities|Casting|CastToSPlus_Omnitool_ComObject _objparam1))
          (Utilities|Array|Clear _presets)
          (Utilities|Array|AppendArray _presets (Variables|/QoLPlus/_ComObjects/SPlus_Omnitool_ComObject.SPlus_Omnitool_ComObject_C|GetTransferData _assplus_omnitool_com_object_2)))
        (:GetTransferPresetsFromStructure
          (bind _asprimal_buff (Utilities|Casting|CastToPrimalBuff _objparam1))
          (bind _returnvalue (Class|VictoryCore|ConstructObjectAutoNameBP "/QoLPlus/_ComObjects/SPlus_Omnitool_ComObject.SPlus_Omnitool_ComObject_C" _asprimal_buff))
          (bind _assplus_omnitool_com_object_3 (Utilities|Casting|CastToSPlus_Omnitool_ComObject _returnvalue))
          (Utilities|Array|AppendArray (Variables|/QoLPlus/_ComObjects/SPlus_Omnitool_ComObject.SPlus_Omnitool_ComObject_C|GetTransferData _assplus_omnitool_com_object_3) (Variables|Default|GetPresets))
          (CallFunction|BPServerHandleNetExecCommand _asprimal_buff FromPC "GetTransferPresetsFromStructure" (Utilities|Struct|MakeBPNetExecParams 0 0 _assplus_omnitool_com_object_3))
          (for (_array_element _array_index) (Variables|Default|GetPresetNames)
            (CallFunction|BPServerHandleNetExecCommand _asprimal_buff FromPC "Transfer_SavePresetName" (Utilities|Struct|MakeBPNetExecParams _array_index 0 0 _array_element))))))
    (:then_1
      (return true))))

(fn BPCanbeActivatedbyPlayer
  (params (PC :type Shooter%20Player%20Controller%20Object%20Reference))
  (return (and (>= (Class|VictoryCore|GetNetworkTimeinSeconds) (+ (Variables|Default|GetLastPullTime) (Variables|Default|GetPullCooldown))) (not (Variables|Default|GetbContainerActivated)))))

(fn PerformTransfer
  (params (PC :type Player%20Controller%20Object%20Reference))
  (bind _presets (Variables|Default|GetPresets))
  (bind _activetransferindex (Variables|Default|GetActiveTransferIndex))
  (if (>= (Class|VictoryCore|GetNetworkTimeinSeconds) (+ (Variables|Default|GetLastPullTime) (Variables|Default|GetPullCooldown)))
    (if (Utilities|Array|IsValidIndex _presets _activetransferindex)
      (bind _log (CallFunction|SPDoBulkTransfer PC (Utilities|Array|Get(acopy) _presets _activetransferindex) (Transformation|GetActorLocation) (Variables|Default|GetPullRange)))
      (Utilities|FlowControl|Sequence
        (:then_0
          (if (Utilities|Array|IsValidIndex _log (Utilities|Array|LastIndex _log))
            (CallFunction|SPMessageClient PC (Utilities|Array|Get(acopy) _log (Utilities|Array|LastIndex _log)))))
        (:then_1
          (Variables|Default|SetLastPullTime (Class|VictoryCore|GetNetworkTimeinSeconds) true))))))

(fn BPClientDoMultiUse
  (params (ForPC :type Player%20Controller%20Object%20Reference) (ClientUseIndex :type Integer))
  (bind _asshooter_player_controller (Utilities|Casting|CastToShooterPlayerController ForPC))
  (switch int ClientUseIndex
    (:9001
      (Class|ShooterPlayerController|SetMultiUseWheelCategory _asshooter_player_controller ClientUseIndex 0 0))))

(fn BPConsumeUsePinCode
  (params (FromKeypadActor :type Actor%20Object%20Reference) (ForPC :type Player%20Controller%20Object%20Reference) (appledPinCode :type Integer) (bIsActivating :type Boolean))
  (Utilities|FlowControl|Sequence
    (:then_0
      (if (and bIsActivating (Class|PrimalStructureItemContainer|VerifyPinCode appledPinCode))
        (CallFunction|PerformTransfer ForPC)))
    (:then_1
      (return false))))

(fn BPIsAllowedtoBuildEx
  (params (OutPlacementData :type Placement%20Data%20Structure%20%28by%20ref%29) (CurrentAllowedReason :type Integer) (PC :type Player%20Controller%20Object%20Reference) (bFinalPlacement :type Boolean) (bChoosingRotation :type Boolean))
  (bind _buildreason (CallFunction|SPCheckTribeLimit self "TCU" CurrentAllowedReason (Variables|Default|GetTribeLimit) (Utilities|String|BuildString(Integer) "SPlusTCUs_" "" (Variables|Default|GetTargetingTeam)) bFinalPlacement PC))
  (return _buildreason))

(fn ReceiveDestroyed
  (Networking|SwitchHasAuthority
    (:Authority
      (if (not (Variables|Default|GetbIsPreviewStructure))
        (CallFunction|SPRemovefromCustomActorList self (Utilities|String|BuildString(Integer) "SPlusTCUs_" "" (Variables|Default|GetTargetingTeam)))))))

(fn BPonStructurePickup
  (params (PlayerController :type Player%20Controller%20Object%20Reference) (ItemType :type Primal%20Item%20Class%20Reference) (NewlyPickedUpItem :type Primal%20Item%20Object%20Reference) (bIsQuickPickup :type Boolean))
  (Networking|SwitchHasAuthority
    (:Authority
      (CallFunction|SPRemovefromCustomActorList self (Utilities|String|BuildString(Integer) "SPlusTCUs_" "" (Variables|Default|GetTargetingTeam))))))