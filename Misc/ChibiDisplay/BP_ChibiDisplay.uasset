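; BP_ChibiDisplay is a Structures Plus placeable that showcases a chibi dino skin item in a hideable frame.
; Multi-use entries store or take chibis through its inventory, set yaw, or copy it to linked displays.
; Replicated ChibiData carries presence and yaw; its OnRep polls each tick for the skin component, then applies per-class transforms.
; Placement can toggle snapping, and non-shipping builds can cycle chibis from the MultiTool conversion list.
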(event Custom|TriggerChibiUpdate
  (Utilities|IsValid (Actor|GetComponentbyClass "/Game/PrimalEarth/CoreBlueprints/Items/Armor/Skin/ChibiDinos/SKComponent_SkinAttachment_ChibiDino.SKComponent_SkinAttachment_ChibiDino_C")
    (:Is%20Valid
      (CallFunction|UpdateChibiMesh))
    (:Is%20Not%20Valid
      (Class|KismetSystemLibrary|SetTimerforNextTick 0 "TriggerChibiUpdate" false))))

(event Input|ActionEvents|InputActionDrag
  (params (Key :type Key%20Structure :default "None"))
  (:Pressed
    (bind _returnvalue (Class|Actor|GetOwnerController))
    (bind _success (CallFunction|SPToggleGlobalBuffDisabledSnaps _returnvalue (Utilities|Array|MakeArray) (Utilities|Array|MakeArray 1) (not (Variables|Default|GetDisableSnaps))))
    (if _success
      (Variables|Default|SetDisableSnaps (not (Variables|Default|GetDisableSnaps))))))

(fn ConstructionScript
  (|CallParentFunction))

(fn BPIsAllowedtoBuild
  (params (OutPlacementData :type Placement%20Data%20Structure%20%28by%20ref%29) (CurrentAllowedReason :type Integer))
  (return (Math|Integer|SelectInt 1 CurrentAllowedReason (== CurrentAllowedReason -9))))

(fn BPGetMultiUseEntries
  (params (ForPC :type Player%20Controller%20Object%20Reference) (MultiUseEntries :type Array%20of%20Multi%20Use%20Entry%20Structures))
  (bind _color (CallFunction|SPGetMultiUseSpecialColor))
  (bind _self self)
  (bind _returnvalue (Math|Conversions|ToColor(LinearColor) _color))
  (bind _entriesout (CallFunction|SPUpdateMultiUseMenu ForPC MultiUseEntries _self false false false false))
  (Utilities|FlowControl|Sequence
    (:then_0
      (bind _accesslevel (CallFunction|SPGetAccessLevel ForPC _self))
      (if (>= _accesslevel 2)
        (Utilities|Array|Add _entriesout (Utilities|Struct|MakeMultiUseEntry (Utilities|String|SelectString "Show Frame" "Hide Frame" (Variables|Default|GetHideFrame)) 9003 -250))
        (bind _returnvalue_2 (Class|PrimalInventoryComponent|GetEquippedItemOfClass (Variables|Default|GetMyInventoryComponent) "/Game/PrimalEarth/CoreBlueprints/Items/Armor/Skin/ChibiDinos/PrimalItemSkin_ChibiDino_Base.PrimalItemSkin_ChibiDino_Base_C"))
        (Utilities|IsValid _returnvalue_2
          (:Is%20Valid
            (Utilities|Array|Add _entriesout (Utilities|Struct|MakeMultiUseEntry "Take Chibi" 9001 5000))
            (Utilities|Array|Add _entriesout (Utilities|Struct|MakeMultiUseEntry "Apply Rotation to Connected" 9002 -50))
            (Utilities|Array|Add _entriesout (Utilities|Struct|MakeMultiUseEntry "[Set Rotation]" 9009 -49 true true true false 0 _returnvalue))
            (for (_array_element _array_index) (Variables|Default|GetAvailableRotations)
              (Utilities|Array|Add _entriesout (Utilities|Struct|MakeMultiUseEntry (Utilities|String|ToString(Integer) _array_element) (+ _array_index 9010) (* _array_index -1) (Math|Float|NearlyEqual(Float) (Math|Conversions|ToFloat(Integer) _array_element) (.Y (Math|Vector|BreakVector (Variables|Default|GetChibiData))) 0.01) true false 0 9009 _returnvalue))))
          (:Is%20Not%20Valid
            (bind _asshooter_player_controller (Utilities|Casting|CastToShooterPlayerController ForPC))
            (bind _returnvalue_3 (Class|PrimalInventoryComponent|BPGetItemOfTemplate (Variables|/Script/ShooterGame.PrimalCharacter|GetMyInventoryComponent (Class|ShooterPlayerController|GetPlayerCharacter _asshooter_player_controller)) "/Game/PrimalEarth/CoreBlueprints/Items/Armor/Skin/ChibiDinos/PrimalItemSkin_ChibiDino_Base.PrimalItemSkin_ChibiDino_Base_C" false false false false false false false false false false))
            (Utilities|IsValid _returnvalue_3
              (:Is%20Valid
                (Utilities|Array|Add _entriesout (Utilities|Struct|MakeMultiUseEntry "Store Chibi" 9000 5000))))))))
    (:then_1
      (if (not (Class|VictoryCore|IsShipping))
        (Utilities|Array|Add _entriesout (Utilities|Struct|MakeMultiUseEntry "Next Chibi" 11111 15000 true))
        (Utilities|Array|Add _entriesout (Utilities|Struct|MakeMultiUseEntry "Prev Chibi" 11112 14000 true))))
    (:then_2
      (return _entriesout))))

(fn BPTryMultiUse
  (params (ForPC :type Player%20Controller%20Object%20Reference) (UseIndex :type Integer))
  (bind _returnvalue (Class|KismetSystemLibrary|MakeLiteralInteger 9010))
  (bind _availablerotations (Variables|Default|GetAvailableRotations))
  (Utilities|FlowControl|Sequence
    (:then_0
      (switch int UseIndex
        (:Default
          (if (== UseIndex 601)
            (Variables|Default|SetIsUnlocked (not (Variables|Default|GetbIsLocked)))
            (elif (and (>= UseIndex _returnvalue) (<= UseIndex (+ _returnvalue (Utilities|Array|LastIndex _availablerotations))))
              (Variables|Default|SetChibiData (Math|Vector|MakeVector (.X (Math|Vector|BreakVector (Variables|Default|GetChibiData))) (Math|Conversions|ToFloat(Integer) (Utilities|Array|Get(acopy) _availablerotations (- UseIndex _returnvalue))) 0.0) true)
              (elif (not (Class|VictoryCore|IsShipping))
                (bind _items (CallFunction|GetAvailableChibiItems))
                (switch int UseIndex
                  (:11111
                    (Variables|Default|SetCurChibiIndex (Math|Integer|SelectInt (+ (Variables|Default|GetCurChibiIndex) 1) 0 (>= (Utilities|Array|LastIndex _items) (+ (Variables|Default|GetCurChibiIndex) 1))) true))
                  (:11112
                    (Variables|Default|SetCurChibiIndex (Math|Integer|SelectInt (Utilities|Array|LastIndex _items) (- (Variables|Default|GetCurChibiIndex) 1) (< (- (Variables|Default|GetCurChibiIndex) 1) 0)) true)))))))
        (:9000
          (CallFunction|StoreChibi ForPC))
        (:9001
          (CallFunction|TakeChibi ForPC))
        (:9002
          (CallFunction|ApplyRotationtoConnected))
        (:9003
          (Variables|Default|SetHideFrame (not (Variables|Default|GetHideFrame)) true))))
    (:then_1
      (return true))))

(fn ReceiveBeginPlay
  (|CallParentFunction)
  (if (Variables|Default|GetbIsPreviewStructure)
    (bind _returnvalue (Class|Actor|GetOwnerController))
    (Input|EnableInput _returnvalue)
    (CallFunction|SPClearGlobalBuffDisabledSnaps _returnvalue)
    (else
      (Networking|SwitchHasAuthority
        (:Authority
          (Utilities|FlowControl|Sequence
            (:then_0
              (Variables|Default|SetbIsLocked (not (Variables|Default|GetIsUnlocked)) true))
            (:then_1
              (Utilities|SwitchNetAuthority
                (:PlayerServer
                  (CallFunction|OnRepChibiData)
                  (CallFunction|OnRepHideFrame))))))))))

(fn IsValidSnapPointfrom
  (params (ParentStructure :type Primal%20Structure%20Object%20Reference) (MySnapPointFromIndex :type Integer))
  (return (not (Variables|Default|GetDisableSnaps))))

(fn BPSetPlayerConstructor
  (params (PC :type Player%20Controller%20Object%20Reference))
  (bind _asbuff_structures_plus_global_buff (Utilities|Casting|CastToBuff_StructuresPlus_GlobalBuff (CallFunction|SPGetGlobalBuff PC)))
  (Variables|Default|SetDisableSnaps (> (Utilities|Array|Length (Variables|/QoLPlus/_Buffs/Buff_StructuresPlus_GlobalBuff.Buff_StructuresPlus_GlobalBuff_C|GetDisabledSnapsFrom _asbuff_structures_plus_global_buff)) 0))
  (CallFunction|SPClearGlobalBuffDisabledSnaps PC))

(fn OnRepChibiData
  (Class|KismetSystemLibrary|CanRunCosmeticEvents
    (:Yes
      (if (> (.X (Math|Vector|BreakVector (Variables|Default|GetChibiData))) 0.0)
        (CallFunction|TriggerChibiUpdate)))))

(fn BPClientDoMultiUse
  (params (ForPC :type Player%20Controller%20Object%20Reference) (ClientUseIndex :type Integer))
  (bind _asshooter_player_controller (Utilities|Casting|CastToShooterPlayerController ForPC))
  (switch int ClientUseIndex
    (:9009
      (Class|ShooterPlayerController|SetMultiUseWheelCategory _asshooter_player_controller ClientUseIndex 0 0))))

(fn ApplyRotationtoConnected
  (bind _self self)
  (bind _asprimal_structure (Utilities|Casting|CastToPrimalStructureClass (Utilities|GetClass _self)))
  (bind _connectedstructures (CallFunction|SPGetLinkedStructures _self true (Utilities|Array|MakeArray _asprimal_structure) (Utilities|Array|MakeArray)))
  (for _array_element _connectedstructures
    (bind _asbp_chibi_display (Utilities|Casting|CastToBP_ChibiDisplay _array_element))
    (Variables|BP_ChibiDisplay_C|SetChibiData _asbp_chibi_display (Math|Vector|MakeVector (.X (Math|Vector|BreakVector (Variables|BP_ChibiDisplay_C|GetChibiData _asbp_chibi_display))) (.Y (Math|Vector|BreakVector (Variables|Default|GetChibiData))) 0.0) false)
    (Class|PrimalActor|MulticastProperty _asbp_chibi_display "ChibiData" false)))

(fn UpdateChibiMesh
  (bind _returnvalue (Transformation|GetActorRotation))
  (LocalVariables|SetComponents_UCM (Actor|GetComponentsByClass "/Game/PrimalEarth/CoreBlueprints/Items/Armor/Skin/ChibiDinos/SKComponent_SkinAttachment_ChibiDino.SKComponent_SkinAttachment_ChibiDino_C"))
  (for _array_element (LocalVariables|GetComponents_UCM)
    (bind _asskcomponent_skin_attachment_chibi_dino (Utilities|Casting|CastToSKComponent_SkinAttachment_ChibiDino _array_element))
    (Default|AttachSubMeshes _asskcomponent_skin_attachment_chibi_dino)
    (bind (_scale _locoffset _rotoffset) (CallFunction|GetChibiTransform _asskcomponent_skin_attachment_chibi_dino))
    (Transformation|SetWorldTransform _asskcomponent_skin_attachment_chibi_dino (Math|Transform|MakeTransform (+ (Math|Vector|RotateVector _locoffset _returnvalue) (Math|Vector|RotateVector (Variables|/Game/PrimalEarth/CoreBlueprints/Items/Armor/Skin/ChibiDinos/SKComponent_SkinAttachment_ChibiDino.SKComponent_SkinAttachment_ChibiDino_C|GetGroundedPositionOffset _asskcomponent_skin_attachment_chibi_dino) _returnvalue) (Transformation|GetWorldLocation (Variables|Default|GetBottom_Mesh))) (Math|Rotator|CombineRotators _rotoffset (Math|Rotator|CombineRotators (Math|Rotator|CombineRotators _returnvalue (Math|Rotator|MakeRotator 0.0 0.0 (.y (Variables|Default|GetChibiData)))) "0,90.000000, 0")) _scale) false false)
    (Rendering|SetVisibility _asskcomponent_skin_attachment_chibi_dino true true)))

(fn StoreChibi
  (params (PC :type Player%20Controller%20Object%20Reference))
  (bind _chibis (CallFunction|GetChibis PC))
  (switch int (Utilities|Array|Length _chibis)
    (:Default
      (for _array_element _chibis
        (bind _returnvalue (Default|BPGetItemName _array_element))
        (Utilities|Array|Add (LocalVariables|GetChibisInInventory_SC) (Utilities|Struct|MakeSP_AlphabetizationObject _returnvalue _array_element)))
      (bind _asshooter_player_controller (Utilities|Casting|CastToShooterPlayerController PC))
      (bind _returnvalue_2 (Class|PrimalBuff|StaticAddBuff "/QoLPlus/_Buffs/Buff_StructuresPlus_SelectBoxFilter.Buff_StructuresPlus_SelectBoxFilter_C" (Class|ShooterPlayerController|GetPlayerCharacter _asshooter_player_controller) 0 0 false))
      (bind _asbuff_structures_plus_select_box_filter (Utilities|Casting|CastToBuff_StructuresPlus_SelectBoxFilter _returnvalue_2))
      (Default|InitializeUI _asbuff_structures_plus_select_box_filter "Select a Chibi:" (LocalVariables|GetChibisInInventory_SC) self "SelectChibi" false true false))
    (:0
      (CallFunction|SPMessageClient PC "No Chibi Found."))
    (:1
      (CallFunction|SelectChibi PC (Utilities|Array|Get(acopy) _chibis)))))

(fn TakeChibi
  (params (PC :type Player%20Controller%20Object%20Reference))
  (bind _returnvalue (Class|PrimalInventoryComponent|GetEquippedItemOfClass (Variables|Default|GetMyInventoryComponent) "/Game/PrimalEarth/CoreBlueprints/Items/Armor/Skin/ChibiDinos/PrimalItemSkin_ChibiDino_Base.PrimalItemSkin_ChibiDino_Base_C"))
  (Utilities|IsValid _returnvalue
    (:Is%20Valid
      (bind _asshooter_player_controller (Utilities|Casting|CastToShooterPlayerController PC))
      (bind _returnvalue_2 (Class|PrimalInventoryComponent|AddItemObject (Variables|/Script/ShooterGame.PrimalCharacter|GetMyInventoryComponent (Class|ShooterPlayerController|GetPlayerCharacter _asshooter_player_controller)) _returnvalue))
      (Utilities|IsValid _returnvalue_2
        (:Is%20Valid
          (Class|PrimalInventoryComponent|RemoveItem (Variables|Default|GetMyInventoryComponent) (Variables|/Script/ShooterGame.PrimalItem|GetItemID _returnvalue) false false true false)
          (Variables|Default|SetChibiData (Math|Vector|MakeVector -1.0 (.y (Variables|Default|GetChibiData)) 0.0) true))))))

(fn SelectChibi
  (params (PC :type Player%20Controller%20Object%20Reference) (ChibiItem :type Primal%20Item%20Skin%20Chibi%20Dino%20Base%20Object%20Reference))
  (Utilities|IsValid ChibiItem
    (:Is%20Valid
      (bind _asshooter_player_controller (Utilities|Casting|CastToShooterPlayerController PC))
      (bind _returnvalue (Class|PrimalInventoryComponent|AddItemObjectEx (Variables|Default|GetMyInventoryComponent) ChibiItem true false false true false false 0 false 0 false))
      (Utilities|IsValid _returnvalue
        (:Is%20Valid
          (Class|PrimalInventoryComponent|RemoveItem (Variables|/Script/ShooterGame.PrimalCharacter|GetMyInventoryComponent (Class|ShooterPlayerController|GetPlayerCharacter _asshooter_player_controller)) (Variables|/Script/ShooterGame.PrimalItem|GetItemID ChibiItem) false false true true)
          (Variables|Default|SetChibiData (Math|Vector|MakeVector 1.0 (.y (Variables|Default|GetChibiData)) 0.0) true))))))

(fn GetChibis
  (params (PC :type Player%20Controller%20Object%20Reference))
  (Utilities|FlowControl|Sequence
    (:then_0
      (bind _asshooter_player_controller (Utilities|Casting|CastToShooterPlayerController PC))
      (bind _returnvalue (Class|PrimalInventoryComponent|FindAllItemsOfType (Variables|/Script/ShooterGame.PrimalCharacter|GetMyInventoryComponent (Class|ShooterPlayerController|GetPlayerCharacter _asshooter_player_controller)) "/Game/PrimalEarth/CoreBlueprints/Items/Armor/Skin/ChibiDinos/PrimalItemSkin_ChibiDino_Base.PrimalItemSkin_ChibiDino_Base_C" false true true false false false false))
      (for _array_element _returnvalue
        (bind _asprimal_item_skin_chibi_dino_base (Utilities|Casting|CastToPrimalItemSkin_ChibiDino_Base _array_element))
        (Utilities|Array|Add (LocalVariables|GetChibis_GC) _asprimal_item_skin_chibi_dino_base)))
    (:then_1
      (return (LocalVariables|GetChibis_GC)))))

(fn BPServerHandleNetExecCommand
  (params (FromPC :type Player%20Controller%20Object%20Reference) (CommandName :type Name :default "None") (ExecParams :type BP%20Net%20Exec%20Params%20Structure%20%28by%20ref%29))
  (Utilities|FlowControl|Sequence
    (:then_0
      (Utilities|IsValid FromPC
        (:Is%20Valid
          (switch name CommandName
            (:SelectChibi
              (bind _asprimal_item_skin_chibi_dino_base (Utilities|Casting|CastToPrimalItemSkin_ChibiDino_Base (.ObjParam1 (Utilities|Struct|BreakBPNetExecParams ExecParams))))
              (CallFunction|SelectChibi FromPC _asprimal_item_skin_chibi_dino_base))))))
    (:then_1
      (return true))))

(fn GetChibiTransform
  (params (SK_Comp :type SK%20Component%20Skin%20Attachment%20Chibi%20Dino%20Object%20Reference))
  (bind _displayscale (Variables|/Game/PrimalEarth/CoreBlueprints/Items/Armor/Skin/ChibiDinos/SKComponent_SkinAttachment_ChibiDino.SKComponent_SkinAttachment_ChibiDino_C|GetDisplayScale SK_Comp))
  (Utilities|FlowControl|Sequence
    (:then_0
      (LocalVariables|SetChibiOffset_GCT (Math|Transform|MakeTransform "0, 0, 0" "0, 0, 0" _displayscale))
      (bind _returnvalue (Class|PrimalInventoryComponent|GetEquippedItemOfClass (Variables|Default|GetMyInventoryComponent) "/Game/PrimalEarth/CoreBlueprints/Items/Armor/Skin/ChibiDinos/PrimalItemSkin_ChibiDino_Base.PrimalItemSkin_ChibiDino_Base_C"))
      (Utilities|IsValid _returnvalue
        (:Is%20Valid
          (bind _array_element (Utilities|Array|ForEachLoopwithBreak (Variables|Default|GetChibiTransforms) :!label _label)
            (:LoopBody
              (if (== (.ChibiItemClass (Utilities|Struct|BreakSP_ChibiTransform _array_element)) (Utilities|GetClass _returnvalue))
                (LocalVariables|SetChibiOffset_GCT (Math|Transform|MakeTransform (.LocOffset (Utilities|Struct|BreakSP_ChibiTransform _array_element)) (.RotOffset (Utilities|Struct|BreakSP_ChibiTransform _array_element)) (Math|Vector|SelectVector _displayscale (.Scale (Utilities|Struct|BreakSP_ChibiTransform _array_element)) (Class|KismetMathLibrary|NearlyEqualVectorVector (.Scale (Utilities|Struct|BreakSP_ChibiTransform _array_element)) "0, 0, 0" 1e-06))))
                (goto _label Break)))))))
    (:then_1
      (return (.scale (LocalVariables|GetChibiOffset_GCT)) (Math|Vector|MakeVector (.X (Math|Vector|BreakVector (.location (LocalVariables|GetChibiOffset_GCT)))) (+ (- (.x (Variables|/Game/PrimalEarth/CoreBlueprints/Items/Armor/Skin/ChibiDinos/SKComponent_SkinAttachment_ChibiDino.SKComponent_SkinAttachment_ChibiDino_C|GetDisplayLocOffset SK_Comp)) 1e+02) (.Y (Math|Vector|BreakVector (.location (LocalVariables|GetChibiOffset_GCT))))) (.Z (Math|Vector|BreakVector (.location (LocalVariables|GetChibiOffset_GCT))))) (.rotation (LocalVariables|GetChibiOffset_GCT))))))

(fn GetAvailableChibiItems
  (bind _chibiitems (Variables|Default|GetChibiItems))
  (Utilities|FlowControl|Sequence
    (:then_0
      (if (== (Utilities|Array|Length _chibiitems) 0)
        (bind _returnvalue (Class|VictoryCore|GetClassDefaultObject "/QoLPlus/_Buffs/Buff_StructuresPlus_MultiTool.Buff_StructuresPlus_MultiTool_C"))
        (bind _asbuff_structures_plus_multi_tool (Utilities|Casting|CastToBuff_StructuresPlus_MultiTool _returnvalue))
        (for _array_element (Variables|/QoLPlus/_Buffs/Buff_StructuresPlus_MultiTool.Buff_StructuresPlus_MultiTool_C|GetChibiDinoConversions _asbuff_structures_plus_multi_tool)
          (for _array_element_2 (.ToClasses (Utilities|Struct|BreakClassRemappingWeight _array_element))
            (bind _asprimal_item (Utilities|Casting|CastToPrimalItemClass (Utilities|ResolveSoftReference _array_element_2)))
            (Utilities|Array|AddUnique (Variables|Default|GetChibiItems) _asprimal_item)))))
    (:then_1
      (return _chibiitems))))

(fn OnRepCurChibiIndex
  (bind _curchibiindex (Variables|Default|GetCurChibiIndex))
  (if (not (Class|VictoryCore|IsShipping))
    (Utilities|SwitchNetAuthority
      (:DedicatedServer
        _)
      (:PlayerServer
        _))
    (Utilities|FlowControl|Sequence
      (:then_0
        (bind _returnvalue (Class|PrimalInventoryComponent|GetEquippedItemOfClass (Variables|Default|GetMyInventoryComponent) "/Game/PrimalEarth/CoreBlueprints/Items/Armor/Skin/ChibiDinos/PrimalItemSkin_ChibiDino_Base.PrimalItemSkin_ChibiDino_Base_C"))
        (Utilities|IsValid _returnvalue
          (:Is%20Valid
            (Class|PrimalInventoryComponent|RemoveItem (Variables|Default|GetMyInventoryComponent) (Variables|/Script/ShooterGame.PrimalItem|GetItemID _returnvalue) false false true false)
            (Variables|Default|SetChibiData (Math|Vector|MakeVector 0.0 0.0 0.0) true))))
      (:then_1
        (bind _items (CallFunction|GetAvailableChibiItems))
        (if (>= (Utilities|Array|LastIndex _items) _curchibiindex)
          (Class|PrimalItem|AddNewItem (Utilities|Array|Get(acopy) _items _curchibiindex) (Variables|Default|GetMyInventoryComponent) true false 0.0 false 1 false 0.0 false 0 0.0 false false false)
          (Development|PrintString 0 (Utilities|GetClassDisplayName (Utilities|Array|Get(acopy) _items _curchibiindex)))
          (Variables|Default|SetChibiData (Math|Vector|MakeVector 1.0 0.0 0.0) true))))))

(fn OnRepHideFrame
  (Class|KismetSystemLibrary|CanRunCosmeticEvents
    (:Yes
      (Rendering|SetVisibility (Variables|Default|GetScene_Top) (not (Variables|Default|GetHideFrame)) true))))