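; Item collector structure that gathers ground items and selected creature resources, and can distribute poop to compost bins and beetles.
; On the authority, BeginPlay applies server config for slots, range and distribution, and resets collection settings.
; While active, DoScan reschedules itself, collecting ground items each tick plus one round-robin secondary scan from ActiveScans.
; Multi-use entries open the options UI or toggle poop distribution; net exec commands update settings and item lists.
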(fn ConstructionScript
  (|CallParentFunction))

(fn BPServerHandleNetExecCommand
  (params (FromPC :type Player%20Controller%20Object%20Reference) (CommandName :type Name :default "None") (ExecParams :type BP%20Net%20Exec%20Params%20Structure%20%28by%20ref%29))
  (bind _objparam1 (Utilities|Struct|BreakBPNetExecParams ExecParams))
  (Utilities|FlowControl|Sequence
    (:then_0
      (Utilities|IsValid FromPC
        (:Is%20Valid
          (bind _assplus_item_collector_com_object (Utilities|Casting|CastToSPlus_ItemCollector_ComObject _objparam1)
            (:then
              (switch name CommandName
                (:ItemCollector_CollectSettings
                  (Variables|Default|SetCollectData_Ground (Variables|/QoLPlus/_ComObjects/SPlus_ItemCollector_ComObject.SPlus_ItemCollector_ComObject_C|GetCollectData _assplus_item_collector_com_object))
                  (Variables|Default|SetCollectData_Inventory (Variables|/QoLPlus/_ComObjects/SPlus_ItemCollector_ComObject.SPlus_ItemCollector_ComObject_C|GetInvCollectData _assplus_item_collector_com_object))
                  (CallFunction|GetActiveScans))))
            (:CastFailed
              (bind _assplus_misc_com_object (Utilities|Casting|CastToSPlus_Misc_ComObject _objparam1))
              (switch name CommandName
                (:ItemCollector_CollectBlacklist
                  (Variables|Default|SetCollectionBlacklist (Variables|/QoLPlus/_ComObjects/SPlus_Misc_ComObject.SPlus_Misc_ComObject_C|GetObjectClasses _assplus_misc_com_object)))
                (:ItemCollector_CollectDestroylist
                  (Variables|Default|SetCollectionDestroylist (Variables|/QoLPlus/_ComObjects/SPlus_Misc_ComObject.SPlus_Misc_ComObject_C|GetObjectClasses _assplus_misc_com_object)))))))))
    (:then_1
      (return false))))

(fn ReceiveBeginPlay
  (bind _returnvalue (Game|GetGameMode))
  (|CallParentFunction)
  (if (not (Variables|Default|GetbIsPreviewStructure))
    (Networking|SwitchHasAuthority
      (:Authority
        (Utilities|FlowControl|Sequence
          (:then_0
            (bind _value (CallFunction|SPGetConfigSetting-InventorySize _returnvalue "ItemCollectorSlotCount" 300))
            (Variables|Default|SetInvSlotOverride _value true))
          (:then_1
            (bind _value_2 (CallFunction|SPGetConfig-Int _returnvalue "ItemCollectorRangeInFoundations" 25 1 100))
            (Variables|Default|SetScanRadius (* _value_2 3e+02) true))
          (:then_2
            (bind _value_3 (CallFunction|SPGetConfig-Bool _returnvalue "ItemCollectorDisableDistribution"))
            (Variables|Default|SetDisableDistribution _value_3 true))
          (:then_3
            (Utilities|Struct|SetmembersinSP_ItemCollectorDistributeData (Variables|Default|GetDistributeData) true true))
          (:then_4
            (Utilities|Struct|SetmembersinSP_ItemCollectorCollectData (Variables|Default|GetCollectData_Ground) false false false false false) ; Can remove after update... just to force clean old settings
            (Utilities|Struct|SetmembersinSP_ItemCollectorInvCollectData (Variables|Default|GetCollectData_Inventory) false false false false)
            (Utilities|Struct|SetmembersinSP_ItemCollectorDistributeData (Variables|Default|GetDistributeData) false 0 false false 0 false 0 false false false false))
          (:then_5
            (CallFunction|GetActiveScans)))))))

(fn BPGetMultiUseEntries
  (params (ForPC :type Player%20Controller%20Object%20Reference) (MultiUseEntries :type Array%20of%20Multi%20Use%20Entry%20Structures))
  (bind _returnvalue (|CallParentFunction ForPC MultiUseEntries))
  (Utilities|FlowControl|Sequence
    (:then_0
      (if (== (Variables|/Script/Engine.Actor|GetTargetingTeam ForPC) (Variables|Default|GetTargetingTeam))
        (Utilities|Array|Add _returnvalue (Utilities|Struct|MakeMultiUseEntry "[Collection Options]" 9002 -1005 true true false 0 (Math|Conversions|ToColor(LinearColor) (CallFunction|SPGetMultiUseSpecialColor))))
        (if (not (Variables|Default|GetDisableDistribution))
          (Utilities|Array|Add _returnvalue (Utilities|Struct|MakeMultiUseEntry (Utilities|String|SelectString "Distribute Poop to Bins & Beetles" "Stop Distributing Poop" (Variables|Default|GetDisablePoopDistribute)) 9003 -1005 true)))))
    (:then_1
      (return _returnvalue))))

(fn BPTryMultiUse
  (params (ForPC :type Player%20Controller%20Object%20Reference) (UseIndex :type Integer))
  (|CallParentFunction ForPC UseIndex)
  (Utilities|FlowControl|Sequence
    (:then_0
      (switch int UseIndex
        (:9002
          (bind _asshooter_player_controller (Utilities|Casting|CastToShooterPlayerController ForPC))
          (bind _returnvalue (Class|PrimalBuff|StaticAddBuff "/QoLPlus/_Buffs/Buff_StructuresPlus_ItemAggregator.Buff_StructuresPlus_ItemAggregator_C" (Class|ShooterPlayerController|GetPlayerCharacter _asshooter_player_controller) 0 0 false))
          (bind _asbuff_structures_plus_item_aggregator (Utilities|Casting|CastToBuff_StructuresPlus_ItemAggregator _returnvalue))
          (Default|InitializeUI-SimpleCollect _asbuff_structures_plus_item_aggregator self (Variables|Default|GetCollectData_Ground) (Variables|Default|GetCollectData_Inventory) (Variables|Default|GetCollectionBlacklist) (Variables|Default|GetCollectionDestroylist)))
        (:9003
          (Variables|Default|SetDisablePoopDistribute (not (Variables|Default|GetDisablePoopDistribute)) true)
          (CallFunction|GetActiveScans))))
    (:then_1
      (return true))))

(fn DoScan
  (bind _activescans (Variables|Default|GetActiveScans))
  (if (Variables|Default|GetbContainerActivated)
    (CallFunction|Collect-Ground)
    (Utilities|FlowControl|Sequence
      (:then_0
        (if (Utilities|Array|IsValidIndex _activescans)
          (Utilities|FlowControl|Sequence
            (:then_0
              (switch Utilities|FlowControl|Switch|SwitchonSP_Enum_AggregatorScanType (Utilities|Array|Get(acopy) _activescans (Variables|Default|GetSecondaryScanIndex))
                (:NewEnumerator7
                  (CallFunction|Collect-OilDinos))
                (:NewEnumerator8
                  (CallFunction|Collect-Sheep))
                (:NewEnumerator9
                  (CallFunction|Collect-Snails))
                (:NewEnumerator11
                  (CallFunction|Collect-Turtles))
                (:NewEnumerator13
                  (CallFunction|Distribute-Beetles))
                (:NewEnumerator14
                  (CallFunction|Distribute-CompostBins))))
            (:then_1
              (Variables|Default|SetSecondaryScanIndex (Math|Integer|SelectInt 0 (+ (Variables|Default|GetSecondaryScanIndex) 1) (> (+ (Variables|Default|GetSecondaryScanIndex) 1) (Utilities|Array|LastIndex (Variables|Default|GetActiveScans)))))))))
      (:then_1
        (Utilities|Time|SetTimerbyFunctionName 0 "DoScan" (CallFunction|GetScanInterval))))))

(fn GetActiveScans
  (bind _collectdata_inventory (Variables|Default|GetCollectData_Inventory))
  (bind (_organicpolymer _snailpaste _oil _rareflowers _raremushrooms) (Utilities|Struct|BreakSP_ItemCollectorInvCollectData _collectdata_inventory))
  (Utilities|Array|Clear (Variables|Default|GetActiveScans))
  (Variables|Default|SetSecondaryScanIndex 0)
  (Utilities|FlowControl|Sequence
    (:then_0
      (if (and (not (Variables|Default|GetDisablePoopDistribute)) (not (Variables|Default|GetDisableDistribution)))
        (CallFunction|AddScanType "NewEnumerator13")
        (CallFunction|AddScanType "NewEnumerator14")))
    (:then_1
      (if (or _organicpolymer _snailpaste)
        (CallFunction|AddScanType "NewEnumerator9")))
    (:then_2
      (if _oil
        (CallFunction|AddScanType "NewEnumerator7")))
    (:then_3
      (if (or _rareflowers _raremushrooms)
        (CallFunction|AddScanType "NewEnumerator11")))
    (:then_4
      (if (Utilities|Struct|BreakSP_ItemCollectorCollectData (Variables|Default|GetCollectData_Ground))
        (CallFunction|AddScanType "NewEnumerator8")))))

(fn BPContainerActivated
  (|CallParentFunction)
  (Networking|SwitchHasAuthority
    (:Authority
      (CallFunction|GetActiveScans))))

(fn AddScanType
  (params (ScanType :type SP_Enum_AggregatorScanType%20Enum :default "NewEnumerator0"))
  (Utilities|Array|Add (Variables|Default|GetActiveScans) ScanType))