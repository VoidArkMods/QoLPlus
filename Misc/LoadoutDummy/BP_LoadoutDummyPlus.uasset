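; BP_LoadoutDummyPlus is the QoL+ Loadout Mannequin structure, whose inventory slows spoilage and is described as a fridge when powered.
; It spawns and links a companion hotbar structure at its extra mesh, mirroring and replicating lock state to it.
; During placement preview, the Drag input toggles snapping through the StructuresPlus global buff.
; AddItemSafe adds items to a target inventory, falling back to source, alternate inventory, then overflow drop.
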(event EventBeginPlay
  (bind _serverhotbar (Variables|Default|GetServerHotbar))
  (bind _myinventorycomponent (Variables|Default|GetMyInventoryComponent))
  (|CallParentFunction)
  (Utilities|FlowControl|Delay 0)
  (if (Variables|Default|GetbIsPreviewStructure)
    (bind _returnvalue (Class|Actor|GetOwnerController))
    (Input|EnableInput _returnvalue)
    (CallFunction|SPClearGlobalBuffDisabledSnaps _returnvalue)
    (else
      (Variables|/Script/ShooterGame.PrimalInventoryComponent|SetInventoryNameOverride _myinventorycomponent "QoL+ Loadout Mannequin")
      (Variables|/Script/ShooterGame.PrimalInventoryComponent|SetRemoteInventoryDescriptionString _myinventorycomponent "If powered will act like a fridge.")
      (Variables|/Script/ShooterGame.PrimalInventoryComponent|SetItemSpoilingTimeMultipliers _myinventorycomponent (Utilities|Array|MakeArray (Utilities|Struct|MakeItemMultiplier "/Script/ShooterGame.PrimalItem" 1e+02)))
      (Networking|SwitchHasAuthority
        (:Authority
          (Variables|Default|SetbIsLocked (not (Variables|Default|GetIsUnlocked)) true)
          (Utilities|IsValid _serverhotbar
            (:Is%20Valid
              (Variables|/Script/ShooterGame.PrimalStructureItemContainer|SetbIsLocked _serverhotbar (Variables|Default|GetbIsLocked) false)
              (Class|PrimalActor|MulticastProperty _serverhotbar "bIsLocked" false))))))))

(event Input|ActionEvents|InputActionDrag
  (params (Key :type Key%20Structure :default "None"))
  (:Pressed
    (bind _returnvalue (Class|Actor|GetOwnerController))
    (bind _success (CallFunction|SPToggleGlobalBuffDisabledSnaps _returnvalue (Utilities|Array|MakeArray) (Utilities|Array|MakeArray 1) (not (Variables|Default|GetDisableSnaps))))
    (if _success
      (Variables|Default|SetDisableSnaps (not (Variables|Default|GetDisableSnaps))))))

(fn ConstructionScript
  (|CallParentFunction))

(fn CreateHotbarStructure
  (params (PC :type Player%20Controller%20Object%20Reference))
  (bind _myextrastaticmesh (Variables|Default|GetMyExtraStaticMesh))
  (bind _returnvalue (Transformation|GetWorldTransform _myextrastaticmesh))
  (bind (_location _rotation) (Math|Transform|BreakTransform _returnvalue))
  (bind _returnvalue_2 (Game|SpawnActorfromClass "/QoLPlus/Misc/LoadoutDummy/BP_LoadoutDummyPlus_Hotbar.BP_LoadoutDummyPlus_Hotbar_C" _returnvalue "AlwaysSpawn" "MultiplyWithRoot" 0 (Pawn|GetControlledPawn PC)))
  (Variables|Default|SetServerHotbar _returnvalue_2)
  (bind _returnvalue_3 (Class|PrimalStructure|BPGetStructureID _returnvalue_2))
  (Variables|Default|SetHotbarID _returnvalue_3 true)
  (Class|PrimalStructure|FinalStructurePlacement _returnvalue_2 PC _location _rotation (.Rotation (Pawn|GetPlayerViewPoint PC)) 0 "None" false)
  (Variables|/Game/Genesis2/Structures/LoadoutMannequin/Structure_LoadoutDummy_Hotbar.Structure_LoadoutDummy_Hotbar_C|SetServerDummy (Variables|Default|GetServerHotbar) self))

(fn AddItemSafe
  (params (Item :type Primal%20Item%20Object%20Reference) (ToInventory :type Primal%20Inventory%20Component%20Object%20Reference) (FromInventory :type Primal%20Inventory%20Component%20Object%20Reference) (OwningPlayer :type Shooter%20Character%20Object%20Reference) (bDontStack :type Boolean) (AnotherFallbackInventory :type Primal%20Inventory%20Component%20Object%20Reference) (InsertAfterItem :type Primal%20Item%20Object%20Reference))
  (if (Variables|Default|GetbDebugItemTransfers)
    (Development|PrintString 0 "----AddItem----")
    (Development|PrintString 0 (Utilities|String|Append (Utilities|String|Append (Utilities|String|Append "Item: " (Utilities|GetDisplayName Item)) (Utilities|String|Append "To: " (Utilities|GetDisplayName ToInventory))) (Utilities|String|Append "From: " (Utilities|GetDisplayName FromInventory)))))
  (Utilities|FlowControl|Sequence
    (:then_0
      (if (not (Class|PrimalInventoryComponent|IsatMaxInventoryItems ToInventory))
        (bind _returnvalue (Class|PrimalInventoryComponent|AddItemObjectEx ToInventory Item false false bDontStack true true false OwningPlayer false 0 (Utilities|IsValid InsertAfterItem)))
        (LocalVariables|SetOutItem_AIS _returnvalue)
        (Utilities|IsValid _returnvalue
          (:Is%20Valid
            (if (Variables|Default|GetbDebugItemTransfers)
              (Development|PrintString 0 "Added Valid"))
            (LocalVariables|SetAddedToTarget_AIS true))
          (:Is%20Not%20Valid
            (if (Variables|Default|GetbDebugItemTransfers)
              (Development|PrintString 0 "Added Invalid"))))
        (else
          (Development|PrintString 0 (Utilities|String|BuildString(Integer) (Utilities|String|BuildString(Integer) "TargetAtMax: " "CurrentMax: " (Variables|Default|GetCurrentMaxInventoryItems) " ") "Max: " (Variables|/Script/ShooterGame.PrimalInventoryComponent|GetMaxInventoryItems ToInventory))))))
    (:then_1
      (Utilities|IsValid FromInventory
        (:Is%20Valid
          (if (not (Utilities|IsValid (LocalVariables|GetOutItem_AIS)))
            (if (not (Class|PrimalInventoryComponent|IsatMaxInventoryItems FromInventory))
              (bind _returnvalue_2 (Class|PrimalInventoryComponent|AddItemObjectEx FromInventory Item false false false true true false 0 false 0 false))
              (LocalVariables|SetOutItem_AIS _returnvalue_2)
              (if (Variables|Default|GetbDebugItemTransfers)
                (Utilities|IsValid _returnvalue_2
                  (:Is%20Valid
                    (Development|PrintString 0 "AddedBackToSourceInv Valid"))
                  (:Is%20Not%20Valid
                    (Development|PrintString 0 "AddedBackToSourceInv Invalid")))))))))
    (:then_2
      (Utilities|IsValid AnotherFallbackInventory
        (:Is%20Valid
          (if (not (Utilities|IsValid (LocalVariables|GetOutItem_AIS)))
            (if (not (Class|PrimalInventoryComponent|IsatMaxInventoryItems AnotherFallbackInventory))
              (bind _returnvalue_3 (Class|PrimalInventoryComponent|AddItemObjectEx AnotherFallbackInventory Item false false false true true false 0 false 0 false))
              (LocalVariables|SetOutItem_AIS _returnvalue_3)
              (if (Variables|Default|GetbDebugItemTransfers)
                (Utilities|IsValid _returnvalue_3
                  (:Is%20Valid
                    (Development|PrintString 0 "AddedToFallback Valid"))
                  (:Is%20Not%20Valid
                    (Development|PrintString 0 "AddedToFallback Invalid")))))))))
    (:then_3
      (if (not (Utilities|IsValid (LocalVariables|GetOutItem_AIS)))
        (bind _newitem (CallFunction|AddtoOverflowDroppedInventory Item))
        (LocalVariables|SetOutItem_AIS _newitem)
        (if (Variables|Default|GetbDebugItemTransfers)
          (Utilities|IsValid _newitem
            (:Is%20Valid
              (Development|PrintString 0 "AddedToOverflow Valid"))
            (:Is%20Not%20Valid
              (Development|PrintString 0 "AddedToOverflow Invalid"))))))
    (:then_4
      (return (LocalVariables|GetOutItem_AIS) (LocalVariables|GetAddedToTarget_AIS)))))

(fn BPTryMultiUse
  (params (ForPC :type Player%20Controller%20Object%20Reference) (UseIndex :type Integer))
  (bind _serverhotbar (Variables|Default|GetServerHotbar))
  (Utilities|FlowControl|Sequence
    (:then_0
      (if (== UseIndex 601)
        (Variables|Default|SetIsUnlocked (not (Variables|Default|GetbIsLocked)))
        (Utilities|IsValid _serverhotbar
          (:Is%20Valid
            (Variables|/Script/ShooterGame.PrimalStructureItemContainer|SetbIsLocked _serverhotbar (Variables|Default|GetbIsLocked) false)
            (Class|PrimalActor|MulticastProperty _serverhotbar "bIsLocked" false)))))
    (:then_1
      (bind _returnvalue (|CallParentFunction ForPC UseIndex))
      (return _returnvalue))))

(fn BPSetPlayerConstructor
  (params (PC :type Player%20Controller%20Object%20Reference))
  (bind _asbuff_structures_plus_global_buff (Utilities|Casting|CastToBuff_StructuresPlus_GlobalBuff (CallFunction|SPGetGlobalBuff PC)))
  (Variables|Default|SetDisableSnaps (> (Utilities|Array|Length (Variables|/QoLPlus/_Buffs/Buff_StructuresPlus_GlobalBuff.Buff_StructuresPlus_GlobalBuff_C|GetDisabledSnapsFrom _asbuff_structures_plus_global_buff)) 0))
  (CallFunction|SPClearGlobalBuffDisabledSnaps PC))

(fn IsValidSnapPointfrom
  (params (ParentStructure :type Primal%20Structure%20Object%20Reference) (MySnapPointFromIndex :type Integer))
  (return (not (Variables|Default|GetDisableSnaps))))