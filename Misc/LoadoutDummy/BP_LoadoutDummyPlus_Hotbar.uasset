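; Hotbar variant or component structure of the QoL+ Loadout Mannequin, configuring the inventory that carries the mannequin's hotbar name.
; Shortly after BeginPlay, skipping preview structures, it overrides the inventory's display name and applies a large spoiling-time multiplier to every PrimalItem.
; All other behavior comes from the parent class, and the construction script only calls its parent.
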(event EventBeginPlay
  (bind _myinventorycomponent (Variables|Default|GetMyInventoryComponent))
  (|CallParentFunction)
  (Utilities|FlowControl|Delay 0)
  (if (not (Variables|Default|GetbIsPreviewStructure))
    (Variables|/Script/ShooterGame.PrimalInventoryComponent|SetInventoryNameOverride _myinventorycomponent "QoL+ Loadout Mannequin Hotbar")
    (Variables|/Script/ShooterGame.PrimalInventoryComponent|SetItemSpoilingTimeMultipliers _myinventorycomponent (Utilities|Array|MakeArray (Utilities|Struct|MakeItemMultiplier "/Script/ShooterGame.PrimalItem" 1e+02)))))

(fn ConstructionScript
  (|CallParentFunction))