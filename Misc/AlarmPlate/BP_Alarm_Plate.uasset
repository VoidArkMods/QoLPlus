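; BP_Alarm_Plate is a placeable alarm plate structure with Structures Plus snap-toggle support, configuring its detection sphere and box extents on BeginPlay.
; As a placement preview, it skips parent BeginPlay and takes input so the Drag action can toggle snapping through the player's global buff.
; IsValidSnapPointFrom rejects snaps while disabled.
; BPSetPlayerConstructor copies the disabled state from that buff, then clears it.
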(event Input|ActionEvents|InputActionDrag
  (params (Key :type Key%20Structure :default "None"))
  (:Pressed
    (bind _returnvalue (Class|Actor|GetOwnerController))
    (bind _success (CallFunction|SPToggleGlobalBuffDisabledSnaps _returnvalue (Utilities|Array|MakeArray) (Utilities|Array|MakeArray 1) (not (Variables|Default|GetDisableSnaps))))
    (if _success
      (Variables|Default|SetDisableSnaps (not (Variables|Default|GetDisableSnaps))))))

(fn ConstructionScript
  (|CallParentFunction))

(fn ReceiveBeginPlay
  (CallFunction|SetStructureDetectSphereRadius (.X (Math|Vector|BreakVector (Variables|Default|GetCurrentStructureDetectBoxExtent))))
  (CallFunction|SetTargetDetectBoxExtent (Variables|Default|GetCurrentTargetDetectBoxExtent))
  (if (Variables|Default|GetbIsPreviewStructure)
    (bind _returnvalue (Class|Actor|GetOwnerController))
    (Input|EnableInput _returnvalue)
    (CallFunction|SPClearGlobalBuffDisabledSnaps _returnvalue)
    (else
      (|CallParentFunction))))

(fn IsValidSnapPointfrom
  (params (ParentStructure :type Primal%20Structure%20Object%20Reference) (MySnapPointFromIndex :type Integer))
  (return (not (Variables|Default|GetDisableSnaps))))

(fn BPSetPlayerConstructor
  (params (PC :type Player%20Controller%20Object%20Reference))
  (bind _asbuff_structures_plus_global_buff (Utilities|Casting|CastToBuff_StructuresPlus_GlobalBuff (CallFunction|SPGetGlobalBuff PC)))
  (Variables|Default|SetDisableSnaps (> (Utilities|Array|Length (Variables|/QoLPlus/_Buffs/Buff_StructuresPlus_GlobalBuff.Buff_StructuresPlus_GlobalBuff_C|GetDisabledSnapsFrom _asbuff_structures_plus_global_buff)) 0))
  (CallFunction|SPClearGlobalBuffDisabledSnaps PC))