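; Temporary OmniTool helper actor that lets a player teleport, alone or as a group, to a Tek Teleporter.
; It opens the local spawn UI filtered to Tek Teleporters and intercepts bed fast travel to run the teleport.
; Group mode waits briefly, then moves nearby characters with their relative transforms, raised clear of the floor.
; Effects scale with dino drag weight, and the actor self-destructs after use or a server-side timeout.
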(event Custom|SpawnGroupTeleportParticle
  (if (not (Networking|IsDedicatedServer))
    (bind _returnvalue (Effects|SpawnEmitteratLocation 0 "/Game/Genesis/Effects/Particles/Creatures/HLNA/P_HLNA_Teleport_Begin.P_HLNA_Teleport_Begin" (Transformation|GetActorLocation) (Transformation|GetActorRotation) "1.000000,1.000000,1.000000" true "None" true true 1.5e+03 false -1.0 0))
    (Transformation|SetWorldScale3D _returnvalue "0.550000,0.550000,0.550000")
    (Variables|/Script/Engine.ParticleSystemComponent|SetCustomTimeDilation _returnvalue 5.0)))

(event Custom|HandleGroupTeleportEvent
  (params (PC :type Shooter%20Player%20Controller%20Object%20Reference) (Teleporter :type Tek%20Teleporter%20Object%20Reference))
  (Utilities|FlowControl|Delay 0 5.0)
  (Utilities|FlowControl|Sequence
    (:then_0
      (Utilities|IsValid PC
        (:Is%20Valid
          (CallFunction|DoTeleport Teleporter PC))))
    (:then_1
      (CallFunction|DestroyActorEvent))))

(event Custom|DoTeleportOutVFX
  (params (EffectScale :type Float%20%28double-precision%29) (EffectLoc :type Vector) (EffectRot :type Rotator))
  (if (not (Networking|IsDedicatedServer))
    (bind _returnvalue (Effects|SpawnEmitteratLocation 0 (Variables|Default|GetTeleportOutEmitter) EffectLoc EffectRot "1.000000,1.000000,1.000000" true "None" true true 1.5e+03 false -1.0 0))
    (Transformation|SetWorldScale3D _returnvalue (Math|Conversions|ToVector(Float) EffectScale))))

(event Custom|DoPlayTeleportOutSound
  (Audio|PlaySoundatLocation 0 (Variables|Default|GetTeleportOutSound) (Transformation|GetActorLocation) "0, 0, 0" 1.0 1.0 0.0 0 0 0 0))

(event Custom|ShowTeleportSelectEvent
  (params (PC :type Player%20Controller%20Object%20Reference) (IsGroup :type Boolean))
  (Variables|Default|SetIsGroupTeleport IsGroup)
  (if (not (Networking|IsDedicatedServer))
    (Utilities|IsValid PC
      (:Is%20Valid
        (if (Pawn|IsLocalController PC)
          (bind _asshooter_hud (Utilities|Casting|CastToShooterHUD (HUD|GetHUD PC)))
          (Class|ShooterHUD|ShowSpawnUI _asshooter_hud self))))))

(event Custom|DestroyActorEvent
  (Utilities|FlowControl|Delay 0)
  (Actor|DestroyActor))

(event EventBeginPlay
  (Networking|SwitchHasAuthority
    (:Authority
      (Utilities|Time|SetTimerbyEvent (delegate Custom|DestroyActorEvent) 9e+01))))

(fn ConstructionScript
  (|CallParentFunction))

(fn DoTeleport
  (params (ToTeleporter :type Tek%20Teleporter%20Object%20Reference) (SPC :type Shooter%20Player%20Controller%20Object%20Reference))
  (Utilities|IsValid ToTeleporter
    (:Is%20Valid
      (CallFunction|DoPlayTeleportOutSound)
      (Default|DoPlayTeleportinSound ToTeleporter false)
      (bind (_characters _transforms) (CallFunction|GetCharactersforTeleport SPC))
      (for (_array_element _array_index) _characters
        (Variables|/Script/ShooterGame.PrimalCharacterMovement|SetDisableMovementPhysicsUntilTime (Class|PrimalAutocastFunctions|CharacterMovementtoPCM (Variables|/Script/Engine.Character|GetCharacterMovement _array_element)) (- (Utilities|Time|GetGameTimeinSeconds) (Math|Conversions|ToFloat(Integer) -2.0)))
        (CallFunction|DoTeleportOutVFX (CallFunction|GetTeleportEffectScale _array_element) (Transformation|GetActorLocation _array_element) (Transformation|GetActorRotation _array_element))
        (LocalVariables|SetTargetLoc (+ (Math|Vector|SelectVector (.Location (Math|Transform|BreakTransform (Math|Transform|ComposeTransforms (Utilities|Array|Get(acopy) _transforms _array_index) (Transformation|GetActorTransform ToTeleporter)))) (Math|Vector|MakeVector (.X (Math|Vector|BreakVector (.Location (Math|Transform|BreakTransform (Math|Transform|ComposeTransforms (Utilities|Array|Get(acopy) _transforms _array_index) (Transformation|GetActorTransform ToTeleporter)))))) (.Y (Math|Vector|BreakVector (.Location (Math|Transform|BreakTransform (Math|Transform|ComposeTransforms (Utilities|Array|Get(acopy) _transforms _array_index) (Transformation|GetActorTransform ToTeleporter)))))) (+ (Variables|/Script/Engine.CapsuleComponent|GetCapsuleHalfHeight (Variables|/Script/Engine.Character|GetCapsuleComponent _array_element)) (.z (Transformation|GetActorLocation ToTeleporter)))) (>= (.Z (Math|Vector|BreakVector (.Location (Math|Transform|BreakTransform (Math|Transform|ComposeTransforms (Utilities|Array|Get(acopy) _transforms _array_index) (Transformation|GetActorTransform ToTeleporter)))))) (+ (Variables|/Script/Engine.CapsuleComponent|GetCapsuleHalfHeight (Variables|/Script/Engine.Character|GetCapsuleComponent _array_element)) (.z (Transformation|GetActorLocation ToTeleporter))))) "0, 0,25.000000"))
        (Transformation|Teleport _array_element (LocalVariables|GetTargetLoc) (.Rotation (Math|Transform|BreakTransform (Math|Transform|ComposeTransforms (Utilities|Array|Get(acopy) _transforms _array_index) (Transformation|GetActorTransform ToTeleporter)))))
        (Networking|ForceNetUpdate _array_element)
        (Default|DoTeleportinVFX ToTeleporter (CallFunction|GetTeleportEffectScale _array_element) (Transformation|GetActorLocation _array_element) (Transformation|GetActorRotation _array_element) false)))))

(fn BPHandleBedFastTravel
  (params (ForPC :type Shooter%20Player%20Controller%20Object%20Reference) (ToBed :type Primal%20Structure%20Object%20Reference))
  (Utilities|FlowControl|Sequence
    (:then_0
      (bind _astek_teleporter (Utilities|Casting|CastToTekTeleporter ToBed))
      (if (Variables|Default|GetIsGroupTeleport)
        (CallFunction|SpawnGroupTeleportParticle)
        (CallFunction|HandleGroupTeleportEvent ForPC _astek_teleporter)
        (else
          (CallFunction|DoTeleport _astek_teleporter ForPC)
          (CallFunction|DestroyActorEvent))))
    (:then_1
      (return true))))

(fn GetBedFilterClass
  (return "/Game/PrimalEarth/Structures/TekTier/TekTeleporter.TekTeleporter_C"))

(fn GetTeleportEffectScale
  (params (ForCharacter :type Primal%20Character%20Object%20Reference))
  (bind _teleporteffectscaledinomindrag (Variables|Default|GetTeleportEffectScaleDinoMinDrag))
  (bind _teleporteffectscaledinomaxdrag (Variables|Default|GetTeleportEffectScaleDinoMaxDrag))
  (Utilities|FlowControl|Sequence
    (:then_0
      (Utilities|Casting|CastToShooterCharacter ForCharacter
        (:then
          (LocalVariables|SetretVal 3.0))
        (:CastFailed
          (bind _asprimal_dino_character (Utilities|Casting|CastToPrimalDinoCharacter ForCharacter))
          (LocalVariables|SetretVal (Math|Float|MapRangeUnclamped (Math|Float|Clamp(Float) (Variables|/Script/ShooterGame.PrimalCharacter|GetDragWeight _asprimal_dino_character) _teleporteffectscaledinomindrag _teleporteffectscaledinomaxdrag) _teleporteffectscaledinomindrag _teleporteffectscaledinomaxdrag (Variables|Default|GetTeleportEffectScaleDinoMinScale) (Variables|Default|GetTeleportEffectScaleDinoMaxScale))))))
    (:then_1
      (return (LocalVariables|GetretVal)))))

(fn BPPreventSpawnforPlayer
  (params (PC :type Shooter%20Player%20Controller%20Object%20Reference) (bCheckCooldownTime :type Boolean) (FromStructure :type Primal%20Structure%20Object%20Reference))
  (return true))

(fn GetCharactersforTeleport
  (params (PC :type Player%20Controller%20Object%20Reference))
  (Utilities|FlowControl|Sequence
    (:then_0
      (if (Variables|Default|GetIsGroupTeleport)
        (bind (_characters _transforms) (CallFunction|SPGetCharactersforTeleport self 8e+02 (Utilities|Array|MakeArray) false))
        (LocalVariables|SetCharacters_GCT _characters)
        (LocalVariables|SetTransforms_GCT _transforms)
        (else
          (bind _asshooter_player_controller (Utilities|Casting|CastToShooterPlayerController PC))
          (Utilities|Array|Add (LocalVariables|GetCharacters_GCT) (Class|ShooterPlayerController|GetPlayerCharacter _asshooter_player_controller))
          (Utilities|Array|Add (LocalVariables|GetTransforms_GCT) (Math|Transform|MakeTransform "0, 0, 0")))))
    (:then_1
      (return (LocalVariables|GetCharacters_GCT) (LocalVariables|GetTransforms_GCT)))))