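; Spray painter weapon that applies its item's dye color to selected color regions of a traced structure.
; Alt1–Alt6 toggle the six regions, saved as item custom data and sent to a server-added buff that drives the UI.
; Firing traces on the local client, then sets structure region colors and, when clearing with color index zero or running on the server, edits dynamic material parameters directly.
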(event Custom|HandleFired
  (params (Structure :type Primal%20Structure%20Object%20Reference) (ColorIndex :type Integer))
  (bind _regions (CallFunction|GetRegionArray))
  (CallFunction|BroadcastChanges Structure ColorIndex _regions))

(event Custom|HandleRegionToggle
  (params (RegionIndex :type Integer))
  (bind _buffref (Variables|Default|GetBuffRef))
  (CallFunction|ToggleRegion RegionIndex)
  (Utilities|IsValid _buffref
    (:Is%20Valid
      (bind _regions (CallFunction|GetRegionArray))
      (Default|SendNewDatatoClient _buffref _regions))))

(event Custom|BroadcastChanges
  (params (Structure :type Primal%20Structure%20Object%20Reference) (ColorIndex :type Integer) (Regions :type Array%20of%20Booleans))
  (for (_array_element _array_index) Regions
    (if _array_element
      (Class|PrimalStructure|SetStructureColorValue Structure _array_index ColorIndex)))
  (CallFunction|UpdateMaterials Structure ColorIndex Regions)
  (Class|KismetSystemLibrary|CanRunCosmeticEvents
    (:Yes
      (if (Variables|/Script/ShooterGame.PrimalStructure|GetbUseBPRefreshedStructureColors Structure)
        (Class|PrimalStructure|RefreshStructureColors Structure 0)))))

(event EventEndPlay
  (params (EndPlayReason :type EEndPlayReason%20Enum :default "Destroyed"))
  (bind _buffref (Variables|Default|GetBuffRef))
  (Networking|SwitchHasAuthority
    (:Authority
      (Utilities|IsValid _buffref
        (:Is%20Valid
          (Actor|DestroyActor _buffref))))))

(event EventBeginPlay
  (Utilities|FlowControl|Delay 0)
  (bind _returnvalue (Class|Actor|GetOwnerController))
  (Utilities|FlowControl|Sequence
    (:then_0
      (if (Pawn|IsLocalController _returnvalue)
        (Input|EnableInput _returnvalue)))
    (:then_1
      (Networking|SwitchHasAuthority
        (:Authority
          (bind _asshooter_player_controller (Utilities|Casting|CastToShooterPlayerController _returnvalue))
          (bind _returnvalue_2 (Class|PrimalBuff|StaticAddBuff "/QoLPlus/_Buffs/Buff_StructuresPlus_SprayPainter.Buff_StructuresPlus_SprayPainter_C" (Class|ShooterPlayerController|GetPlayerCharacter _asshooter_player_controller) 0 0 false))
          (bind _asbuff_structures_plus_spray_painter (Utilities|Casting|CastToBuff_StructuresPlus_SprayPainter _returnvalue_2))
          (Variables|Default|SetBuffRef _asbuff_structures_plus_spray_painter)
          (bind _regions (CallFunction|GetRegionArray))
          (Default|InitializeUI _asbuff_structures_plus_spray_painter _regions))))))

(event Input|KeyboardEvents|Alt1
  (params (Key :type Key%20Structure))
  (:Pressed
    (CallFunction|HandleRegionToggle)))

(event Input|KeyboardEvents|Alt2
  (params (Key :type Key%20Structure))
  (:Pressed
    (CallFunction|HandleRegionToggle 1)))

(event Input|KeyboardEvents|Alt3
  (params (Key :type Key%20Structure))
  (:Pressed
    (CallFunction|HandleRegionToggle 2)))

(event Input|KeyboardEvents|Alt4
  (params (Key :type Key%20Structure))
  (:Pressed
    (CallFunction|HandleRegionToggle 3)))

(event Input|KeyboardEvents|Alt5
  (params (Key :type Key%20Structure))
  (:Pressed
    (CallFunction|HandleRegionToggle 4)))

(event Input|KeyboardEvents|Alt6
  (params (Key :type Key%20Structure))
  (:Pressed
    (CallFunction|HandleRegionToggle 5)))

(fn ConstructionScript)

(fn BPFiredWeapon
  (bind _returnvalue (Class|Actor|GetOwnerController))
  (if (Pawn|IsLocalController _returnvalue)
    (bind _returnvalue_2 (Class|PrimalItem|GetItemColorID (Variables|Default|GetAssociatedPrimalItem)))
    (bind _target (CallFunction|SPLineTracefromWeapon _returnvalue self (Utilities|Array|MakeArray "ObjectTypeQuery9") false 0.0))
    (Utilities|IsValid _target
      (:Is%20Valid
        (bind _asprimal_structure (Utilities|Casting|CastToPrimalStructure _target))
        (CallFunction|HandleFired _asprimal_structure _returnvalue_2)))))

(fn GetRegionArray
  (bind _associatedprimalitem (Variables|Default|GetAssociatedPrimalItem))
  (bind (_outdata _returnvalue) (Class|PrimalItem|GetCustomItemData _associatedprimalitem "SplusColorRegions"))
  (Utilities|FlowControl|Sequence
    (:then_0
      (if _returnvalue
        (for _array_element (.CustomDataStrings (Utilities|Struct|BreakCustomItemData _outdata))
          (Utilities|Array|Add (LocalVariables|GetRegions_GRA) (Utilities|Enum|Equal(Enum) _array_element "1")))
        (else
          (LocalVariables|SetRegions_GRA (Utilities|Array|MakeArray true false false false false false)))))
    (:then_1
      (return (LocalVariables|GetRegions_GRA)))))

(fn SetRegionArray
  (params (Regions :type Array%20of%20Booleans))
  (for _array_element Regions
    (Utilities|Array|Add (LocalVariables|GetRegions_SRA) (Utilities|String|SelectString "1" "0" _array_element)))
  (Class|PrimalItem|SetCustomItemData (Variables|Default|GetAssociatedPrimalItem) (Utilities|Struct|MakeCustomItemData "SplusColorRegions" (LocalVariables|GetRegions_SRA) "(ByteArrays=)" "(Doubles=)")))

(fn ToggleRegion
  (params (Index :type Integer))
  (bind _regions (CallFunction|GetRegionArray))
  (if (>= (Utilities|Array|LastIndex _regions) Index)
    (LocalVariables|SetTempRegions _regions)
    (Utilities|Array|SetArrayElem (LocalVariables|GetTempRegions) Index (not (Utilities|Array|Get(acopy) _regions Index)))
    (CallFunction|SetRegionArray (LocalVariables|GetTempRegions))))

(fn GetMeshComponents
  (params (Structure :type Primal%20Structure%20Object%20Reference))
  (LocalVariables|SetAllComponents_GMC (Actor|GetComponentsByClass Structure "/Script/Engine.MeshComponent"))
  (for _array_element (LocalVariables|GetAllComponents_GMC)
    (bind _asmesh_component (Utilities|Casting|CastToMeshComponent _array_element))
    (if (and (Variables|/Script/Engine.SceneComponent|GetbVisible _asmesh_component) (not (Variables|/Script/Engine.SceneComponent|GetbHiddenInGame _asmesh_component)))
      (Utilities|Array|Add (LocalVariables|GetMeshComponents_GMC) _asmesh_component)))
  (return (LocalVariables|GetMeshComponents_GMC)))

(fn UpdateMaterials
  (params (Structure :type Primal%20Structure%20Object%20Reference) (ColorIndex :type Integer) (Regions :type Array%20of%20Booleans))
  (Class|KismetSystemLibrary|CanRunCosmeticEvents
    (:Yes
      (if (or (== ColorIndex 0) (Networking|IsServer))
        (bind _meshcomponents (CallFunction|GetMeshComponents Structure))
        (for _array_element _meshcomponents
          (for _index (range 0 (- (Rendering|Material|GetNumMaterials _array_element) 1))
            (bind _asmaterial_instance_dynamic (Utilities|Casting|CastToMaterialInstanceDynamic (Rendering|Material|GetMaterial _array_element _index))
              (:then
                (LocalVariables|SetCurMaterial_UM _asmaterial_instance_dynamic))
              (:CastFailed
                (bind _returnvalue (Rendering|Material|CreateDynamicMaterialInstance _array_element _index 0 "None" :!class /Script/Engine.PrimitiveComponent))
                (LocalVariables|SetCurMaterial_UM _returnvalue)))
            (CallFunction|RefreshMaterialInstance (LocalVariables|GetCurMaterial_UM) Regions (== ColorIndex 0))))))))

(fn RefreshMaterialInstance
  (params (Material :type Material%20Instance%20Dynamic%20Object%20Reference) (Regions :type Array%20of%20Booleans) (ClearColors :type Boolean))
  (bind _returnvalue (Math|Float|SelectFloat 0.0 1.0 ClearColors))
  (for (_array_element _array_index) Regions
    (if _array_element
      (Rendering|Material|SetScalarParameterValue Material (Utilities|String|StringToName (Utilities|String|BuildString(Integer) "UsingColor" "" _array_index)) _returnvalue :!class /Script/Engine.MaterialInstanceDynamic)
      (Rendering|Material|SetScalarParameterValue Material (Utilities|String|StringToName (Utilities|String|BuildString(Integer) "UsingColorizedColor" "" _array_index)) _returnvalue :!class /Script/Engine.MaterialInstanceDynamic)
      (if (not ClearColors)
        (bind _returnvalue_2 (Class|PrimalItem|GetItemDyeColors (Variables|Default|GetAssociatedPrimalItem)))
        (Rendering|Material|SetVectorParameterValue Material (Utilities|String|StringToName (Utilities|String|BuildString(Integer) "Color" "" _array_index)) (Utilities|Array|Get(acopy) _returnvalue_2) :!class /Script/Engine.MaterialInstanceDynamic)))))